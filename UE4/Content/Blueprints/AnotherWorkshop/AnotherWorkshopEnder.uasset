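; AnotherWorkshopEnder watches the workshop pawns and ends the session once all of them finish.
; On its first tick it finds and caches every AnotherWorkshopPawn.
; Every later tick it checks whether each pawn's WorkshopState equals one specific enum value, apparently the done state, and if all match it calls GotoMainMenu on the menu interface.
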(event EventTick
  (params (DeltaSeconds :type Float%20%28single-precision%29))
  (if (Variables|Default|GetFoundActors)
    (Variables|Default|SetAllPlayersDone true)
    (for _array_element (Variables|Default|GetActorList)
      (bind _asanotherworkshoppawn_c (Utilities|Casting|CastToAnotherWorkshopPawn _array_element))
      (if (not (Utilities|Enum|Equal(Enum) (Variables|/Game/Blueprints/AnotherWorkshop/AnotherWorkshopPawn.AnotherWorkshopPawn_C|GetWorkshopState _asanotherworkshoppawn_c) "NewEnumerator8"))
        (Variables|Default|SetAllPlayersDone false)))
    (if (Variables|Default|GetAllPlayersDone)
      (Default|GotoMainMenu (Variables|Default|GetMenuInterface) false))
    (else
      (Variables|Default|SetActorClass "/Game/Blueprints/AnotherWorkshop/AnotherWorkshopPawn.AnotherWorkshopPawn_C")
      (bind _returnvalue (Class|GameStateStatics|FindActorsOfType (Variables|Default|GetActorClass)))
      (Variables|Default|SetActorList _returnvalue)
      (Variables|Default|SetFoundActors true))))

(fn ConstructionScript)