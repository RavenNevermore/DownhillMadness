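; Canvas HUD for the vehicle customisation workshop, drawing text menus and prompts for the owning AnotherWorkshopPawn.
; DrawHUD switches on the pawn's WorkshopState to show slot selection, body selection, save, cancel or delete prompts, or a waiting-for-players message.
; Each screen reads selection state from the pawn to place a cursor texture, scaling everything against a 1920x1080 reference.
; The save prompt also lists wheel and steering errors from the vehicle body, shifting Yes/No down.
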(event EventDrawHUD
  (params (SizeX :type Integer) (SizeY :type Integer))
  (bind _asanotherworkshoppawn_c (Utilities|Casting|CastToAnotherWorkshopPawn (Class|HUD|GetOwningPawn)))
  (Variables|Default|SetWorkshopPawn _asanotherworkshoppawn_c)
  (switch Utilities|FlowControl|Switch|SwitchonAnotherWorkshopStateEnum (Variables|/Game/Blueprints/AnotherWorkshop/AnotherWorkshopPawn.AnotherWorkshopPawn_C|GetWorkshopState _asanotherworkshoppawn_c)
    (:NewEnumerator0
      (CallFunction|SlotSelection SizeX SizeY))
    (:NewEnumerator2
      (CallFunction|BodySelection SizeX SizeY))
    (:NewEnumerator4
      (CallFunction|SavePrompt SizeX SizeY))
    (:NewEnumerator5
      (CallFunction|CancelPrompt SizeX SizeY))
    (:NewEnumerator6
      (CallFunction|DeletePrompt SizeX SizeY))
    (:NewEnumerator8
      (HUD|DrawText "Waiting for all players to finish..." "(R=1.000000,G=1.000000,B=1.000000,A=1.000000)" 2e+01 3e+01 "/Game/Textures/Menu_Main/Font_Harrington_TEX.Font_Harrington_TEX" (Math|Float|Min(Float) (/ (Math|Conversions|ToFloat(Integer) SizeX) 1.92e+03) (/ (Math|Conversions|ToFloat(Integer) SizeY) 1.08e+03)) true))))

(fn ConstructionScript)

(fn SlotSelection
  (params (Screen%20X :type Integer) (Screen%20Y :type Integer))
  (bind _returnvalue (Math|Conversions|ToFloat(Integer) Screen%20Y))
  (bind _returnvalue_2 (Math|Conversions|ToFloat(Integer) Screen%20X))
  (bind _workshoppawn (Variables|Default|GetWorkshopPawn))
  (bind _returnvalue_3 (/ _returnvalue 1.08e+03))
  (bind _returnvalue_4 (/ _returnvalue_2 1.92e+03))
  (bind _returnvalue_5 (Math|Float|Min(Float) _returnvalue_4 _returnvalue_3))
  (for (_array_element _array_index) (Variables|/Game/Blueprints/AnotherWorkshop/AnotherWorkshopPawn.AnotherWorkshopPawn_C|GetVehicleSlots _workshoppawn)
    (bind _returnvalue_6 (Class|VehicleSpawnerLibrary|GetGeneratedVehicleName _array_element))
    (HUD|DrawText (Utilities|String|Append (Utilities|String|Append (Utilities|String|ToString(Integer) _array_index) ": ") _returnvalue_6) "(R=1.000000,G=1.000000,B=1.000000,A=1.000000)" 5e+01 (+ (* _array_index 45.0) 75.0) "/Game/Textures/Menu_Main/Font_Harrington_TEX.Font_Harrington_TEX" _returnvalue_5 true))
  (HUD|DrawText "Done Customising" "(R=1.000000,G=1.000000,B=1.000000,A=1.000000)" 4e+01 (+ (* (Math|Conversions|ToInteger(Byte) (Variables|/Game/Blueprints/AnotherWorkshop/AnotherWorkshopPawn.AnotherWorkshopPawn_C|GetMaxVehicleSlots _workshoppawn)) 45.0) 75.0) "/Game/Textures/Menu_Main/Font_Harrington_TEX.Font_Harrington_TEX" _returnvalue_5 true)
  (HUD|DrawText "Select Vehicle Slot:" "(R=1.000000,G=1.000000,B=1.000000,A=1.000000)" 2e+01 3e+01 "/Game/Textures/Menu_Main/Font_Harrington_TEX.Font_Harrington_TEX" _returnvalue_5 true)
  (Canvas|DrawTexture "/Game/Textures/AnotherWorkshop/SimpleCursor.SimpleCursor" 25.0 (+ (* (Variables|/Game/Blueprints/AnotherWorkshop/AnotherWorkshopPawn.AnotherWorkshopPawn_C|GetCurrentVehicleSlot (Variables|Default|GetWorkshopPawn)) 45.0) 85.0) 21.0 35.0 0.0 0.0 1.0 1.0 "(R=1.000000,G=1.000000,B=1.000000,A=1.000000)" "BLEND_Translucent" _returnvalue_5 true))

(fn BodySelection
  (params (Screen%20X :type Integer) (Screen%20Y :type Integer))
  (bind _returnvalue (Math|Conversions|ToFloat(Integer) Screen%20Y))
  (bind _returnvalue_2 (Math|Conversions|ToFloat(Integer) Screen%20X))
  (bind _returnvalue_3 (/ _returnvalue 1.08e+03))
  (bind _returnvalue_4 (/ _returnvalue_2 1.92e+03))
  (bind _returnvalue_5 (Math|Float|Min(Float) _returnvalue_4 _returnvalue_3))
  (HUD|DrawText "Left/Right: Select Vehicle" "(R=1.000000,G=1.000000,B=1.000000,A=1.000000)" 2e+01 3e+01 "/Game/Textures/Menu_Main/Font_Harrington_TEX.Font_Harrington_TEX" _returnvalue_5 true)
  (HUD|DrawText "A: Confirm" "(R=1.000000,G=1.000000,B=1.000000,A=1.000000)" 2e+01 75.0 "/Game/Textures/Menu_Main/Font_Harrington_TEX.Font_Harrington_TEX" _returnvalue_5 true)
  (HUD|DrawText "B: Cancel" "(R=1.000000,G=1.000000,B=1.000000,A=1.000000)" 2e+01 1.2e+02 "/Game/Textures/Menu_Main/Font_Harrington_TEX.Font_Harrington_TEX" _returnvalue_5 true))

(fn CancelPrompt
  (params (Screen%20X :type Integer) (Screen%20Y :type Integer))
  (bind _returnvalue (Math|Conversions|ToFloat(Integer) Screen%20Y))
  (bind _returnvalue_2 (Math|Conversions|ToFloat(Integer) Screen%20X))
  (bind _returnvalue_3 (/ _returnvalue 1.08e+03))
  (bind _returnvalue_4 (/ _returnvalue_2 1.92e+03))
  (bind _returnvalue_5 (Math|Float|Min(Float) _returnvalue_4 _returnvalue_3))
  (HUD|DrawText "Return to slot selection? (Unsaved changes will be lost)" "(R=1.000000,G=1.000000,B=1.000000,A=1.000000)" 2e+01 3e+01 "/Game/Textures/Menu_Main/Font_Harrington_TEX.Font_Harrington_TEX" _returnvalue_5 true)
  (HUD|DrawText "Yes" "(R=1.000000,G=1.000000,B=1.000000,A=1.000000)" 5e+01 75.0 "/Game/Textures/Menu_Main/Font_Harrington_TEX.Font_Harrington_TEX" _returnvalue_5 true)
  (HUD|DrawText "No" "(R=1.000000,G=1.000000,B=1.000000,A=1.000000)" 5e+01 1.2e+02 "/Game/Textures/Menu_Main/Font_Harrington_TEX.Font_Harrington_TEX" _returnvalue_5 true)
  (if (Variables|/Game/Blueprints/AnotherWorkshop/AnotherWorkshopPawn.AnotherWorkshopPawn_C|GetCancelPromptSelection (Variables|Default|GetWorkshopPawn))
    (Canvas|DrawTexture "/Game/Textures/AnotherWorkshop/SimpleCursor.SimpleCursor" 25.0 85.0 21.0 35.0 0.0 0.0 1.0 1.0 "(R=1.000000,G=1.000000,B=1.000000,A=1.000000)" "BLEND_Translucent" _returnvalue_5 true)
    (else
      (Canvas|DrawTexture "/Game/Textures/AnotherWorkshop/SimpleCursor.SimpleCursor" 25.0 1.3e+02 21.0 35.0 0.0 0.0 1.0 1.0 "(R=1.000000,G=1.000000,B=1.000000,A=1.000000)" "BLEND_Translucent" _returnvalue_5 true))))

(fn SavePrompt
  (params (Screen%20X :type Integer) (Screen%20Y :type Integer))
  (bind _returnvalue (Math|Conversions|ToFloat(Integer) Screen%20Y))
  (bind _returnvalue_2 (Math|Conversions|ToFloat(Integer) Screen%20X))
  (bind _variable (|LocalVariable))
  (bind _returnvalue_3 (/ _returnvalue 1.08e+03))
  (bind _returnvalue_4 (/ _returnvalue_2 1.92e+03))
  (bind _returnvalue_5 (Math|Float|Min(Float) _returnvalue_4 _returnvalue_3))
  (HUD|DrawText (Utilities|String|Append (Utilities|String|Append "Save vehicle to slot " (Utilities|String|ToString(Integer) (Variables|/Game/Blueprints/AnotherWorkshop/AnotherWorkshopPawn.AnotherWorkshopPawn_C|GetCurrentVehicleSlot (Variables|Default|GetWorkshopPawn)))) "? (Old vehicle will be overwritten)") "(R=1.000000,G=1.000000,B=1.000000,A=1.000000)" 2e+01 3e+01 "/Game/Textures/Menu_Main/Font_Harrington_TEX.Font_Harrington_TEX" _returnvalue_5 true)
  (bind _returnvalue_6 (Class|VehicleBodyBase|CheckVehicleforErrors (Variables|/Game/Blueprints/AnotherWorkshop/AnotherWorkshopPawn.AnotherWorkshopPawn_C|GetVehicleBody (Variables|Default|GetWorkshopPawn))))
  (|Assign _variable 0.0)
  (if (.noErrors (Utilities|Struct|BreakVehicleErrorCheck _returnvalue_6))
    _
    (else
      (HUD|DrawText "WARNING:" "(R=1.000000,G=0.000000,B=0.000000,A=1.000000)" 2e+01 75.0 "/Game/Textures/Menu_Main/Font_Harrington_TEX.Font_Harrington_TEX" _returnvalue_5 true)
      (if (.hasNoWheels (Utilities|Struct|BreakVehicleErrorCheck _returnvalue_6))
        (|Assign _variable (+ _variable 45.0))
        (HUD|DrawText "-Vehicle has no wheels" "(R=1.000000,G=0.000000,B=0.000000,A=1.000000)" 2e+01 (+ _variable 75.0) "/Game/Textures/Menu_Main/Font_Harrington_TEX.Font_Harrington_TEX" _returnvalue_5 true))
      (if (.hasNoSteerableWheels (Utilities|Struct|BreakVehicleErrorCheck _returnvalue_6))
        (|Assign _variable (+ _variable 45.0))
        (HUD|DrawText "-No wheels are steerable" "(R=1.000000,G=0.000000,B=0.000000,A=1.000000)" 2e+01 (+ _variable 75.0) "/Game/Textures/Menu_Main/Font_Harrington_TEX.Font_Harrington_TEX" _returnvalue_5 true))
      (|Assign _variable (+ _variable 45.0))))
  (HUD|DrawText "Yes" "(R=1.000000,G=1.000000,B=1.000000,A=1.000000)" 5e+01 (+ _variable 75.0) "/Game/Textures/Menu_Main/Font_Harrington_TEX.Font_Harrington_TEX" _returnvalue_5 true)
  (HUD|DrawText "No" "(R=1.000000,G=1.000000,B=1.000000,A=1.000000)" 5e+01 (+ _variable 1.2e+02) "/Game/Textures/Menu_Main/Font_Harrington_TEX.Font_Harrington_TEX" _returnvalue_5 true)
  (if (Variables|/Game/Blueprints/AnotherWorkshop/AnotherWorkshopPawn.AnotherWorkshopPawn_C|GetSavePromptSelection (Variables|Default|GetWorkshopPawn))
    (Canvas|DrawTexture "/Game/Textures/AnotherWorkshop/SimpleCursor.SimpleCursor" 25.0 (+ _variable 85.0) 21.0 35.0 0.0 0.0 1.0 1.0 "(R=1.000000,G=1.000000,B=1.000000,A=1.000000)" "BLEND_Translucent" _returnvalue_5 true)
    (else
      (Canvas|DrawTexture "/Game/Textures/AnotherWorkshop/SimpleCursor.SimpleCursor" 25.0 (+ _variable 1.3e+02) 21.0 35.0 0.0 0.0 1.0 1.0 "(R=1.000000,G=1.000000,B=1.000000,A=1.000000)" "BLEND_Translucent" _returnvalue_5 true))))

(fn DeletePrompt
  (params (Screen%20X :type Integer) (Screen%20Y :type Integer))
  (bind _returnvalue (Math|Conversions|ToFloat(Integer) Screen%20Y))
  (bind _returnvalue_2 (Math|Conversions|ToFloat(Integer) Screen%20X))
  (bind _returnvalue_3 (/ _returnvalue 1.08e+03))
  (bind _returnvalue_4 (/ _returnvalue_2 1.92e+03))
  (bind _returnvalue_5 (Math|Float|Min(Float) _returnvalue_4 _returnvalue_3))
  (HUD|DrawText "Delete everything and restart from scratch?" "(R=1.000000,G=1.000000,B=1.000000,A=1.000000)" 2e+01 3e+01 "/Game/Textures/Menu_Main/Font_Harrington_TEX.Font_Harrington_TEX" _returnvalue_5 true)
  (HUD|DrawText "Yes" "(R=1.000000,G=1.000000,B=1.000000,A=1.000000)" 5e+01 75.0 "/Game/Textures/Menu_Main/Font_Harrington_TEX.Font_Harrington_TEX" _returnvalue_5 true)
  (HUD|DrawText "No" "(R=1.000000,G=1.000000,B=1.000000,A=1.000000)" 5e+01 1.2e+02 "/Game/Textures/Menu_Main/Font_Harrington_TEX.Font_Harrington_TEX" _returnvalue_5 true)
  (if (Variables|/Game/Blueprints/AnotherWorkshop/AnotherWorkshopPawn.AnotherWorkshopPawn_C|GetDeletePromptSelection (Variables|Default|GetWorkshopPawn))
    (Canvas|DrawTexture "/Game/Textures/AnotherWorkshop/SimpleCursor.SimpleCursor" 25.0 85.0 21.0 35.0 0.0 0.0 1.0 1.0 "(R=1.000000,G=1.000000,B=1.000000,A=1.000000)" "BLEND_Translucent" _returnvalue_5 true)
    (else
      (Canvas|DrawTexture "/Game/Textures/AnotherWorkshop/SimpleCursor.SimpleCursor" 25.0 1.3e+02 21.0 35.0 0.0 0.0 1.0 1.0 "(R=1.000000,G=1.000000,B=1.000000,A=1.000000)" "BLEND_Translucent" _returnvalue_5 true))))