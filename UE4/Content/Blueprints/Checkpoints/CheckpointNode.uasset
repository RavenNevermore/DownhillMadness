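; CheckpointNode is a placeable checkpoint that hands a kart respawn-style transform to any overlapping actor implementing CheckpointInterface.
; On Hitbox overlap it sends SetCheckpointMessage with KartOrientation's location offset from the actor and its rotation used directly, optionally printing a confirmation.
; The construction script applies the checkpoint material, scales the whole actor by Radius, and places an Arrow at KartOrientation as a preview.
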(event OnComponentBeginOverlap(Hitbox)
  (params (OtherActor :type Actor%20Object%20Reference) (OtherComp :type Primitive%20Component%20Object%20Reference) (OtherBodyIndex :type Integer))
  (bind _kartorientation (Variables|Checkpointsettings|GetKartOrientation))
  (bind (_location _rotation) (Math|Transform|BreakTransform _kartorientation))
  (if (Utilities|DoesObjectImplementInterface OtherActor "/Game/Blueprints/Checkpoints/CheckpointInterface.CheckpointInterface_C")
    (Class|CheckpointInterface|SetCheckpoint(Message) OtherActor (Math|Transform|MakeTransform (+ (Transformation|GetActorLocation self) _location) _rotation))
    (if (Variables|Checkpointsettings|GetShowMessageOnHit)
      (Development|PrintString "Checkpoint activated!"))))

(fn ConstructionScript
  (bind _radius (Variables|Checkpointsettings|GetRadius))
  (Rendering|Material|SetMaterial (Variables|Default|GetHitbox) 0 "/Game/Materials/CheckpointMaterial.CheckpointMaterial")
  (Transformation|SetActorScale3D (Math|Vector|MakeVector _radius _radius _radius))
  (Transformation|SetRelativeTransform (Variables|Default|GetArrow) (Variables|Checkpointsettings|GetKartOrientation) false))