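; Workshop pawn for building karts, switching input behavior between body select, kart editing and testdrive states.
; Body select cycles an index through available bodies, respawning the preview at VehicleLocation.
; Editing relays deadzone-filtered left-stick input to the WorkshopCursor found in the level; state changes notify it and the WorkshopController, while part attachment is only stubbed.
; The right stick orbits the camera around a handle using look-at rotation.
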(event EventBeginPlay
  (CallFunction|ChooseSelectedBody)
  (Variables|Default|SetcameraAngle (Transformation|GetActorRotation (Variables|Default|GetVehicleLocation))))

(event Input|GamepadEvents|GamepadRightY
  (params (AxisValue :type Float%20%28single-precision%29))
  (CallFunction|RotateCameraHandle (stale Input|GamepadEvents|GamepadRightX AxisValue) AxisValue))

(event Input|GamepadEvents|GamepadRightX
  (params (AxisValue :type Float%20%28single-precision%29))
  (CallFunction|RotateCameraHandle AxisValue (stale Input|GamepadEvents|GamepadRightY AxisValue)))

(event Input|GamepadEvents|GamepadLeftX
  (params (AxisValue :type Float%20%28single-precision%29))
  (|MoveCursor AxisValue (stale Input|GamepadEvents|GamepadLeftY AxisValue)))

(event Input|GamepadEvents|GamepadLeftY
  (params (AxisValue :type Float%20%28single-precision%29))
  (|MoveCursor (stale Input|GamepadEvents|GamepadLeftX AxisValue) AxisValue) ; enters at executeOnY
)

(event Input|KeyboardEvents|Left
  (:Pressed
    (Utilities|WorkshopState
      (:Kart%20Body%20Select
        (Variables|Default|SetMyBodyIndex (+ (Variables|Default|GetMyBodyIndex) 1))
        (CallFunction|ChooseSelectedBody)
        (Variables|Default|SetcameraAngle (Transformation|GetActorRotation (Variables|Default|GetVehicleLocation)))))))

(event Input|KeyboardEvents|Right
  (:Pressed
    (Utilities|WorkshopState
      (:Kart%20Body%20Select
        (Variables|Default|SetMyBodyIndex (- (Variables|Default|GetMyBodyIndex) 1))
        (CallFunction|ChooseSelectedBody)
        (Variables|Default|SetcameraAngle (Transformation|GetActorRotation (Variables|Default|GetVehicleLocation)))))))

(event Input|GamepadEvents|GamepadFaceButtonBottom
  (:Pressed
    (Utilities|WorkshopState
      (:Kart%20Body%20Select
        (CallFunction|ChooseSelectedBody)
        (CallFunction|SetState "NewEnumerator1"))
      (:Kart%20Editing
        (Utilities|FixParttoBody)))))

(event Input|KeyboardEvents|Enter
  (:Pressed
    (Utilities|WorkshopState
      (:Kart%20Body%20Select
        (CallFunction|ChooseSelectedBody)
        (CallFunction|SetState "NewEnumerator1"))
      (:Kart%20Editing
        (Utilities|FixParttoBody)))))

(event Input|GamepadEvents|GamepadFaceButtonRight
  (:Pressed
    (Utilities|WorkshopState
      (:Kart%20Editing
        (CallFunction|SetState "NewEnumerator0"))
      (:Testdrive
        (CallFunction|SetState "NewEnumerator1")))))

(event Input|KeyboardEvents|Backspace
  (:Pressed
    (Utilities|WorkshopState
      (:Kart%20Editing
        (CallFunction|SetState "NewEnumerator0"))
      (:Testdrive
        (CallFunction|SetState "NewEnumerator1")))))

(event Input|KeyboardEvents|Escape
  (:Pressed
    (Utilities|WorkshopState
      (:Kart%20Editing
        (CallFunction|SetState "NewEnumerator0"))
      (:Testdrive
        (CallFunction|SetState "NewEnumerator1")))))

(event Input|GamepadEvents|GamepadDPadLeft
  (:Pressed
    (Utilities|WorkshopState
      (:Kart%20Body%20Select
        (Variables|Default|SetMyBodyIndex (+ (Variables|Default|GetMyBodyIndex) 1))
        (CallFunction|ChooseSelectedBody)
        (Variables|Default|SetcameraAngle (Transformation|GetActorRotation (Variables|Default|GetVehicleLocation)))))))

(event Input|GamepadEvents|GamepadDPadRight
  (:Pressed
    (Utilities|WorkshopState
      (:Kart%20Body%20Select
        (Variables|Default|SetMyBodyIndex (- (Variables|Default|GetMyBodyIndex) 1))
        (CallFunction|ChooseSelectedBody)
        (Variables|Default|SetcameraAngle (Transformation|GetActorRotation (Variables|Default|GetVehicleLocation)))))))

(event Input|GamepadEvents|GamepadRightThumbstick
  (:Pressed
    (Transformation|SetRelativeRotation (Variables|Default|GetcameraHandle) "0, 0, 0" true)))

(event Input|GamepadEvents|GamepadDPadRight
  (:Pressed
    (Utilities|WorkshopState
      (:Kart%20Editing
        (bind _workshopcursor (Utilities|PerformonHud)
          (:then
            (Default|SetActiveVehiclePart _workshopcursor "/Game/Blueprints/Karts/TestVehicleCapsuleWheel.TestVehicleCapsuleWheel_C")))))))

(fn ConstructionScript)

(fn ChooseSelectedBody
  (Utilities|IsValid (Variables|Default|GetMyBody)
    (:Is%20Valid
      (Actor|DestroyActor (Variables|Default|GetMyBody))
      (Variables|Default|SetMyBody 0))
    (:Is%20Not%20Valid
      _))
  (CallFunction|NormalizeIndex)
  (bind _returnvalue (Game|SpawnActorfromClass (Utilities|Array|Get(acopy) (Variables|Default|GetAvailibleBodies) (Variables|Default|GetMyBodyIndex)) (Transformation|GetActorTransform (Variables|Default|GetVehicleLocation)) true))
  (bind _asvehiclebodybase (Utilities|Casting|CastToVehicleBodyBase _returnvalue)
    (:then
      (Variables|Default|SetMyBody _asvehiclebodybase))
    (:CastFailed
      (Development|PrintString (Utilities|String|ToString(Object) 0) true true "(R=1.000000,G=0.000000,B=0.066515,A=1.000000)"))))

(fn NormalizeIndex
  (if (< (Variables|Default|GetMyBodyIndex) 0)
    (Variables|Default|SetMyBodyIndex (- (Utilities|Array|Length (Variables|Default|GetAvailibleBodies)) 1))
    (else
      (Variables|Default|SetMyBodyIndex (Math|Integer|%(Integer) (Variables|Default|GetMyBodyIndex) (Utilities|Array|Length (Variables|Default|GetAvailibleBodies))))))
  (Development|PrintString (Utilities|String|ToString(Integer) (Variables|Default|GetMyBodyIndex)) true true "(R=0.000000,G=1.000000,B=0.325999,A=1.000000)"))

(fn SetState
  (params (newState :type WorkshopStateMachine%20Enum :default "NewEnumerator0"))
  (Variables|Default|SetState newState)
  (Utilities|FlowControl|Sequence
    (:then_0
      (bind _workshopcursor (Utilities|PerformonHud)
        (:then
          (Default|StateDidChange _workshopcursor (Variables|Default|GetState)))))
    (:then_1
      (bind _asworkshopcontroller_c (Utilities|Casting|CastToWorkshopController (Pawn|GetController)))
      (Default|StateDidChange _asworkshopcontroller_c (Variables|Default|GetState)))))

(fn RotateCameraHandle
  (params (LeftRight :type Float%20%28single-precision%29) (UpDown :type Float%20%28single-precision%29))
  (bind _camera (Variables|Camera|GetCamera))
  (Utilities|FlowControl|Sequence
    (:then_0
      (bind _scaledvalue (Utilities|ValueSmooth LeftRight 1.0))
      (Transformation|AddLocalRotation (Variables|Default|GetcameraHandle) (Math|Vector|RotatorfromAxisandAngle "0, 0,1.000000" _scaledvalue) true))
    (:then_1
      (bind _scaledvalue_2 (Utilities|ValueSmooth UpDown 1.0))
      (Transformation|AddLocalRotation (Variables|Default|GetcameraHandle) (Math|Vector|RotatorfromAxisandAngle "0,1.000000,0.000000" _scaledvalue_2) true))
    (:then_2
      (Transformation|SetWorldRotation _camera (Math|Rotator|FindLookatRotation (Transformation|GetWorldLocation _camera) (Transformation|GetWorldLocation (Variables|Default|GetcameraHandle))) false))))