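; Workshop workstation that spawns a selectable body actor at its VehicleAnchor transform, starting with the currently indexed body on BeginPlay.
; SelectNextBody shifts the index by a step count, wraps it with modulo over the PossibleBodies array, and spawns that entry.
; Spawned actors are neither stored nor destroyed here, so each selection issues a new spawn without removing the previous body.
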(event EventBeginPlay
  (CallFunction|SpawnSelectedBody))

(fn ConstructionScript)

(fn SpawnSelectedBody
  (Game|SpawnActorfromClass (Utilities|Array|Get(acopy) (Variables|Default|GetpossibleBodies) (Variables|Default|GetpossibleBodiesIndex)) (Transformation|GetWorldTransform (Variables|Default|GetvehicleAnchor)) false))

(fn SelectNextBody
  (params (stepCount :type Integer))
  (Variables|Default|SetpossibleBodiesIndex (Math|Integer|%(Integer) (+ stepCount (Variables|Default|GetpossibleBodiesIndex)) (Utilities|Array|Length (Variables|Default|GetpossibleBodies))))
  (CallFunction|SpawnSelectedBody))