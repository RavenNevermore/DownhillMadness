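; Workshop HUD that draws a virtual cursor for placing vehicle parts on a kart body.
; In one workshop state, DrawHUD converts the normalized, clamped cursor position to screen space, updates the active part, then tints and draws the cursor by body hit.
; SetActiveVehiclePart spawns a part and flags repositioning; the update hides it off the body or moves it to the hit point, with only wheels snapping through the body's SnapWheel.
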(event EventDrawHUD
  (params (SizeX :type Integer) (SizeY :type Integer))
  (if (Utilities|Enum|Equal(Enum) (Variables|Default|GetWorkshopState) "NewEnumerator1")
    (Utilities|FlowControl|Sequence
      (:then_1
        (CallFunction|UpdateCursorScreenPosition SizeX SizeY))
      (:then_2
        (CallFunction|UpdateActivePartPosition))
      (:then_3
        (CallFunction|TestCursorHit))
      (:then_4
        (CallFunction|DrawCursor)))))

(fn ConstructionScript)

(fn DrawCursor
  (bind _mycursorscreenposition (Variables|Default|GetMyCursorScreenPosition))
  (bind _cursorsize (Variables|Default|GetCursorSize))
  (bind (_x _y) (Math|Vector2D|BreakVector2D _mycursorscreenposition))
  (Canvas|DrawTexture "/Game/Textures/circledot.circledot" _x _y _cursorsize _cursorsize 0.0 0.0 1.0 1.0 (Variables|Default|GetCursorColor)))

(fn MoveCursor
  (params (x :type Float%20%28single-precision%29) (y :type Float%20%28single-precision%29))
  (bind _movementscale (Variables|Default|GetMovementScale))
  (Variables|Default|SetCursorPosition (Math|Vector2D|MakeVector2D (Math|Float|Max(Float) (Math|Float|Min(Float) (+ (* x _movementscale) (.X (Math|Vector2D|BreakVector2D (Variables|Default|GetCursorPosition)))) 1.0) 0.0) (Math|Float|Max(Float) (Math|Float|Min(Float) (+ (* y _movementscale) (.Y (Math|Vector2D|BreakVector2D (Variables|Default|GetCursorPosition)))) 1.0) 0.0))))

(fn DebugPrintCursorPos
  (bind _mycursorscreenposition (Variables|Default|GetMyCursorScreenPosition))
  (bind (_x _y) (Math|Vector2D|BreakVector2D _mycursorscreenposition))
  (Development|PrintString (Utilities|String|ToString(Text) (Utilities|Text|FormatText "" (Utilities|Text|ToText(Float) _x "HalfToEven") (Utilities|Text|ToText(Float) _y "HalfToEven")))))

(fn SetCursorActive
  (params (active :type Boolean))
  (if active
    (Variables|Default|SetCursorColor (Variables|Default|GetCursorColorActive))
    (else
      (Variables|Default|SetCursorColor (Variables|Default|GetCursorColorPassive)))))

(fn UpdateCursorScreenPosition
  (params (ScreenSizeX :type Integer) (ScreenSizeY :type Integer))
  (bind _cursorposition (Variables|Default|GetCursorPosition))
  (bind _cursorsize (Variables|Default|GetCursorSize))
  (bind _returnvalue (/ _cursorsize 2.0))
  (bind (_x _y) (Math|Vector2D|BreakVector2D _cursorposition))
  (Variables|Default|SetMyCursorScreenPosition (Math|Vector2D|MakeVector2D (+ _returnvalue (* (Math|Conversions|ToFloat(Integer) ScreenSizeX) _x)) (+ _returnvalue (* (Math|Conversions|ToFloat(Integer) ScreenSizeY) _y)))))

(fn TestCursorHit
  (bind _returnvalue (Class|WorkshopHudBase|CursorOverKartBody))
  (if _returnvalue
    (Variables|Default|SetCursorColor (Variables|Default|GetCursorColorActive))
    (else
      (Variables|Default|SetCursorColor (Variables|Default|GetCursorColorPassive)))))

(fn SetActiveVehiclePart
  (params (partClass :type Vehicle%20Part%20Base%20Class%20Reference))
  (bind _returnvalue (Game|SpawnActorfromClass partClass (Math|Transform|MakeTransform "0, 0, 0") true))
  (bind _asvehiclepartbase (Utilities|Casting|CastToVehiclePartBase _returnvalue))
  (Variables|Default|SetactivePart _asvehiclepartbase)
  (Variables|Default|SetneedsRepositioning true))

(fn UpdateActivePartPosition
  (if (Variables|Default|GetneedsRepositioning)
    (Utilities|IsValid (Variables|Default|GetactivePart)
      (:Is%20Valid
        (bind (_hit _returnvalue) (Class|WorkshopHudBase|CursorOverKartBody))
        (if _returnvalue
          (Rendering|SetActorHiddenInGame (Variables|Default|GetactivePart) false)
          (Transformation|SetActorLocation (Variables|Default|GetactivePart) (.Location (Collision|BreakHitResult _hit)) false)
          (bind _asvehiclebodybase (Utilities|Casting|CastToVehicleBodyBase (.HitActor (Collision|BreakHitResult _hit))))
          (bind _wheel (Utilities|ActivePartbyType)
            (:IsWheel
              (bind _newtransform (Class|VehicleBodyBase|SnapWheel _asvehiclebodybase _wheel))
              (Transformation|SetActorTransform (Variables|Default|GetactivePart) _newtransform)))
          (else
            (Rendering|SetActorHiddenInGame (Variables|Default|GetactivePart) true)))
        (Variables|Default|SetneedsRepositioning false)
        (return)))))

(fn RepositioningNeeded
  (Variables|Default|SetneedsRepositioning true))

(event Custom|StateDidChange
  (params (NewState :type WorkshopStateMachine%20Enum :default "NewEnumerator0"))
  (bind _returnvalue (Game|Player|GetOwningPlayerController))
  (bind (_locationx _locationy) (Game|Player|GetMousePosition _returnvalue))
  (Utilities|FlowControl|Sequence
    (:then_0
      (Variables|Default|SetCursorPosition "(X=0.500000,Y=0.500000)"))
    (:then_1
      (Variables|Default|SetMouseZeroPosition (Math|Vector2D|MakeVector2D _locationx _locationy)))
    (:then_2
      (Variables|Default|SetWorkshopState NewState))))