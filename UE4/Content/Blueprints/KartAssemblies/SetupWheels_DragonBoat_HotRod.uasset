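; Kart assembly Blueprint that, going by its name, holds a wheel setup for the DragonBoat HotRod kart.
; AttachTo attaches each actor in its Parts list to a given body actor, keeping relative offsets and using no socket, then returns the list.
; IsBodyValid accepts a body whose class is BodyClass or a child of it.
; The construction script is empty.
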(fn ConstructionScript)

(fn Attachto
  (params (Body :type Vehicle%20Body%20Base%20Object%20Reference))
  (for _array_element (Variables|Default|Getparts)
    (Class|Actor|AttachRootComponenttoActor _array_element Body "None" "KeepRelativeOffset"))
  (return (Variables|Default|Getparts)))

(fn IsBodyValid
  (params (Body :type Vehicle%20Body%20Base%20Object%20Reference))
  (bind _returnvalue (Utilities|GetClass Body))
  (bind _bodyclass (Variables|Default|GetbodyClass))
  (return (or (Utilities|ClassIsChildOf _returnvalue _bodyclass) (== _returnvalue _bodyclass))))