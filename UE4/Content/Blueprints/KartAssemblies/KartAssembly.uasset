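; KartAssembly is an actor that assembles a kart and lets its vehicle body be cycled forwards or backwards.
; It spawns DragonBoatBody at BeginPlay, and SetMyBody destroys the current body before spawning the new class at the Body component's transform.
; NextBody and PreviousBody pass the current class to FindNextBody, whose wrap-around Bodies lookup is left unused.
; NextWheels is an empty stub.
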(event EventBeginPlay
  (Utilities|SetMyBody "/Game/Blueprints/Karts/DragonBoatBody.DragonBoatBody_C"))

(fn ConstructionScript)

(fn NextBody
  (bind _asvehiclebodybase (CallFunction|ClassOfMyBody))
  (Utilities|FlowControl|Sequence
    (:then_0
      (Utilities|SetMyBody (Utilities|FindNextBody true _asvehiclebodybase)))
    (:then_1
      (return (Variables|Default|GetMyBody)))))

(fn ClassOfMyBody
  (bind _asvehiclebodybase (Utilities|Casting|CastToVehicleBodyBaseClass (Utilities|GetClass (Variables|Default|GetMyBody)))
    (:then
      _)
    (:CastFailed
      _))
  (return _asvehiclebodybase))

(fn PreviousBody
  (bind _asvehiclebodybase (CallFunction|ClassOfMyBody))
  (Utilities|FlowControl|Sequence
    (:then_0
      (Utilities|SetMyBody (Utilities|FindNextBody false _asvehiclebodybase)))
    (:then_1
      (return (Variables|Default|GetMyBody)))))

(fn NextWheels)