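; Test kart vehicle built on physics bodies and constraints, with left/right key steering.
; Key flags are read each Tick to pass a fixed positive, negative or zero steering angle to updaters for Wheel2 and Wheel3, along with their constraints and a shared relative transform.
; The camera collider chases a fixed world-space offset from the body by setting its linear velocity, rather than its position.
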(event EventTick
  (params (DeltaSeconds :type Float%20%28single-precision%29))
  (bind _wheel_3_updater (Variables|Default|GetWheel%203%20Updater))
  (bind _relative_wheel_transform (Variables|Default|GetRelative%20Wheel%20Transform))
  (bind _camera_collider (Variables|Default|GetCamera%20Collider))
  (bind _wheel_2_updater (Variables|Default|GetWheel%202%20Updater))
  (bind _wheel_2_constraint (Variables|Default|GetWheel%202%20Constraint))
  (bind _wheel_3_constraint (Variables|Default|GetWheel%203%20Constraint))
  (bind _wheel_2 (Variables|Default|GetWheel%202))
  (bind _wheel_3 (Variables|Default|GetWheel%203))
  (Physics|SetPhysicsLinearVelocity _camera_collider (* (- (+ (Transformation|GetWorldLocation (Variables|Default|GetBody)) "200.000000, 0,200.000000") (Transformation|GetWorldLocation _camera_collider)) 6e+01) false "None")
  (if (Variables|Default|GetRight%20Pressed)
    (Class|WheelConstraint|UpdateWheel _wheel_2_updater _wheel_2 _wheel_2_constraint _relative_wheel_transform 3e+01)
    (Class|WheelConstraint|UpdateWheel _wheel_3_updater _wheel_3 _wheel_3_constraint _relative_wheel_transform 3e+01)
    (elif (Variables|Default|GetLeft%20Pressed)
      (Class|WheelConstraint|UpdateWheel _wheel_2_updater _wheel_2 _wheel_2_constraint _relative_wheel_transform -3e+01)
      (Class|WheelConstraint|UpdateWheel _wheel_3_updater _wheel_3 _wheel_3_constraint _relative_wheel_transform -3e+01)
      (else
        (Class|WheelConstraint|UpdateWheel _wheel_2_updater _wheel_2 _wheel_2_constraint _relative_wheel_transform 0.0)
        (Class|WheelConstraint|UpdateWheel _wheel_3_updater _wheel_3 _wheel_3_constraint _relative_wheel_transform 0.0)))))

(event EventBeginPlay
  (Variables|Default|SetRelative%20Wheel%20Transform (Math|Transform|MakeTransform "0, 0, 0" "0, 0,90.000000")))

(event Input|KeyboardEvents|Left
  (:Pressed
    (Variables|Default|SetLeft%20Pressed true))
  (:Released
    (Variables|Default|SetLeft%20Pressed false)))

(event Input|KeyboardEvents|Right
  (:Pressed
    (Variables|Default|SetRight%20Pressed true))
  (:Released
    (Variables|Default|SetRight%20Pressed false)))

(fn ConstructionScript)