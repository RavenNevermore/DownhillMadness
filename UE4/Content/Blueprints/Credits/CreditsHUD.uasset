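; HUD that plays scrolling credits from two tall textures, Credit01 and Credit02, each drawn PagesPerScreen screen-heights tall.
; Tick advances Travel by Speed, measured in screen-heights, until the end of the second texture.
; DrawHUD scrolls by offsetting texture V, sliding Credit02 up from the bottom over Credit01's final screen.
; Credit02 then continues with V at or above one, which relies on texture wrapping.
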(event EventTick
  (params (DeltaSeconds :type Float%20%28single-precision%29))
  (if (<= (Variables|Default|GetTravel) (- (* (Variables|Default|GetpagesPerScreen) 2.0) 1.0))
    (Variables|Default|SetTravel (+ (* DeltaSeconds (Variables|Default|GetSpeed)) (Variables|Default|GetTravel)))))

(event EventDrawHUD
  (params (SizeX :type Integer) (SizeY :type Integer))
  (bind _returnvalue (Math|Conversions|ToFloat(Integer) SizeX))
  (bind _returnvalue_2 (Math|Conversions|ToFloat(Integer) SizeY))
  (bind _travel (Variables|Default|GetTravel))
  (bind _pagesperscreen (Variables|Default|GetpagesPerScreen))
  (bind _travel_2 (Variables|Default|GetTravel))
  (bind _pagesperscreen_2 (Variables|Default|GetpagesPerScreen))
  (bind _returnvalue_3 (/ _travel _pagesperscreen))
  (bind _returnvalue_4 (- _pagesperscreen_2 1.0))
  (bind _returnvalue_5 (* _returnvalue_2 _pagesperscreen))
  (bind _returnvalue_6 (>= _travel_2 _returnvalue_4))
  (Utilities|FlowControl|Sequence
    (:then_0
      (if (<= _returnvalue_3 1.0)
        (Canvas|DrawTexture "/Game/Textures/Credits/Credit01.Credit01" 0.0 0.0 _returnvalue _returnvalue_5 0.0 _returnvalue_3 1.0 1.0 "(R=1.000000,G=1.000000,B=1.000000,A=1.000000)")))
    (:then_1
      (if (and _returnvalue_6 (< _travel_2 _pagesperscreen_2))
        (Canvas|DrawTexture "/Game/Textures/Credits/Credit02.Credit02" 0.0 (* _returnvalue_2 (- 1.0 (- _travel_2 _returnvalue_4))) _returnvalue _returnvalue_5 0.0 0.0 1.0 1.0 "(R=1.000000,G=1.000000,B=1.000000,A=1.000000)")
        (elif _returnvalue_6
          (Canvas|DrawTexture "/Game/Textures/Credits/Credit02.Credit02" 0.0 0.0 _returnvalue _returnvalue_5 0.0 _returnvalue_3 1.0 1.0 "(R=1.000000,G=1.000000,B=1.000000,A=1.000000)"))))))

(fn ConstructionScript)