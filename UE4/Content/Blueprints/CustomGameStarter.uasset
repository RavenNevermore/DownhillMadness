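; CustomGameStarter is a Blueprint that builds the list of driver pawn classes, apparently for starting a custom game.
; SetArray assigns a class variable per named driver, then appends five entries to DriverClasses.
; Balder reuses the Loki pawn and Ratatosk the Skadi pawn.
; IdunClass is added twice, while LokiClass is set but never added; the construction script is empty.
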(fn ConstructionScript)

(fn SetArray
  (bind _driverclasses (Variables|Default|GetdriverClasses))
  (Variables|Default|SetBalderClass "/Game/Blueprints/Characters/LokiDriverPawn.LokiDriverPawn_C")
  (Variables|Default|SetIdunClass "/Game/Blueprints/Characters/IdunDriverPawn.IdunDriverPawn_C")
  (Variables|Default|SetSkadiClass "/Game/Blueprints/Characters/SkadiDriverPawn.SkadiDriverPawn_C")
  (Variables|Default|SetLokiClass "/Game/Blueprints/Characters/LokiDriverPawn.LokiDriverPawn_C")
  (Variables|Default|SetRatatoskClass "/Game/Blueprints/Characters/SkadiDriverPawn.SkadiDriverPawn_C")
  (Utilities|Array|Add _driverclasses (Variables|Default|GetBalderClass))
  (Utilities|Array|Add _driverclasses (Variables|Default|GetIdunClass))
  (Utilities|Array|Add _driverclasses (Variables|Default|GetSkadiClass))
  (Utilities|Array|Add _driverclasses (Variables|Default|GetIdunClass))
  (Utilities|Array|Add _driverclasses (Variables|Default|GetRatatoskClass)))