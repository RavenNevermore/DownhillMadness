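; Central sound driver that manages the driving audio of every VehicleBodyBase actor in the level.
; Each tick it finds all vehicles, assigns and plays the SoundCue on any audio component lacking a sound, and feeds it VehicleSpeed and TouchingGround parameters.
; An air-time array, keyed by each vehicle's index in the actor search, keeps TouchingGround true through brief airborne moments under a quarter second.
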(event EventTick
  (params (DeltaSeconds :type Float%20%28single-precision%29))
  (bind _outactors (Actor|GetAllActorsOfClass "/Script/DownhillMadness.VehicleBodyBase"))
  (for (_array_element _array_index) _outactors
    (Utilities|FlowControl|Sequence
      (:then_0
        (CallFunction|InitAirTime _array_index))
      (:then_1
        (bind _asvehiclebodybase (Utilities|Casting|CastToVehicleBodyBase _array_element))
        (Utilities|FlowControl|Sequence
          (:then_0
            (Utilities|IsValid (Variables|/Script/Engine.AudioComponent|GetSound (Variables|/Script/DownhillMadness.VehicleBodyBase|GetAudioComponent _asvehiclebodybase))
              (:Is%20Not%20Valid
                (Audio|Components|Audio|SetSound (Variables|/Script/DownhillMadness.VehicleBodyBase|GetAudioComponent _asvehiclebodybase) (Variables|Default|GetSoundCue))
                (Audio|Components|Audio|Play (Variables|/Script/DownhillMadness.VehicleBodyBase|GetAudioComponent _asvehiclebodybase) 0.0))))
          (:then_1
            (bind (_onground _currentspeed) (Class|VehicleBodyBase|GetAudioProperties _asvehiclebodybase))
            (Audio|Parameter|SetFloatParameter (Variables|/Script/DownhillMadness.VehicleBodyBase|GetAudioComponent _asvehiclebodybase) "VehicleSpeed" _currentspeed :!class /Script/Engine.AudioComponent)
            (if _onground
              (Variables|Default|SetCurrentAirTime 0.0)
              (else
                (Variables|Default|SetCurrentAirTime (+ (Variables|Default|GetCurrentAirTime) DeltaSeconds))))
            (Effects|Components|ParticleSystem|SetBoolParameter (Variables|/Script/DownhillMadness.VehicleBodyBase|GetAudioComponent _asvehiclebodybase) "TouchingGround" (< (Variables|Default|GetCurrentAirTime) 0.25)))))
      (:then_2
        (CallFunction|UpdateAirTime _array_index)))))

(fn ConstructionScript)

(fn InitAirTime
  (params (index :type Integer))
  (bind _airtimeclock (Variables|Default|GetAirTimeClock))
  (if (> index (Utilities|Array|LastIndex (Variables|Default|GetAirTimeClock)))
    (Utilities|Array|SetArrayElem _airtimeclock index 0.0 true)
    (Variables|Default|SetCurrentAirTime 0.0)
    (else
      (Variables|Default|SetCurrentAirTime (Utilities|Array|Get(acopy) _airtimeclock index)))))

(fn UpdateAirTime
  (params (index :type Integer))
  (Utilities|Array|SetArrayElem (Variables|Default|GetAirTimeClock) index (Variables|Default|GetCurrentAirTime) true))