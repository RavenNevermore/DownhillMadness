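; MenuSoundPlayer is a menu sound-effect actor for navigation, options, game and workshop starts, and selection of characters, vehicles and tracks.
; Each function plays one cue attached to its Audio component, with several actions sharing the same switch or start cue.
; CharacterSelected switches on a character enum to play a distinct sound for Balder, Idan, Loki, Ratatosk or Skadi.
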(fn ConstructionScript)

(fn CharacterSelected
  (params (character :type CharacterName%20Enum :default "NewEnumerator0"))
  (bind _audio (Variables|Default|GetAudio))
  (switch Utilities|FlowControl|Switch|SwitchonCharacterName character
    (:NewEnumerator0
      (Class|GameplayStatics|PlaySoundAttached "/Game/Sounds/voices/clues/CharacterSelected_Balder.CharacterSelected_Balder" _audio))
    (:NewEnumerator1
      (Class|GameplayStatics|PlaySoundAttached "/Game/Sounds/voices/clues/CharacterSelected_Idan.CharacterSelected_Idan" _audio))
    (:NewEnumerator2
      (Class|GameplayStatics|PlaySoundAttached "/Game/Sounds/voices/clues/CharacterSelected_Loki.CharacterSelected_Loki" _audio))
    (:NewEnumerator3
      (Class|GameplayStatics|PlaySoundAttached "/Game/Sounds/voices/clues/CharacterSelected_Ratatosk.CharacterSelected_Ratatosk" _audio))
    (:NewEnumerator4
      (Class|GameplayStatics|PlaySoundAttached "/Game/Sounds/voices/clues/CharacterSelected_Skadi.CharacterSelected_Skadi" _audio))))

(fn MainMenuUp
  (Class|GameplayStatics|PlaySoundAttached "/Game/Sounds/ui/select_up_Cue.select_up_Cue" (Variables|Default|GetAudio)))

(fn MainMenuDown
  (Class|GameplayStatics|PlaySoundAttached "/Game/Sounds/ui/select_down_Cue.select_down_Cue" (Variables|Default|GetAudio)))

(fn SwitchMenu
  (Class|GameplayStatics|PlaySoundAttached "/Game/Sounds/ui/menuswitch_Cue.menuswitch_Cue" (Variables|Default|GetAudio)))

(fn Optionschange
  (Class|GameplayStatics|PlaySoundAttached "/Game/Sounds/ui/slashclick_Cue.slashclick_Cue" (Variables|Default|GetAudio)))

(fn StartWorkshop
  (Class|GameplayStatics|PlaySoundAttached "/Game/Sounds/ui/startstuff_Cue.startstuff_Cue" (Variables|Default|GetAudio)))

(fn StartGame
  (Class|GameplayStatics|PlaySoundAttached "/Game/Sounds/ui/startstuff_Cue.startstuff_Cue" (Variables|Default|GetAudio)))

(fn SwitchThroughCharacters
  (Class|GameplayStatics|PlaySoundAttached "/Game/Sounds/ui/charselectswitch_Cue.charselectswitch_Cue" (Variables|Default|GetAudio)))

(fn SwitchThroughVehicles
  (Class|GameplayStatics|PlaySoundAttached "/Game/Sounds/ui/charselectswitch_Cue.charselectswitch_Cue" (Variables|Default|GetAudio)))

(fn SwitchThroughTracks
  (Class|GameplayStatics|PlaySoundAttached "/Game/Sounds/ui/charselectswitch_Cue.charselectswitch_Cue" (Variables|Default|GetAudio)))