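; Racing HUD that shows each player's controller icon, a speedometer, the race timer, a track progress bar with all players' markers, and the current rank.
; It reads the owning DriverPawn and the level's GameStarter, rotating the needle by capsule physics velocity.
; Elements scale from a 1920x1080 reference.
; DrawCustomString renders text from per-character textures with left, center or right alignment.
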(event EventDrawHUD
  (params (SizeX :type Integer) (SizeY :type Integer))
  (bind _returnvalue (Math|Conversions|ToFloat(Integer) SizeY))
  (bind _returnvalue_2 (Math|Conversions|ToFloat(Integer) SizeX))
  (bind _returnvalue_3 (Math|Conversions|ToFloat(Integer) SizeX))
  (bind _returnvalue_4 (Math|Conversions|ToFloat(Integer) SizeY))
  (bind _driverpawn (Variables|Default|GetDriverPawn))
  (bind _gamestarter (Variables|Default|GetGameStarter))
  (bind _returnvalue_5 (/ _returnvalue 1.08e+03))
  (bind _returnvalue_6 (/ _returnvalue_2 1.92e+03))
  (bind _returnvalue_7 (Math|Float|Min(Float) _returnvalue_6 _returnvalue_5))
  (bind _returnvalue_8 (* _returnvalue_7 3.8e+02))
  (bind _returnvalue_9 (* _returnvalue_7 3e+02))
  (bind _returnvalue_10 (- _returnvalue_3 _returnvalue_8))
  (bind _returnvalue_11 (- _returnvalue_4 _returnvalue_9))
  (if (!= _driverpawn 0)
    (Utilities|FlowControl|Sequence
      (:then_0
        (Canvas|DrawTexture (CallFunction|GetControllerTexture (Variables|/Script/DownhillMadness.DriverPawn|GetcontrollerIndex _driverpawn)) 5e+01 5e+01 1.5e+02 1.5e+02 0.0 0.0 1.0 1.0 "(R=1.000000,G=1.000000,B=1.000000,A=0.500000)" "BLEND_Translucent" _returnvalue_7 true))
      (:then_1
        (Canvas|DrawTexture "/Game/Textures/UI/Leiste.Leiste" 0.0 (- (Math|Conversions|ToFloat(Integer) SizeY) (* _returnvalue_7 1.7e+02)) 807.0 1.7e+02 0.0 0.0 1.0 1.0 "(R=1.000000,G=1.000000,B=1.000000,A=1.000000)" "BLEND_Translucent" _returnvalue_7)
        (Canvas|DrawTexture "/Game/Textures/UI/tacho.tacho" _returnvalue_10 _returnvalue_11 3.8e+02 3e+02 0.0 0.0 1.0 1.0 "(R=1.000000,G=1.000000,B=1.000000,A=1.000000)" "BLEND_Translucent" _returnvalue_7)
        (bind _returnvalue_12 (Physics|GetPhysicsLinearVelocity (Variables|/Script/DownhillMadness.DriverPawn|GetDriverCapsule (Variables|Default|GetDriverPawn)) "None"))
        (Canvas|DrawTexture "/Game/Textures/UI/zeiger_skaliert.zeiger_skaliert" _returnvalue_10 _returnvalue_11 3.8e+02 3e+02 0.0 0.0 1.0 1.0 "(R=1.000000,G=1.000000,B=1.000000,A=1.000000)" "BLEND_Translucent" _returnvalue_7 false (Math|Float|Lerp 0.0 135.0 (Math|Float|Clamp(Float) (/ (Math|Vector|VectorLength _returnvalue_12) 2.5e+03))) "(X=0.661404,Y=0.705100)")
        (if (!= _gamestarter 0)
          (bind _returnvalue_13 (Class|GameStateStatics|TrackTimetoString (Variables|/Script/DownhillMadness.GameStarter|GetcurrentRaceDuration _gamestarter)))
          (CallFunction|DrawCustomString _returnvalue_13 1e+02 (/ 1.92e+03 2.0) 5e+01 1 _returnvalue_6 true)
          (bind _returnvalue_14 (Class|GameStateStatics|GetNumberOfPlayers))
          (for _index (range 0 (- (Math|Conversions|ToInteger(Byte) _returnvalue_14) 1))
            (Canvas|DrawTexture (CallFunction|GetControllerTexture (Math|Conversions|ToByte(Integer) _index)) (* (+ (* (Utilities|Array|Get(acopy) (Variables|/Script/DownhillMadness.GameStarter|GetprogressArray _gamestarter) _index) 6e+02) 29.0) _returnvalue_7) (- (Math|Conversions|ToFloat(Integer) SizeY) (* _returnvalue_7 185.0)) 1e+02 1e+02 0.0 0.0 1.0 1.0 "(R=1.000000,G=1.000000,B=1.000000,A=0.500000)" "BLEND_Translucent" _returnvalue_7))
          (bind _returnvalue_15 (Class|GameStateStatics|GetNumberOfPlayers))
          (CallFunction|DrawCustomString (Utilities|String|Append (Utilities|String|Append (Utilities|String|ToString(Integer) (+ (Utilities|Array|FindItem (Variables|/Script/DownhillMadness.GameStarter|GetrankingArray _gamestarter) (Variables|/Script/DownhillMadness.DriverPawn|GetcontrollerIndex (Variables|Default|GetDriverPawn))) 1)) "/") (Utilities|String|ToString(Byte) _returnvalue_15)) 1.5e+02 (- (Math|Conversions|ToFloat(Integer) SizeX) (* _returnvalue_7 5e+01)) (* _returnvalue_7 5e+01) 2 _returnvalue_7 false))))))

(event EventBeginPlay
  (Variables|Default|SetGameStarterClass "/Game/Blueprints/CustomGameStarter.CustomGameStarter_C")
  (bind _returnvalue (Class|GameStateStatics|FindActorsOfType (Variables|Default|GetGameStarterClass)))
  (if (> (Utilities|Array|Length _returnvalue) 0)
    (bind _asgamestarter (Utilities|Casting|CastToGameStarter (Utilities|Array|Get(acopy) _returnvalue))
      (:then
        (Variables|Default|SetGameStarter _asgamestarter))
      (:CastFailed
        (bind _asdriverpawn (Utilities|Casting|CastToDriverPawn (Class|HUD|GetOwningPawn) :!label _label))
        (Variables|Default|SetDriverPawn _asdriverpawn)))
    (else
      (goto _label))))

(event EventTick
  (params (DeltaSeconds :type Float%20%28single-precision%29))
  (if (== (Variables|Default|GetDriverPawn) 0)
    (bind _asdriverpawn (Utilities|Casting|CastToDriverPawn (Class|HUD|GetOwningPawn)))
    (Variables|Default|SetDriverPawn _asdriverpawn)))

(fn ConstructionScript)

(fn DrawCustomString
  (params (InString :type String) (Height :type Float%20%28single-precision%29) (X%20Pos :type Float%20%28single-precision%29) (Y%20Pos :type Float%20%28single-precision%29) (Allign :type Byte) (Scale :type Float%20%28single-precision%29) (Scale%20Position :type Boolean))
  (bind _returnvalue (* X%20Pos Scale))
  (bind _returnvalue_2 (* Height Scale))
  (bind _variable (|LocalVariable))
  (bind _variable_2 (|LocalVariable))
  (bind _variable_3 (|LocalVariable))
  (|Assign _variable 0.0)
  (for _index (range 0 (- (Utilities|String|Len InString) 1))
    (|Assign _variable (+ _variable (* (Math|Conversions|ToFloat(Integer) (Class|Texture2D|BlueprintGetSizeX (CallFunction|GetCharacterTexture (Utilities|String|GetSubstring InString _index)))) (/ _returnvalue_2 (Math|Conversions|ToFloat(Integer) (Class|Texture2D|BlueprintGetSizeY (CallFunction|GetCharacterTexture (Utilities|String|GetSubstring InString _index)))))))))
  (if Scale%20Position
    (|Assign _variable_3 (* Y%20Pos Scale))
    (else
      (|Assign _variable_3 Y%20Pos)))
  (if Scale%20Position
    (switch int (Math|Conversions|ToInteger(Byte) Allign)
      (:0
        (|Assign _variable_2 _returnvalue))
      (:1
        (|Assign _variable_2 (- _returnvalue (/ _variable 2.0))))
      (:2
        (|Assign _variable_2 (- _returnvalue _variable))))
    (else
      (switch int (Math|Conversions|ToInteger(Byte) Allign)
        (:0
          (|Assign _variable_2 X%20Pos))
        (:1
          (|Assign _variable_2 (- X%20Pos (/ _variable 2.0))))
        (:2
          (|Assign _variable_2 (- X%20Pos _variable))))))
  (for _index_2 (range 0 (- (Utilities|String|Len InString) 1))
    (Canvas|DrawTexture (CallFunction|GetCharacterTexture (Utilities|String|GetSubstring InString _index_2)) _variable_2 _variable_3 (* (Math|Conversions|ToFloat(Integer) (Class|Texture2D|BlueprintGetSizeX (CallFunction|GetCharacterTexture (Utilities|String|GetSubstring InString _index_2)))) (/ _returnvalue_2 (Math|Conversions|ToFloat(Integer) (Class|Texture2D|BlueprintGetSizeY (CallFunction|GetCharacterTexture (Utilities|String|GetSubstring InString _index_2)))))) _returnvalue_2 0.0 0.0 1.0 1.0 "(R=1.000000,G=1.000000,B=1.000000,A=1.000000)")
    (|Assign _variable_2 (+ _variable_2 (* (Math|Conversions|ToFloat(Integer) (Class|Texture2D|BlueprintGetSizeX (CallFunction|GetCharacterTexture (Utilities|String|GetSubstring InString _index_2)))) (/ _returnvalue_2 (Math|Conversions|ToFloat(Integer) (Class|Texture2D|BlueprintGetSizeY (CallFunction|GetCharacterTexture (Utilities|String|GetSubstring InString _index_2))))))))))

(fn GetCharacterTexture
  (params (Character :type String))
  (bind _variable (|LocalVariable))
  (switch string Character
    (:0
      (|Assign _variable "/Game/Textures/UI/0.0"))
    (:1
      (|Assign _variable "/Game/Textures/UI/1.1"))
    (:2
      (|Assign _variable "/Game/Textures/UI/2.2"))
    (:3
      (|Assign _variable "/Game/Textures/UI/3.3"))
    (:4
      (|Assign _variable "/Game/Textures/UI/4.4"))
    (:5
      (|Assign _variable "/Game/Textures/UI/5.5"))
    (:6
      (|Assign _variable "/Game/Textures/UI/6.6"))
    (:7
      (|Assign _variable "/Game/Textures/UI/7.7"))
    (:8
      (|Assign _variable "/Game/Textures/UI/8.8"))
    (:9
      (|Assign _variable "/Game/Textures/UI/9.9"))
    (:/
      (|Assign _variable "/Game/Textures/UI/slash.Slash"))
    (::
      (|Assign _variable "/Game/Textures/UI/colon.colon"))
    (:,
      (|Assign _variable "/Game/Textures/UI/comma.Comma"))
    (:.
      (|Assign _variable "/Game/Textures/UI/period.Period")))
  (return _variable))

(fn GetControllerTexture
  (params (ControllerIndex :type Byte))
  (bind _variable (|LocalVariable))
  (switch int (Math|Conversions|ToInteger(Byte) ControllerIndex)
    (:Default
      (|Assign _variable "/Game/Textures/Menu_Main/Menu_PlayerIndicator_P1_TEX.Menu_PlayerIndicator_P1_TEX" :!label _label))
    (:0
      (goto _label))
    (:1
      (|Assign _variable "/Game/Textures/Menu_Main/Menu_PlayerIndicator_P2_TEX.Menu_PlayerIndicator_P2_TEX"))
    (:2
      (|Assign _variable "/Game/Textures/Menu_Main/Menu_PlayerIndicator_P3_TEX.Menu_PlayerIndicator_P3_TEX"))
    (:3
      (|Assign _variable "/Game/Textures/Menu_Main/Menu_PlayerIndicator_P4_TEX.Menu_PlayerIndicator_P4_TEX")))
  (return _variable))