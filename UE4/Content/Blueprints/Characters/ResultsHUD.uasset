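; HUD for the race results screen, drawn on canvas each frame from the owning ResultsPawn.
; When the race is over it lists ranked rows of controller indicator, position and recorded time with a return prompt; otherwise it shows the player's indicator, time and, in multiplayer, rank.
; DrawCustomString renders digits and time punctuation as per-character textures with left, center or right alignment.
; Layout scales from a 1920x1080 reference to the viewport.
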(event EventDrawHUD
  (params (SizeX :type Integer) (SizeY :type Integer))
  (bind _returnvalue (Math|Conversions|ToFloat(Integer) SizeY))
  (bind _returnvalue_2 (Math|Conversions|ToFloat(Integer) SizeX))
  (bind _returnvalue_3 (/ _returnvalue 1.08e+03))
  (bind _returnvalue_4 (/ _returnvalue_2 1.92e+03))
  (bind _returnvalue_5 (* 9.6e+02 _returnvalue_4))
  (bind _returnvalue_6 (Math|Float|Min(Float) _returnvalue_4 _returnvalue_3))
  (bind _asresultspawn (Utilities|Casting|CastToResultsPawn (Class|HUD|GetOwningPawn)))
  (if (Variables|/Script/DownhillMadness.ResultsPawn|GetraceOver _asresultspawn)
    (bind _returnvalue_7 (Class|GameStateStatics|GetNumberOfPlayers))
    (Variables|Default|SetYPos (* 1.5e+02 _returnvalue_3))
    (for _index (range 0 (Math|Conversions|ToInteger(Byte) (- _returnvalue_7 1)))
      (Canvas|DrawTexture (CallFunction|GetControllerTexture (Utilities|Array|Get(acopy) (Variables|/Script/DownhillMadness.ResultsPawn|GetrankingArray _asresultspawn) _index)) (- (* 9.6e+02 _returnvalue_4) (* 7.5e+02 _returnvalue_6)) (Variables|Default|GetYPos) 1.5e+02 1.5e+02 0.0 0.0 1.0 1.0 "(R=1.000000,G=1.000000,B=1.000000,A=0.500000)" "BLEND_Translucent" _returnvalue_6)
      (CallFunction|DrawCustomString (Utilities|String|Append (Utilities|String|Append (Utilities|String|ToString(Integer) (+ _index 1)) "/") (Utilities|String|ToString(Byte) _returnvalue_7)) 1.5e+02 (- (* 9.6e+02 _returnvalue_4) (* 375.0 _returnvalue_6)) (Variables|Default|GetYPos) 1 _returnvalue_6 false)
      (if (or (== _returnvalue_7 1) (< _index (Math|Conversions|ToInteger(Byte) (- _returnvalue_7 1))))
        (bind _returnvalue_8 (Class|GameStateStatics|TrackTimetoString (Utilities|Array|Get(acopy) (Variables|/Script/DownhillMadness.ResultsPawn|GetrecordsArray _asresultspawn) _index)))
        (CallFunction|DrawCustomString _returnvalue_8 1.5e+02 (+ (* 9.6e+02 _returnvalue_4) (* 3e+02 _returnvalue_6)) (Variables|Default|GetYPos) 1 _returnvalue_6 false))
      (Variables|Default|SetYPos (+ (Variables|Default|GetYPos) (* 2e+02 _returnvalue_6))))
    (HUD|DrawText "Press     to return" "(R=1.000000,G=1.000000,B=1.000000,A=1.000000)" (- (* 9.6e+02 _returnvalue_4) (* (.OutWidth (Class|HUD|GetTextSize "Press     to return" "/Game/Textures/Menu_Main/Font_Harrington_TEX.Font_Harrington_TEX" _returnvalue_6)) 0.5)) (Variables|Default|GetYPos) "/Game/Textures/Menu_Main/Font_Harrington_TEX.Font_Harrington_TEX" _returnvalue_6 false)
    (Canvas|DrawTexture "/Game/Textures/AnotherWorkshop/Xbox_Sprites/Button_A_TEX.Button_A_TEX" (- (* 9.6e+02 _returnvalue_4) (* 55.0 _returnvalue_6)) (Variables|Default|GetYPos) 5e+01 5e+01 0.0 0.0 1.0 1.0 "(R=1.000000,G=1.000000,B=1.000000,A=1.000000)" "BLEND_Translucent" _returnvalue_6)
    (else
      (bind _returnvalue_9 (Class|GameStateStatics|GetNumberOfPlayers))
      (bind _returnvalue_10 (Class|GameStateStatics|TrackTimetoString (Variables|/Script/DownhillMadness.ResultsPawn|GetplayerTime _asresultspawn)))
      (Canvas|DrawTexture (CallFunction|GetControllerTexture (Variables|/Script/DownhillMadness.ResultsPawn|GetcontrollerIndex _asresultspawn)) 5e+01 5e+01 1.5e+02 1.5e+02 0.0 0.0 1.0 1.0 "(R=1.000000,G=1.000000,B=1.000000,A=0.500000)" "BLEND_Translucent" _returnvalue_6 true)
      (CallFunction|DrawCustomString _returnvalue_10 2e+02 _returnvalue_5 (* 6.9e+02 _returnvalue_3) 1 _returnvalue_6 false)
      (if (> _returnvalue_9 1)
        (CallFunction|DrawCustomString (Utilities|String|Append (Utilities|String|Append (Utilities|String|ToString(Byte) (+ (Variables|/Script/DownhillMadness.ResultsPawn|Getranking _asresultspawn) 1)) "/") (Utilities|String|ToString(Byte) _returnvalue_9)) 3e+02 _returnvalue_5 (* 2.4e+02 _returnvalue_3) 1 _returnvalue_6 false)))))

(fn ConstructionScript)

(fn GetControllerTexture
  (params (ControllerIndex :type Byte))
  (bind _variable (|LocalVariable))
  (switch int (Math|Conversions|ToInteger(Byte) ControllerIndex)
    (:Default
      (|Assign _variable "/Game/Textures/Menu_Main/Menu_PlayerIndicator_P1_TEX.Menu_PlayerIndicator_P1_TEX" :!label _label))
    (:0
      (goto _label))
    (:1
      (|Assign _variable "/Game/Textures/Menu_Main/Menu_PlayerIndicator_P2_TEX.Menu_PlayerIndicator_P2_TEX"))
    (:2
      (|Assign _variable "/Game/Textures/Menu_Main/Menu_PlayerIndicator_P3_TEX.Menu_PlayerIndicator_P3_TEX"))
    (:3
      (|Assign _variable "/Game/Textures/Menu_Main/Menu_PlayerIndicator_P4_TEX.Menu_PlayerIndicator_P4_TEX")))
  (return _variable))

(fn GetCharacterTexture
  (params (Character :type String))
  (bind _variable (|LocalVariable))
  (switch string Character
    (:0
      (|Assign _variable "/Game/Textures/UI/0.0"))
    (:1
      (|Assign _variable "/Game/Textures/UI/1.1"))
    (:2
      (|Assign _variable "/Game/Textures/UI/2.2"))
    (:3
      (|Assign _variable "/Game/Textures/UI/3.3"))
    (:4
      (|Assign _variable "/Game/Textures/UI/4.4"))
    (:5
      (|Assign _variable "/Game/Textures/UI/5.5"))
    (:6
      (|Assign _variable "/Game/Textures/UI/6.6"))
    (:7
      (|Assign _variable "/Game/Textures/UI/7.7"))
    (:8
      (|Assign _variable "/Game/Textures/UI/8.8"))
    (:9
      (|Assign _variable "/Game/Textures/UI/9.9"))
    (:/
      (|Assign _variable "/Game/Textures/UI/slash.Slash"))
    (::
      (|Assign _variable "/Game/Textures/UI/colon.colon"))
    (:,
      (|Assign _variable "/Game/Textures/UI/comma.Comma"))
    (:.
      (|Assign _variable "/Game/Textures/UI/period.Period")))
  (return _variable))

(fn DrawCustomString
  (params (InString :type String) (Height :type Float%20%28single-precision%29) (X%20Pos :type Float%20%28single-precision%29) (Y%20Pos :type Float%20%28single-precision%29) (Allign :type Byte) (Scale :type Float%20%28single-precision%29) (Scale%20Position :type Boolean))
  (bind _returnvalue (* X%20Pos Scale))
  (bind _returnvalue_2 (* Height Scale))
  (bind _variable (|LocalVariable))
  (bind _variable_2 (|LocalVariable))
  (bind _variable_3 (|LocalVariable))
  (|Assign _variable 0.0)
  (for _index (range 0 (- (Utilities|String|Len InString) 1))
    (|Assign _variable (+ _variable (* (Math|Conversions|ToFloat(Integer) (Class|Texture2D|BlueprintGetSizeX (CallFunction|GetCharacterTexture (Utilities|String|GetSubstring InString _index)))) (/ _returnvalue_2 (Math|Conversions|ToFloat(Integer) (Class|Texture2D|BlueprintGetSizeY (CallFunction|GetCharacterTexture (Utilities|String|GetSubstring InString _index)))))))))
  (if Scale%20Position
    (|Assign _variable_3 (* Y%20Pos Scale))
    (else
      (|Assign _variable_3 Y%20Pos)))
  (if Scale%20Position
    (switch int (Math|Conversions|ToInteger(Byte) Allign)
      (:0
        (|Assign _variable_2 _returnvalue))
      (:1
        (|Assign _variable_2 (- _returnvalue (/ _variable 2.0))))
      (:2
        (|Assign _variable_2 (- _returnvalue _variable))))
    (else
      (switch int (Math|Conversions|ToInteger(Byte) Allign)
        (:0
          (|Assign _variable_2 X%20Pos))
        (:1
          (|Assign _variable_2 (- X%20Pos (/ _variable 2.0))))
        (:2
          (|Assign _variable_2 (- X%20Pos _variable))))))
  (for _index_2 (range 0 (- (Utilities|String|Len InString) 1))
    (Canvas|DrawTexture (CallFunction|GetCharacterTexture (Utilities|String|GetSubstring InString _index_2)) _variable_2 _variable_3 (* (Math|Conversions|ToFloat(Integer) (Class|Texture2D|BlueprintGetSizeX (CallFunction|GetCharacterTexture (Utilities|String|GetSubstring InString _index_2)))) (/ _returnvalue_2 (Math|Conversions|ToFloat(Integer) (Class|Texture2D|BlueprintGetSizeY (CallFunction|GetCharacterTexture (Utilities|String|GetSubstring InString _index_2)))))) _returnvalue_2 0.0 0.0 1.0 1.0 "(R=1.000000,G=1.000000,B=1.000000,A=1.000000)")
    (|Assign _variable_2 (+ _variable_2 (* (Math|Conversions|ToFloat(Integer) (Class|Texture2D|BlueprintGetSizeX (CallFunction|GetCharacterTexture (Utilities|String|GetSubstring InString _index_2)))) (/ _returnvalue_2 (Math|Conversions|ToFloat(Integer) (Class|Texture2D|BlueprintGetSizeY (CallFunction|GetCharacterTexture (Utilities|String|GetSubstring InString _index_2))))))))))