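; TestVehicle is a test vehicle Blueprint with a body, four wheels, physics constraints and a spring arm.
; Tick keeps the spring arm at a world offset from the body and snaps Wheel2, Wheel3 and their constraints to a fixed steering angle from Left/Right key flags.
; The left branch omits PhysicsConstraint2, unlike the right and neutral branches.
; Each wheel's hit event draws its impact normal as a colour-coded debug line.
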(event OnComponentHit(Wheel1)
  (params (OtherActor :type Actor%20Object%20Reference) (OtherComp :type Primitive%20Component%20Object%20Reference) (NormalImpulse :type Vector) (Hit :type Hit%20Result%20Structure%20%28by%20ref%29))
  (bind (_location _normal) (Collision|BreakHitResult Hit))
  (Rendering|Debug|DrawDebugLine _location (+ _location (* _normal 25.0)) "(R=0.585000,G=0.000000,B=0.398915,A=1.000000)" 5.0 2.0))

(event OnComponentHit(Wheel4)
  (params (OtherActor :type Actor%20Object%20Reference) (OtherComp :type Primitive%20Component%20Object%20Reference) (NormalImpulse :type Vector) (Hit :type Hit%20Result%20Structure%20%28by%20ref%29))
  (bind (_location _normal) (Collision|BreakHitResult Hit))
  (Rendering|Debug|DrawDebugLine _location (+ _location (* _normal 25.0)) "(R=0.000000,G=0.585000,B=0.062958,A=1.000000)" 5.0 2.0))

(event OnComponentHit(Wheel2)
  (params (OtherActor :type Actor%20Object%20Reference) (OtherComp :type Primitive%20Component%20Object%20Reference) (NormalImpulse :type Vector) (Hit :type Hit%20Result%20Structure%20%28by%20ref%29))
  (bind (_location _normal) (Collision|BreakHitResult Hit))
  (Rendering|Debug|DrawDebugLine _location (+ _location (* _normal 25.0)) "(R=0.022749,G=0.000000,B=0.585000,A=1.000000)" 5.0 2.0))

(event OnComponentHit(Wheel3)
  (params (OtherActor :type Actor%20Object%20Reference) (OtherComp :type Primitive%20Component%20Object%20Reference) (NormalImpulse :type Vector) (Hit :type Hit%20Result%20Structure%20%28by%20ref%29))
  (bind (_location _normal) (Collision|BreakHitResult Hit))
  (Rendering|Debug|DrawDebugLine _location (+ _location (* _normal 25.0)) "(R=0.000000,G=0.556891,B=0.585000,A=1.000000)" 5.0 2.0))

(event EventTick
  (params (DeltaSeconds :type Float%20%28single-precision%29))
  (bind _physicsconstraint3 (Variables|Default|GetPhysicsConstraint3))
  (Transformation|SetWorldLocation (Variables|Default|GetSpringArm1) (+ (Transformation|GetWorldLocation (Variables|Default|GetBody)) "25.000000, 0,65.000000") false)
  (if (Variables|Default|GetRight%20Pressed)
    (Transformation|SetRelativeRotation _physicsconstraint3 "0,30.000000, 0" false)
    (elif (Variables|Default|GetLeft%20Pressed)
      (Transformation|SetRelativeRotation _physicsconstraint3 "0,-30.000000, 0" false)
      (else
        (Transformation|SetRelativeRotation _physicsconstraint3 "0,0.000000, 0" false)))))

(event Input|KeyboardEvents|Left
  (:Pressed
    (Variables|Default|SetLeft%20Pressed true))
  (:Released
    (Variables|Default|SetLeft%20Pressed false)))

(event Input|KeyboardEvents|Right
  (:Pressed
    (Variables|Default|SetRight%20Pressed true))
  (:Released
    (Variables|Default|SetRight%20Pressed false)))

(fn ConstructionScript)