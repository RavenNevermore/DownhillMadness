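; Starting line Blueprint that opens a race barrier shortly after play begins.
; Tick accumulates elapsed time and, after a two-second delay, plays the door-open sound once at the volume from the game options.
; From then on, Tick slides the Barrier component down at a constant, frame-rate-independent speed, without sweeping, until it passes its lowered height limit.
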(event EventTick
  (params (DeltaSeconds :type Float%20%28single-precision%29))
  (bind _barrier (Variables|Default|GetBarrier))
  (bind _audio (Variables|Default|GetAudio))
  (bind _relativelocation (Variables|/Script/Engine.SceneComponent|GetRelativeLocation _barrier))
  (bind (_x _y _z) (Math|Vector|BreakVector _relativelocation))
  (Variables|Default|SetTotalTime (+ DeltaSeconds (Variables|Default|GetTotalTime)))
  (if (> (Variables|Default|GetTotalTime) 2.0)
    (Utilities|FlowControl|Sequence
      (:then_0
        (if (Variables|Default|GetfirstTick)
          (Variables|Default|SetfirstTick false)
          (bind _soundvolume (Class|GameStateStatics|GetGameOptions))
          (Audio|Components|Audio|SetVolumeMultiplier _audio _soundvolume :!class /Script/Engine.AudioComponent)
          (Variables|/Script/Engine.AudioComponent|SetSound _audio "/Game/Sounds/RaceDoorOpen.RaceDoorOpen")
          (Audio|Components|Audio|Play _audio 0.0)))
      (:then_1
        (if (> _z -3.9e+02)
          (Transformation|SetRelativeLocation _barrier (Math|Vector|MakeVector _x _y (+ _z (* DeltaSeconds -234.0))) false))))))

(fn ConstructionScript)