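; Main menu controller that drives five 3D buttons: Start, Options, Highscores, Credits and Exit.
; Keyboard and gamepad input cycles a wrapping selection index and calls the selected button's press event.
; Tick eases each button's scale and light glow toward the selection.
; Show/Hide functions set flags that Tick turns into timeline-driven vertical slides with lights zeroed, suppressing input from hide until show finishes.
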(event EventBeginPlay
  ;[1 1 1] Init
  (Variables|Default|SetSelected_Button_INDX 0)
  (Variables|Default|SetButton_Start_Scale "1.000000,1.000000,1.000000")
  (Variables|Default|SetButton_Credits_Scale "1.000000,1.000000,1.000000")
  (Variables|Default|SetButton_Highscores_Scale "1.000000,1.000000,1.000000")
  (Variables|Default|SetButton_Options_Scale "1.000000,1.000000,1.000000")
  (Variables|Default|SetButton_Exit_Scale "1.000000,1.000000,1.000000")
  (Variables|Default|SetButton_Start_Lerp 0.0)
  (Variables|Default|SetButton_Credits_Lerp 0.0)
  (Variables|Default|SetButton_Highscores_Lerp 0.0)
  (Variables|Default|SetButton_Options_Lerp 0.0)
  (Variables|Default|SetButton_Exit_Lerp 0.0)
  (Variables|Default|SetFadeIn_Learp 0.0)
  (Variables|Default|SetFadeOff_Learp 0.0)
  (Variables|Default|SetFadeOff_InProgress false)
  (Variables|Default|SetFadeIn_InProgress false)
  (Variables|Default|SetFadeOff_InProgress false))

(event EventTick
  (params (DeltaSeconds :type Float%20%28single-precision%29))
  (bind _selected_button_indx (Variables|Default|GetSelected_Button_INDX))
  ;[1 1 1] Update delta time
  (Variables|Default|SetDeltaTime (+ DeltaSeconds (Variables|Default|GetDeltaTime)))
  (Utilities|FlowControl|Sequence
    (:then_0
      ;[1 1 1] Input focus management
      (if true
        (Utilities|FlowControl|Sequence
          (:then_0
            (Utilities|FlowControl|DoOnce false :!label _label
              (:Completed
                (Input|EnableInput (Game|GetPlayerController 0)))))
          (:then_1
            (goto _label_2 Reset)))
        (else
          (Utilities|FlowControl|Sequence
            (:then_0
              (Utilities|FlowControl|DoOnce false :!label _label_2
                (:Completed
                  (Input|DisableInput (Game|GetPlayerController 0)))))
            (:then_1
              (goto _label Reset))))))
    (:then_1
      ;[1 1 1] Show / Hide Buttons animation
      (if (Variables|Default|GetFadeOff_InProgress)
        (Utilities|FlowControl|DoOnce false :!label _label_3
          (:Completed
            (Utilities|FlowControl|Sequence
              (:then_0
                (bind _returnvalue (Transformation|GetRelativeTransform (Variables|Default|GetButton_Start) :!label _label_4))
                (bind _returnvalue_2 (Transformation|GetRelativeTransform (Variables|Default|GetButton_Options)))
                (bind _returnvalue_3 (Transformation|GetRelativeTransform (Variables|Default|GetButton_Highscores)))
                (bind _returnvalue_4 (Transformation|GetRelativeTransform (Variables|Default|GetButton_Credits)))
                (bind _returnvalue_5 (Transformation|GetRelativeTransform (Variables|Default|GetButton_Exit))))
              (:then_1
                ;[1 1 1] Shutdown lights
                (Class|LightComponent|SetBrightness (Variables|Rendering|GetButton_Start_Light) 0.0 :!label _label_5)
                (Class|LightComponent|SetBrightness (Variables|Rendering|GetButton_Options_Light) 0.0)
                (Class|LightComponent|SetBrightness (Variables|Rendering|GetButton_Highscores_Light) 0.0)
                (Class|LightComponent|SetBrightness (Variables|Rendering|GetButton_Credits_Light) 0.0)
                (Class|LightComponent|SetBrightness (Variables|Rendering|GetButton_Exit_Light) 0.0))
              (:then_2
                (Variables|Default|SetSuppress_Input true)
                (bind (_direction _track_e1_hide _track_e1_show _track_e2_hide _track_e2_show _track_e3_hide _track_e3_show _track_e4_hide _track_e4_show _track_e5_hide) (Timeline|Timeline_0 PlayFromStart)
                  (:Update
                    (Transformation|SetRelativeLocation (Variables|Default|GetButton_Start) (Math|Vector|MakeVector (.X (Math|Vector|BreakVector (.Location (Math|Transform|BreakTransform _returnvalue)))) (.Y (Math|Vector|BreakVector (.Location (Math|Transform|BreakTransform _returnvalue)))) (Math|Float|Lerp (.Z (Math|Vector|BreakVector (.Location (Math|Transform|BreakTransform _returnvalue)))) 4.8e+02 _track_e1_hide)) false)
                    (Transformation|SetRelativeLocation (Variables|Default|GetButton_Options) (Math|Vector|MakeVector (.X (Math|Vector|BreakVector (.Location (Math|Transform|BreakTransform _returnvalue_2)))) (.Y (Math|Vector|BreakVector (.Location (Math|Transform|BreakTransform _returnvalue_2)))) (Math|Float|Lerp (.Z (Math|Vector|BreakVector (.Location (Math|Transform|BreakTransform _returnvalue_2)))) 4.1e+02 _track_e2_hide)) false)
                    (Transformation|SetRelativeLocation (Variables|Default|GetButton_Highscores) (Math|Vector|MakeVector (.X (Math|Vector|BreakVector (.Location (Math|Transform|BreakTransform _returnvalue_3)))) (.Y (Math|Vector|BreakVector (.Location (Math|Transform|BreakTransform _returnvalue_3)))) (Math|Float|Lerp (.Z (Math|Vector|BreakVector (.Location (Math|Transform|BreakTransform _returnvalue_3)))) 3.4e+02 _track_e3_hide)) false)
                    (Transformation|SetRelativeLocation (Variables|Default|GetButton_Credits) (Math|Vector|MakeVector (.X (Math|Vector|BreakVector (.Location (Math|Transform|BreakTransform _returnvalue_4)))) (.Y (Math|Vector|BreakVector (.Location (Math|Transform|BreakTransform _returnvalue_4)))) (Math|Float|Lerp (.Z (Math|Vector|BreakVector (.Location (Math|Transform|BreakTransform _returnvalue_4)))) 2.7e+02 _track_e4_hide)) false)
                    (Transformation|SetRelativeLocation (Variables|Default|GetButton_Exit) (Math|Vector|MakeVector (.X (Math|Vector|BreakVector (.Location (Math|Transform|BreakTransform _returnvalue_5)))) (.Y (Math|Vector|BreakVector (.Location (Math|Transform|BreakTransform _returnvalue_5)))) (Math|Float|Lerp (.Z (Math|Vector|BreakVector (.Location (Math|Transform|BreakTransform _returnvalue_5)))) 2e+02 _track_e5_hide)) false))
                  (:Finished
                    (Variables|Default|SetFadeOff_InProgress false)))))))
        (else
          (goto _label_3 Reset))))
    (:then_2
      (if (Variables|Default|GetFadeIn_InProgress)
        (Utilities|FlowControl|DoOnce false :!label _label_6
          (:Completed
            (Utilities|FlowControl|Sequence
              (:then_0
                (goto _label_4))
              (:then_1
                (goto _label_5))
              (:then_2
                (bind (_direction_2 _track_e1_hide_2 _track_e1_show_2 _track_e2_hide_2 _track_e2_show_2 _track_e3_hide_2 _track_e3_show_2 _track_e4_hide_2 _track_e4_show_2 _track_e5_hide_2 _track_e5_show) (Timeline|Timeline_1 PlayFromStart)
                  (:Update
                    (Transformation|SetRelativeLocation (Variables|Default|GetButton_Start) (Math|Vector|MakeVector (.X (Math|Vector|BreakVector (.Location (Math|Transform|BreakTransform _returnvalue)))) (.Y (Math|Vector|BreakVector (.Location (Math|Transform|BreakTransform _returnvalue)))) (Math|Float|Lerp 0.0 (.Z (Math|Vector|BreakVector (.Location (Math|Transform|BreakTransform _returnvalue)))) _track_e1_show_2)) false)
                    (Transformation|SetRelativeLocation (Variables|Default|GetButton_Options) (Math|Vector|MakeVector (.X (Math|Vector|BreakVector (.Location (Math|Transform|BreakTransform _returnvalue_2)))) (.Y (Math|Vector|BreakVector (.Location (Math|Transform|BreakTransform _returnvalue_2)))) (Math|Float|Lerp -7e+01 (.Z (Math|Vector|BreakVector (.Location (Math|Transform|BreakTransform _returnvalue_2)))) _track_e2_show_2)) false)
                    (Transformation|SetRelativeLocation (Variables|Default|GetButton_Highscores) (Math|Vector|MakeVector (.X (Math|Vector|BreakVector (.Location (Math|Transform|BreakTransform _returnvalue_3)))) (.Y (Math|Vector|BreakVector (.Location (Math|Transform|BreakTransform _returnvalue_3)))) (Math|Float|Lerp -1.4e+02 (.Z (Math|Vector|BreakVector (.Location (Math|Transform|BreakTransform _returnvalue_3)))) _track_e3_show_2)) false)
                    (Transformation|SetRelativeLocation (Variables|Default|GetButton_Credits) (Math|Vector|MakeVector (.X (Math|Vector|BreakVector (.Location (Math|Transform|BreakTransform _returnvalue_4)))) (.Y (Math|Vector|BreakVector (.Location (Math|Transform|BreakTransform _returnvalue_4)))) (Math|Float|Lerp -2.1e+02 (.Z (Math|Vector|BreakVector (.Location (Math|Transform|BreakTransform _returnvalue_4)))) _track_e4_show_2)) false)
                    (Transformation|SetRelativeLocation (Variables|Default|GetButton_Exit) (Math|Vector|MakeVector (.X (Math|Vector|BreakVector (.Location (Math|Transform|BreakTransform _returnvalue_5)))) (.Y (Math|Vector|BreakVector (.Location (Math|Transform|BreakTransform _returnvalue_5)))) (Math|Float|Lerp -2.8e+02 (.Z (Math|Vector|BreakVector (.Location (Math|Transform|BreakTransform _returnvalue_5)))) _track_e5_show)) false))
                  (:Finished
                    (Variables|Default|SetFadeIn_InProgress false)
                    (Variables|Default|SetSuppress_Input false)))))))
        (else
          (goto _label_6 Reset))))
    (:then_3
      (if (not (Variables|Default|GetSuppress_Input))
        ;[1 1 1] Update button scales + glow controls
        (Transformation|SetRelativeScale3D (Variables|Default|GetButton_Start) (* (Variables|Default|GetButton_Start_Scale) (Math|Float|Lerp 8.0 1e+01 (Variables|Default|GetButton_Start_Lerp))))
        (Class|LightComponent|SetBrightness (Variables|Rendering|GetButton_Start_Light) (Math|Float|Lerp 0.0 7e+03 (Variables|Default|GetButton_Start_Lerp)))
        (Transformation|SetRelativeScale3D (Variables|Default|GetButton_Credits) (* (Variables|Default|GetButton_Credits_Scale) (Math|Float|Lerp 8.0 1e+01 (Variables|Default|GetButton_Credits_Lerp))))
        (Class|LightComponent|SetBrightness (Variables|Rendering|GetButton_Credits_Light) (Math|Float|Lerp 0.0 7e+03 (Variables|Default|GetButton_Credits_Lerp)))
        (Transformation|SetRelativeScale3D (Variables|Default|GetButton_Highscores) (* (Variables|Default|GetButton_Highscores_Scale) (Math|Float|Lerp 8.0 1e+01 (Variables|Default|GetButton_Highscores_Lerp))))
        (Class|LightComponent|SetBrightness (Variables|Rendering|GetButton_Highscores_Light) (Math|Float|Lerp 0.0 7e+03 (Variables|Default|GetButton_Highscores_Lerp)))
        (Transformation|SetRelativeScale3D (Variables|Default|GetButton_Options) (* (Variables|Default|GetButton_Options_Scale) (Math|Float|Lerp 8.0 1e+01 (Variables|Default|GetButton_Options_Lerp))))
        (Class|LightComponent|SetBrightness (Variables|Rendering|GetButton_Options_Light) (Math|Float|Lerp 0.0 7e+03 (Variables|Default|GetButton_Options_Lerp)))
        (Transformation|SetRelativeScale3D (Variables|Default|GetButton_Exit) (* (Variables|Default|GetButton_Exit_Scale) (Math|Float|Lerp 8.0 1e+01 (Variables|Default|GetButton_Exit_Lerp))))
        (Class|LightComponent|SetBrightness (Variables|Rendering|GetButton_Exit_Light) (Math|Float|Lerp 0.0 7e+03 (Variables|Default|GetButton_Exit_Lerp)))
        ;[1 1 1] Scaling lerps
        (Utilities|FlowControl|Sequence
          (:then_0
            (if (== _selected_button_indx 0)
              (if (!= (Variables|Default|GetButton_Start_Lerp) 1.0)
                (if (>= (Variables|Default|GetDeltaTime) 0.01)
                  (if (<= (+ (Variables|Default|GetDeltaTime) (Variables|Default|GetButton_Start_Lerp)) 0.99)
                    (Variables|Default|SetButton_Start_Lerp (+ (Variables|Default|GetDeltaTime) (Variables|Default|GetButton_Start_Lerp)))
                    (else
                      (Variables|Default|SetButton_Start_Lerp 1.0)
                      (Variables|Default|SetDeltaTime 0.0 :!label _label_7)))))
              (elif (!= (Variables|Default|GetButton_Start_Lerp) 0.0)
                (if (>= (Variables|Default|GetDeltaTime) 0.01)
                  (if (>= (- (Variables|Default|GetButton_Start_Lerp) (Variables|Default|GetDeltaTime)) 0.01)
                    (Variables|Default|SetButton_Start_Lerp (- (Variables|Default|GetButton_Start_Lerp) (Variables|Default|GetDeltaTime)))
                    (else
                      (Variables|Default|SetButton_Start_Lerp 0.0)
                      (goto _label_7)))))))
          (:then_1
            (if (== _selected_button_indx 1)
              (if (!= (Variables|Default|GetButton_Options_Lerp) 1.0)
                (if (>= (Variables|Default|GetDeltaTime) 0.01)
                  (if (<= (+ (Variables|Default|GetDeltaTime) (Variables|Default|GetButton_Options_Lerp)) 0.99)
                    (Variables|Default|SetButton_Options_Lerp (+ (Variables|Default|GetDeltaTime) (Variables|Default|GetButton_Options_Lerp)))
                    (else
                      (Variables|Default|SetButton_Options_Lerp 1.0)
                      (goto _label_7)))))
              (elif (!= (Variables|Default|GetButton_Options_Lerp) 0.0)
                (if (>= (Variables|Default|GetDeltaTime) 0.01)
                  (if (>= (- (Variables|Default|GetButton_Options_Lerp) (Variables|Default|GetDeltaTime)) 0.01)
                    (Variables|Default|SetButton_Options_Lerp (- (Variables|Default|GetButton_Options_Lerp) (Variables|Default|GetDeltaTime)))
                    (else
                      (Variables|Default|SetButton_Options_Lerp 0.0)
                      (goto _label_7)))))))
          (:then_2
            (if (== _selected_button_indx 2)
              (if (!= (Variables|Default|GetButton_Highscores_Lerp) 1.0)
                (if (>= (Variables|Default|GetDeltaTime) 0.01)
                  (if (<= (+ (Variables|Default|GetDeltaTime) (Variables|Default|GetButton_Highscores_Lerp)) 0.99)
                    (Variables|Default|SetButton_Highscores_Lerp (+ (Variables|Default|GetDeltaTime) (Variables|Default|GetButton_Highscores_Lerp)))
                    (else
                      (Variables|Default|SetButton_Highscores_Lerp 1.0)
                      (goto _label_7)))))
              (elif (!= (Variables|Default|GetButton_Highscores_Lerp) 0.0)
                (if (>= (Variables|Default|GetDeltaTime) 0.01)
                  (if (>= (- (Variables|Default|GetButton_Highscores_Lerp) (Variables|Default|GetDeltaTime)) 0.01)
                    (Variables|Default|SetButton_Highscores_Lerp (- (Variables|Default|GetButton_Highscores_Lerp) (Variables|Default|GetDeltaTime)))
                    (else
                      (Variables|Default|SetButton_Highscores_Lerp 0.0)
                      (goto _label_7)))))))
          (:then_3
            (if (== _selected_button_indx 3)
              (if (!= (Variables|Default|GetButton_Credits_Lerp) 1.0)
                (if (>= (Variables|Default|GetDeltaTime) 0.01)
                  (if (<= (+ (Variables|Default|GetDeltaTime) (Variables|Default|GetButton_Credits_Lerp)) 0.99)
                    (Variables|Default|SetButton_Credits_Lerp (+ (Variables|Default|GetDeltaTime) (Variables|Default|GetButton_Credits_Lerp)))
                    (else
                      (Variables|Default|SetButton_Credits_Lerp 1.0)
                      (goto _label_7)))))
              (elif (!= (Variables|Default|GetButton_Credits_Lerp) 0.0)
                (if (>= (Variables|Default|GetDeltaTime) 0.01)
                  (if (>= (- (Variables|Default|GetButton_Credits_Lerp) (Variables|Default|GetDeltaTime)) 0.01)
                    (Variables|Default|SetButton_Credits_Lerp (- (Variables|Default|GetButton_Credits_Lerp) (Variables|Default|GetDeltaTime)))
                    (else
                      (Variables|Default|SetButton_Credits_Lerp 0.0)
                      (goto _label_7)))))))
          (:then_4
            (if (== _selected_button_indx 4)
              (if (!= (Variables|Default|GetButton_Exit_Lerp) 1.0)
                (if (>= (Variables|Default|GetDeltaTime) 0.01)
                  (if (<= (+ (Variables|Default|GetDeltaTime) (Variables|Default|GetButton_Exit_Lerp)) 0.99)
                    (Variables|Default|SetButton_Exit_Lerp (+ (Variables|Default|GetDeltaTime) (Variables|Default|GetButton_Exit_Lerp)))
                    (else
                      (Variables|Default|SetButton_Exit_Lerp 1.0)
                      (goto _label_7)))))
              (elif (!= (Variables|Default|GetButton_Exit_Lerp) 0.0)
                (if (>= (Variables|Default|GetDeltaTime) 0.01)
                  (if (>= (- (Variables|Default|GetButton_Exit_Lerp) (Variables|Default|GetDeltaTime)) 0.01)
                    (Variables|Default|SetButton_Exit_Lerp (- (Variables|Default|GetButton_Exit_Lerp) (Variables|Default|GetDeltaTime)))
                    (else
                      (Variables|Default|SetButton_Exit_Lerp 0.0)
                      (goto _label_7))))))))))))

(event Input|KeyboardEvents|Enter
  (bind _selected_button_indx (Variables|Default|GetSelected_Button_INDX))
  ;[1 1 1] Menu switch events
  (:Pressed
    (if (not (Variables|Default|GetSuppress_Input))
      (Utilities|FlowControl|Sequence
        (:then_0
          (if (== _selected_button_indx 0)
            (Default|CallPressButtonStart)))
        (:then_1
          (if (== _selected_button_indx 1)
            (Default|CallPressButtonOptions)))
        (:then_2
          (if (== _selected_button_indx 2)
            (Default|CallPressButtonHighscores)))
        (:then_3
          (if (== _selected_button_indx 3)
            (Default|CallPressButtonCredits)))
        (:then_4
          (if (== _selected_button_indx 4)
            (Default|CallPressButtonExit)))))))

(event Input|GamepadEvents|GamepadDPadDown
  ;[1 1 1] Up down counter
  (:Pressed
    (if (not (Variables|Default|GetSuppress_Input))
      (if (== (+ (Variables|Default|GetSelected_Button_INDX) 1) 5)
        (Variables|Default|SetSelected_Button_INDX 0)
        (else
          (Variables|Default|SetSelected_Button_INDX (+ (Variables|Default|GetSelected_Button_INDX) 1))))
      (Utilities|FlowControl|Delay 0.2))))

(event Input|GamepadEvents|GamepadDPadUp
  ;[1 1 1] Up down counter
  (:Pressed
    (if (not (Variables|Default|GetSuppress_Input))
      (if (== (- (Variables|Default|GetSelected_Button_INDX) 1) -1)
        (Variables|Default|SetSelected_Button_INDX 4)
        (else
          (Variables|Default|SetSelected_Button_INDX (- (Variables|Default|GetSelected_Button_INDX) 1))))
      (Utilities|FlowControl|Delay 0.2))))

(event Input|GamepadEvents|GamepadLeftStickDown
  ;[1 1 1] Up down counter
  (:Pressed
    (if (not (Variables|Default|GetSuppress_Input))
      (if (== (+ (Variables|Default|GetSelected_Button_INDX) 1) 5)
        (Variables|Default|SetSelected_Button_INDX 0)
        (else
          (Variables|Default|SetSelected_Button_INDX (+ (Variables|Default|GetSelected_Button_INDX) 1))))
      (Utilities|FlowControl|Delay 0.2))))

(event Input|GamepadEvents|GamepadLeftStickUp
  ;[1 1 1] Up down counter
  (:Pressed
    (if (not (Variables|Default|GetSuppress_Input))
      (if (== (- (Variables|Default|GetSelected_Button_INDX) 1) -1)
        (Variables|Default|SetSelected_Button_INDX 4)
        (else
          (Variables|Default|SetSelected_Button_INDX (- (Variables|Default|GetSelected_Button_INDX) 1))))
      (Utilities|FlowControl|Delay 0.2))))

(event Input|GamepadEvents|GamepadFaceButtonBottom
  (bind _selected_button_indx (Variables|Default|GetSelected_Button_INDX))
  ;[1 1 1] Menu switch events
  (:Pressed
    (if (not (Variables|Default|GetSuppress_Input))
      (Utilities|FlowControl|Sequence
        (:then_0
          (if (== _selected_button_indx 0)
            (Default|CallPressButtonStart)))
        (:then_1
          (if (== _selected_button_indx 1)
            (Default|CallPressButtonOptions)))
        (:then_2
          (if (== _selected_button_indx 2)
            (Default|CallPressButtonHighscores)))
        (:then_3
          (if (== _selected_button_indx 3)
            (Default|CallPressButtonCredits)))
        (:then_4
          (if (== _selected_button_indx 4)
            (Default|CallPressButtonExit)))))))

(event Input|KeyboardEvents|Down
  ;[1 1 1] Up down counter
  (:Pressed
    (if (not (Variables|Default|GetSuppress_Input))
      (if (== (+ (Variables|Default|GetSelected_Button_INDX) 1) 5)
        (Variables|Default|SetSelected_Button_INDX 0)
        (else
          (Variables|Default|SetSelected_Button_INDX (+ (Variables|Default|GetSelected_Button_INDX) 1))))
      (Utilities|FlowControl|Delay 0.2))))

(event Input|KeyboardEvents|Up
  ;[1 1 1] Up down counter
  (:Pressed
    (if (not (Variables|Default|GetSuppress_Input))
      (if (== (- (Variables|Default|GetSelected_Button_INDX) 1) -1)
        (Variables|Default|SetSelected_Button_INDX 4)
        (else
          (Variables|Default|SetSelected_Button_INDX (- (Variables|Default|GetSelected_Button_INDX) 1))))
      (Utilities|FlowControl|Delay 0.2))))

(fn ConstructionScript)

(fn ShowMainMenu
  (Variables|Default|SetFadeIn_Learp 0.0)
  (Variables|Default|SetFadeIn_InProgress true))

(fn HideMainMenu
  (Variables|Default|SetFadeOff_Learp 0.0)
  (Variables|Default|SetFadeOff_InProgress true))

(fn GetFocus
  (Variables|Default|SetInputFocus true))

(fn LeaveFocus
  (Variables|Default|SetInputFocus false))