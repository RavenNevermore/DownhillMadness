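; Main menu camera pawn that possesses itself at start, slides between three page positions and carries animated top and bottom bars.
; Public functions set flags and bar content; Tick turns flags into timelines for movement, bar show/hide and screen fades.
; Tick also feeds camera X into parallax background material parameters.
; On aspect-ratio changes, FOV trigonometry repositions camera and bars, and menu controllers shrink on screens narrower than 16:9.
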(event EventBeginPlay
  (bind _returnvalue (Game|GetPlayerController 0))
  (bind _topbar (Variables|Default|GetTopBar))
  (bind _bottombar (Variables|Default|GetBottomBar))
  (bind _menucamera (Variables|Default|GetMenuCamera))
  ;[1 1 1] Initialize
  (CallFunction|RefreshAspectRatio)
  (Utilities|FlowControl|Sequence
    (:then_0
      (Variables|/Script/Engine.CameraComponent|SetPostProcessSettings _menucamera (Utilities|Struct|MakePostProcessSettings false false false false false false false false false false false false false false false false false false false false false false false false false false false false false false false false false false false false false false false false false false false false false false false false false false false false false false false false false false false false false false false false false false false false false false false false false false false false false false false false false false false false false false false false false false false true true false false true false false false false "(R=1.000000,G=1.000000,B=1.000000,A=1.000000)" "(R=1.000000,G=1.000000,B=1.000000,A=1.000000)" 0.5 0.0 1.0 "(R=1.000000,G=0.000000,B=0.000000,A=1.000000)" "(R=0.000000,G=1.000000,B=0.000000,A=1.000000)" "(R=0.000000,G=0.000000,B=1.000000,A=1.000000)" 0.03 1.0 0.18 4.0 "(R=1.000000,G=1.000000,B=1.000000,A=1.000000)" 0.0 0.5 1.0 1.0 1.0 4.0 16.0 32.0 1e+02 "(R=0.500000,G=0.500000,B=0.500000,A=1.000000)" "(R=0.500000,G=0.500000,B=0.500000,A=1.000000)" "(R=0.500000,G=0.500000,B=0.500000,A=1.000000)" "(R=0.500000,G=0.500000,B=0.500000,A=1.000000)" "(R=0.500000,G=0.500000,B=0.500000,A=1.000000)" 1.0 "(R=0.500000,G=0.500000,B=0.500000,A=1.000000)" 0 1.0 0.0 0.64 5312.0 0.0 0.0 0.384 1.0 1.0 "(R=1.000000,G=1.000000,B=1.000000,A=1.000000)" 1.0 0 8e+01 98.300003 0.03 2.0 3.0 1.0 0.0 -8.0 4.0 1.0 "(R=1.000000,G=1.000000,B=1.000000,A=1.000000)" 3.0 8.0 0 "(R=1.000000,G=0.800000,B=0.400000,A=0.600000)" 0.0 "(R=0.000000,G=0.000000,B=0.000000,A=1.000000)" 0.0 0.0 0.5 1.0 4e+01 false 8e+03 5e+03 8e+02 2.0 3.0 5e+01 0.6 1.7 0.01 "(R=1.000000,G=1.000000,B=1.000000,A=1.000000)" 1.0 1.0 0 "DOFM_BokehDOF" 1e+03 0.0 3e+02 5e+02 0.0 15.0 15.0 15.0 0 0.4 1.0 0.08 0.0 0.0 0.0 0.5 1e+02 "AAM_FXAA" 1e+02 5e+01 0.6 (Utilities|Array|MakeArray _menucamera)))
      (Transformation|SetActorLocation (Game|Player|GetPlayerPawn 0) "-200.000000,-200.000000,-200.000000" false)
      (Pawn|Possess _returnvalue self)
      (Input|EnableInput _returnvalue)
      (bind _ypos (CallFunction|GetCameraYPos))
      (Transformation|SetActorLocation (Math|Vector|MakeVector 1e+02 _ypos (.Z (Math|Vector|BreakVector (Transformation|GetWorldLocation (VehicleSound|GetRootComponent (Variables|Default|GetParallaxPlane)))))) false))
    (:then_1
      ;[1 1 1] Show / Hide top bar
      (bind _returnvalue_2 (Transformation|GetRelativeTransform _topbar))
      (bind _zpos (CallFunction|GetTopBarZPos))
      (Transformation|SetRelativeLocation _topbar (Math|Vector|MakeVector (.X (Math|Vector|BreakVector (.Location (Math|Transform|BreakTransform _returnvalue_2)))) (.Y (Math|Vector|BreakVector (.Location (Math|Transform|BreakTransform _returnvalue_2)))) _zpos) false)
      (bind _returnvalue_3 (Transformation|GetRelativeTransform _bottombar))
      (bind _zpos_2 (CallFunction|GetBottomBarZPos))
      (Transformation|SetRelativeLocation _bottombar (Math|Vector|MakeVector (.X (Math|Vector|BreakVector (.Location (Math|Transform|BreakTransform _returnvalue_3)))) (.Y (Math|Vector|BreakVector (.Location (Math|Transform|BreakTransform _returnvalue_3)))) _zpos_2) false))))

(event EventTick
  (params (DeltaSeconds :type Float%20%28single-precision%29))
  (bind _returnvalue (Transformation|GetActorLocation))
  (bind _parallaxplane (Variables|Default|GetParallaxPlane))
  (bind _newcameratarget (Variables|Default|GetNewCameraTarget))
  (bind _x (Math|Vector|BreakVector _returnvalue))
  (bind _returnvalue_2 (VehicleSound|GetRootComponent _parallaxplane))
  (bind _returnvalue_3 (Transformation|GetWorldLocation _returnvalue_2))
  (bind _z (Math|Vector|BreakVector _returnvalue_3))
  ;[1 1 1] Update logic--> Process input action
  (CallFunction|RefreshAspectRatio)
  (Utilities|FlowControl|Sequence
    (:then_0
      (if (!= (Variables|Default|GetNewCameraTarget) (Variables|Default|GetCurrentCameraTarget))
        (if (Variables|Default|GetTrackGate)
          (Utilities|FlowControl|DoOnce false :!label _label
            (:Completed
              (Variables|Default|SetTrackGate true)
              (Utilities|FlowControl|Sequence
                (:then_0
                  (if (Variables|Default|GetMoveRight)
                    (Utilities|FlowControl|Sequence
                      (:then_0
                        (Variables|Default|SetMoveRight false))
                      (:then_1
                        (if (== _newcameratarget 1)
                          ;[1 1 1] Camera movement control timelines
                          (bind _cameratrack1_2 (Timeline|Timeline_2 PlayFromStart)
                            (:Update
                              (bind _ypos (CallFunction|GetCameraYPos))
                              (Transformation|SetActorLocation (Math|Vector|MakeVector (.X (Math|Vector|BreakVector (* _cameratrack1_2 1e+03))) _ypos _z) false))
                            (:Finished
                              (Variables|Default|SetCurrentCameraTarget 1)
                              (Variables|Default|SetTrackGate false :!label _label_2)))))
                      (:then_2
                        (if (== _newcameratarget 2)
                          (bind _cameratrack2_3 (Timeline|Timeline_3 PlayFromStart)
                            (:Update
                              (bind _ypos_2 (CallFunction|GetCameraYPos))
                              (Transformation|SetActorLocation (Math|Vector|MakeVector (.X (Math|Vector|BreakVector (* _cameratrack2_3 1e+03))) _ypos_2 _z) false))
                            (:Finished
                              (Variables|Default|SetCurrentCameraTarget 2)
                              (goto _label_2))))))))
                (:then_1
                  (if (Variables|Default|GetMoveLeft)
                    (Utilities|FlowControl|Sequence
                      (:then_0
                        (Variables|Default|SetMoveLeft false))
                      (:then_1
                        (if (== _newcameratarget 0)
                          (bind _cameratrack1_2_2 (Timeline|Timeline_0 ReverseFromEnd)
                            (:Update
                              (bind _ypos_3 (CallFunction|GetCameraYPos))
                              (Transformation|SetActorLocation (Math|Vector|MakeVector (.X (Math|Vector|BreakVector (* _cameratrack1_2_2 1e+03))) _ypos_3 _z) false))
                            (:Finished
                              (Variables|Default|SetCurrentCameraTarget 0)
                              (goto _label_2)))))
                      (:then_2
                        (if (== _newcameratarget 1)
                          (bind _cameratrack2_3_2 (Timeline|Timeline_1 ReverseFromEnd)
                            (:Update
                              (bind _ypos_4 (CallFunction|GetCameraYPos))
                              (Transformation|SetActorLocation (Math|Vector|MakeVector (.X (Math|Vector|BreakVector (* _cameratrack2_3_2 1e+03))) _ypos_4 _z) false))
                            (:Finished
                              (Variables|Default|SetCurrentCameraTarget 1)
                              (goto _label_2)))))))))))
          (else
            (Utilities|FlowControl|Sequence
              (:then_0
                (goto _label Reset))
              (:then_1
                (Variables|Default|SetTrackGate true)))))))
    (:then_1
      (Rendering|Material|SetScalarParameterValue "/Game/Materials/Menu_Main/BackgroundParallax/ParallaxBackground_PARAMS.ParallaxBackground_PARAMS" "CameraXPos" (/ (- _x 2.8e+02) 1e+03) :!class /Script/Engine.KismetMaterialLibrary)
      (Rendering|Material|SetScalarParameterValue "/Game/Materials/Menu_Main/BackgroundParallax/ParallaxBackground_PARAMS.ParallaxBackground_PARAMS" "CameraYPos" (Class|KismetMathLibrary|MapRange _x -5.8e+02 5.8e+02 2e+01 0.0) :!class /Script/Engine.KismetMaterialLibrary))
    (:then_2
      ;[1 1 1] Show / Hide top bar
      (if (Variables|Default|GetTopBarChanging)
        (Utilities|FlowControl|DoOnce false :!label _label_3
          (:Completed
            (if (Variables|Default|GetTopBarVisible)
              (Utilities|FlowControl|Sequence
                (:then_0
                  (Variables|Default|SetTopBarChanging false :!label _label_4))
                (:then_1
                  (bind _show_hide (Timeline|TopBar_Track ReverseFromEnd)
                    (:Update
                      (bind _zpos (CallFunction|GetTopBarZPos))
                      (Variables|Default|SetLastTopBarAlpha _show_hide)
                      (Transformation|SetRelativeLocation (Variables|Default|GetTopBar) (Math|Vector|MakeVector (.X (Math|Vector|BreakVector (.Location (Math|Transform|BreakTransform (stale EventBeginPlay _returnvalue_2))))) (.Y (Math|Vector|BreakVector (.Location (Math|Transform|BreakTransform (stale EventBeginPlay _returnvalue_2))))) (Math|Float|Lerp (- _zpos 8.8) _zpos _show_hide)) false))))
                (:then_2
                  (Variables|Default|SetTopBarVisible true)))
              (else
                (Utilities|FlowControl|Sequence
                  (:then_0
                    (goto _label_4))
                  (:then_1
                    (Timeline|TopBar_Track PlayFromStart))
                  (:then_2
                    (Variables|Default|SetTopBarVisible false)))))))
        (else
          (goto _label_3 Reset))))
    (:then_3
      ;[1 1 1] Screen fadein / out
      (if (Variables|Default|GetFadingIn)
        (if (Variables|Default|GetFadingOut)
          (Variables|Default|SetFadingIn false)
          (bind _track (Timeline|ScreenFadeIN Stop)
            (:Update
              (Variables|Default|SetCurrentScreenFade (Math|Float|Lerp 1.0 0.0 _track))
              (Rendering|Material|SetScalarParameterValue "/Game/Materials/Menu_Main/Menu_Fade_PARAMS.Menu_Fade_PARAMS" "Visibility" (Math|Float|Lerp 1.0 0.0 _track) :!class /Script/Engine.KismetMaterialLibrary)))
          (else
            (Variables|Default|SetFadingIn false)
            (Timeline|ScreenFadeIN PlayFromStart)))
        (elif (Variables|Default|GetFadingOut)
          (Variables|Default|SetFadingOut false)
          (bind _track_2 (Timeline|ScreenFadeOUT PlayFromStart)
            (:Update
              (Rendering|Material|SetScalarParameterValue "/Game/Materials/Menu_Main/Menu_Fade_PARAMS.Menu_Fade_PARAMS" "Visibility" (Math|Float|Lerp (Variables|Default|GetCurrentScreenFade) 1.0 _track_2) :!class /Script/Engine.KismetMaterialLibrary))))))
    (:then_4
      (if (Variables|Default|GetBottomBarChanging)
        (Utilities|FlowControl|DoOnce false :!label _label_5
          (:Completed
            (if (Variables|Default|GetBottomBarVisible)
              (Utilities|FlowControl|Sequence
                (:then_0
                  (Variables|Default|SetBottomBarChanging false :!label _label_6))
                (:then_1
                  (bind _show_hide_2 (Timeline|BottomBar_Track ReverseFromEnd)
                    (:Update
                      (bind _zpos_2 (CallFunction|GetBottomBarZPos))
                      (Variables|Default|SetLastBottomBarAlpha _show_hide_2)
                      (Transformation|SetRelativeLocation (Variables|Default|GetBottomBar) (Math|Vector|MakeVector (.X (Math|Vector|BreakVector (.Location (Math|Transform|BreakTransform (stale EventBeginPlay _returnvalue_3))))) (.Y (Math|Vector|BreakVector (.Location (Math|Transform|BreakTransform (stale EventBeginPlay _returnvalue_3))))) (Math|Float|Lerp (+ _zpos_2 8.8) _zpos_2 _show_hide_2)) false))))
                (:then_2
                  (Variables|Default|SetBottomBarVisible true)))
              (else
                (Utilities|FlowControl|Sequence
                  (:then_0
                    (goto _label_6))
                  (:then_1
                    (Timeline|BottomBar_Track PlayFromStart))
                  (:then_2
                    (Variables|Default|SetBottomBarVisible false)))))))
        (else
          (goto _label_5 Reset))))))

(fn ConstructionScript)

(fn MoveCameraRight
  (bind _currentcameratarget (Variables|Default|GetCurrentCameraTarget))
  (Utilities|FlowControl|Sequence
    (:then_0
      (if (== _currentcameratarget 0)
        (Variables|Default|SetNewCameraTarget 1)
        (Variables|Default|SetMoveRight true :!label _label)))
    (:then_1
      (if (== _currentcameratarget 1)
        (Variables|Default|SetNewCameraTarget 2)
        (goto _label)))))

(fn MoveCameraLeft
  (bind _currentcameratarget (Variables|Default|GetCurrentCameraTarget))
  (Utilities|FlowControl|Sequence
    (:then_0
      (if (== _currentcameratarget 1)
        (Variables|Default|SetNewCameraTarget 0)
        (Variables|Default|SetMoveLeft true :!label _label)))
    (:then_1
      (if (== _currentcameratarget 2)
        (Variables|Default|SetNewCameraTarget 1)
        (goto _label)))))

(fn HideTopBar
  (if (Variables|Default|GetTopBarVisible)
    (Variables|Default|SetTopBarVisible false)
    (Variables|Default|SetTopBarChanging true)))

(fn ShowTopBar
  (if (not (Variables|Default|GetTopBarVisible))
    (Variables|Default|SetTopBarVisible true)
    (Variables|Default|SetTopBarChanging true)))

(fn SetRightTopBarButton
  (params (ButtonName :type String))
  (bind _returnvalue (Utilities|Enum|Equal(Enum) ButtonName "XBOX_X"))
  (bind _returnvalue_2 (Utilities|Enum|Equal(Enum) ButtonName "XBOX_Y"))
  (bind _returnvalue_3 (Utilities|Enum|Equal(Enum) ButtonName "XBOX_A"))
  (bind _returnvalue_4 (Utilities|Enum|Equal(Enum) ButtonName "XBOX_B"))
  (Rendering|SetVisibility (Variables|Default|GetButton_X_R) _returnvalue false)
  (Rendering|SetVisibility (Variables|Default|GetButton_Y_R) _returnvalue_2 false)
  (Rendering|SetVisibility (Variables|Default|GetButton_A_R) _returnvalue_3 false)
  (Rendering|SetVisibility (Variables|Default|GetButton_B_R) _returnvalue_4 false)
  (Rendering|SetVisibility (Variables|Default|GetButton_X_R2) _returnvalue false)
  (Rendering|SetVisibility (Variables|Default|GetButton_Y_R2) _returnvalue_2 false)
  (Rendering|SetVisibility (Variables|Default|GetButton_A_R2) _returnvalue_3 false)
  (Rendering|SetVisibility (Variables|Default|GetButton_B_R2) _returnvalue_4 false))

(fn SetLeftTopBarButton
  (params (ButtonName :type String))
  (bind _returnvalue (Utilities|Enum|Equal(Enum) ButtonName "XBOX_X"))
  (bind _returnvalue_2 (Utilities|Enum|Equal(Enum) ButtonName "XBOX_Y"))
  (bind _returnvalue_3 (Utilities|Enum|Equal(Enum) ButtonName "XBOX_A"))
  (bind _returnvalue_4 (Utilities|Enum|Equal(Enum) ButtonName "XBOX_B"))
  (Rendering|SetVisibility (Variables|Default|GetButton_X_L) _returnvalue false)
  (Rendering|SetVisibility (Variables|Default|GetButton_Y_L) _returnvalue_2 false)
  (Rendering|SetVisibility (Variables|Default|GetButton_A_L) _returnvalue_3 false)
  (Rendering|SetVisibility (Variables|Default|GetButton_B_L) _returnvalue_4 false)
  (Rendering|SetVisibility (Variables|Default|GetButton_X_L2) _returnvalue false)
  (Rendering|SetVisibility (Variables|Default|GetButton_Y_L2) _returnvalue_2 false)
  (Rendering|SetVisibility (Variables|Default|GetButton_A_L2) _returnvalue_3 false)
  (Rendering|SetVisibility (Variables|Default|GetButton_B_L2) _returnvalue_4 false))

(fn SetTopBarTitle
  (params (TitleText :type String))
  (Rendering|Components|TextRender|SetText (Variables|Default|GetTitleText) TitleText))

(fn SetTopBarRightButtonText
  (params (RightText :type String))
  (Rendering|Components|TextRender|SetText (Variables|Default|GetRightTExt) RightText))

(fn SetTopBarLeftButtonText
  (params (LeftText :type String))
  (Rendering|Components|TextRender|SetText (Variables|Default|GetLeftText) LeftText))

(fn UnPossessController
  (Pawn|UnPossess (Game|GetPlayerController 0)))

(fn MoveCameratoTarget
  (params (TargetMaenuPage :type String))
  (if (Utilities|Enum|Equal(Enum) TargetMaenuPage "TrackSelection")
    (bind _ypos (CallFunction|GetCameraYPos))
    (Transformation|SetActorLocation (Math|Vector|MakeVector 5.8e+02 _ypos (.Z (Math|Vector|BreakVector (Transformation|GetWorldLocation (VehicleSound|GetRootComponent (Variables|Default|GetParallaxPlane)))))) false)
    (Variables|Default|SetCurrentCameraTarget 2)
    (Variables|Default|SetNewCameraTarget 2)
    (Variables|Default|SetTrackGate false)))

(fn GetCameraYPos
  (bind _parallaxplane (Variables|Default|GetParallaxPlane))
  (bind _returnvalue (VehicleSound|GetRootComponent _parallaxplane))
  (bind _returnvalue_2 (Transformation|GetWorldScale _returnvalue))
  (bind _z (Math|Vector|BreakVector _returnvalue_2))
  (bind _returnvalue_3 (/ _z 2.0))
  (bind _returnvalue_4 (* _returnvalue_3 256.0))
  (bind _returnvalue_5 (Math|Vector2D|MakeVector2D 0.0 _returnvalue_4))
  (bind (_x _y) (Math|Vector2D|BreakVector2D _returnvalue_5))
  (bind _returnvalue_6 (Math|Vector|MakeVector _x _y 0.0))
  (bind _aspectratio (CallFunction|GetAspectRatio))
  (bind _returnvalue_7 (Class|GameStateStatics|GetNearClipPlane))
  (return (+ (.Y (Math|Vector|BreakVector (Transformation|GetWorldLocation (VehicleSound|GetRootComponent (Variables|Default|GetParallaxPlane))))) (.X (Math|Vector|BreakVector (- (/ (Math|Vector|MakeVector (.X (Math|Vector2D|BreakVector2D (Math|Vector2D|MakeVector2D _returnvalue_7 (/ (* (Math|Trig|Tan(Degrees) (/ (Variables|/Script/Engine.CameraComponent|GetFieldOfView (Variables|Default|GetMenuCamera)) 2.0)) _returnvalue_7) _aspectratio)))) (.Y (Math|Vector2D|BreakVector2D (Math|Vector2D|MakeVector2D _returnvalue_7 (/ (* (Math|Trig|Tan(Degrees) (/ (Variables|/Script/Engine.CameraComponent|GetFieldOfView (Variables|Default|GetMenuCamera)) 2.0)) _returnvalue_7) _aspectratio)))) 0.0) (/ (Math|Vector|VectorLength (Class|KismetMathLibrary|Projectonto (Math|Vector|MakeVector (.X (Math|Vector2D|BreakVector2D (Math|Vector2D|MakeVector2D _returnvalue_7 (/ (* (Math|Trig|Tan(Degrees) (/ (Variables|/Script/Engine.CameraComponent|GetFieldOfView (Variables|Default|GetMenuCamera)) 2.0)) _returnvalue_7) _aspectratio)))) (.Y (Math|Vector2D|BreakVector2D (Math|Vector2D|MakeVector2D _returnvalue_7 (/ (* (Math|Trig|Tan(Degrees) (/ (Variables|/Script/Engine.CameraComponent|GetFieldOfView (Variables|Default|GetMenuCamera)) 2.0)) _returnvalue_7) _aspectratio)))) 0.0) _returnvalue_6)) (Math|Vector|VectorLength _returnvalue_6))) _returnvalue_6))))))

(fn GetTopBarZPos
  (bind _aspectratio (CallFunction|GetAspectRatio))
  (bind _returnvalue (Class|GameStateStatics|GetNearClipPlane))
  (bind _returnvalue_2 (Transformation|GetRelativeTransform (Variables|Default|GetTopBar)))
  (return (+ (* (/ (.X (Math|Vector|BreakVector (.Location (Math|Transform|BreakTransform _returnvalue_2)))) _returnvalue) (/ (* (Math|Trig|Tan(Degrees) (/ (Variables|/Script/Engine.CameraComponent|GetFieldOfView (Variables|Default|GetMenuCamera)) 2.0)) _returnvalue) _aspectratio)) 5.0)))

(fn GetAspectRatio
  (bind _variable (|LocalVariable))
  (bind _menucamera (Variables|Default|GetMenuCamera))
  (if (Variables|/Script/Engine.CameraComponent|GetbConstrainAspectRatio _menucamera)
    (|Assign _variable (Variables|/Script/Engine.CameraComponent|GetAspectRatio _menucamera))
    (else
      (bind (_posx _posy) (Class|VictoryBPFunctionLibrary|ViewportGetCenterOfViewport (Game|GetPlayerController 0)))
      (|Assign _variable (/ _posx _posy))))
  (return _variable))

(fn RefreshAspectRatio
  (bind _returnvalue (Transformation|GetActorLocation))
  (bind _returnvalue_2 (Math|Vector|MakeVector 1.0 1.0 1.0))
  (bind _bottombar (Variables|Default|GetBottomBar))
  (bind _trackcontroller (Variables|Default|GetTrackController))
  (bind _kartscontroller (Variables|Default|GetKartsController))
  (bind _topbar (Variables|Default|GetTopBar))
  (bind _charactercontroller (Variables|Default|GetCharacterController))
  (bind _optionscontroller (Variables|Default|GetOptionsController))
  (bind _maincontroller (Variables|Default|GetMainController))
  (bind (_x _y _z) (Math|Vector|BreakVector _returnvalue))
  (bind _aspectratio (CallFunction|GetAspectRatio))
  (if (!= _aspectratio (Variables|Default|GetLastAspectRatio))
    (Variables|Default|SetLastAspectRatio _aspectratio)
    (bind _zpos (CallFunction|GetBottomBarZPos))
    (bind _returnvalue_3 (Transformation|GetRelativeTransform _bottombar))
    (Transformation|SetRelativeLocation _bottombar (Math|Vector|MakeVector (.X (Math|Vector|BreakVector (.Location (Math|Transform|BreakTransform _returnvalue_3)))) (.Y (Math|Vector|BreakVector (.Location (Math|Transform|BreakTransform _returnvalue_3)))) (Math|Float|Lerp (+ _zpos 8.8) _zpos (Variables|Default|GetLastBottomBarAlpha))) false)
    (bind _zpos_2 (CallFunction|GetTopBarZPos))
    (bind _returnvalue_4 (Transformation|GetRelativeTransform _topbar))
    (Transformation|SetRelativeLocation _topbar (Math|Vector|MakeVector (.X (Math|Vector|BreakVector (.Location (Math|Transform|BreakTransform _returnvalue_4)))) (.Y (Math|Vector|BreakVector (.Location (Math|Transform|BreakTransform _returnvalue_4)))) (Math|Float|Lerp (- _zpos_2 8.8) _zpos_2 (Variables|Default|GetLastTopBarAlpha))) false)
    (bind _ypos (CallFunction|GetCameraYPos))
    (Transformation|SetActorLocation (Math|Vector|MakeVector _x _ypos _z) false)
    (if (< _aspectratio 1.777778)
      (Transformation|SetActorScale3D _charactercontroller (Math|Vector|MakeVector (/ _aspectratio 1.777778) (/ _aspectratio 1.777778) (/ _aspectratio 1.777778)))
      (Transformation|SetActorScale3D _optionscontroller (Math|Vector|MakeVector (/ _aspectratio 1.777778) (/ _aspectratio 1.777778) (/ _aspectratio 1.777778)))
      (Transformation|SetActorScale3D _maincontroller (Math|Vector|MakeVector (/ _aspectratio 1.777778) (/ _aspectratio 1.777778) (/ _aspectratio 1.777778)))
      (Transformation|SetActorScale3D _trackcontroller (Math|Vector|MakeVector (/ _aspectratio 1.777778) (/ _aspectratio 1.777778) (/ _aspectratio 1.777778)))
      (Transformation|SetActorScale3D _kartscontroller (Math|Vector|MakeVector (/ _aspectratio 1.777778) (/ _aspectratio 1.777778) (/ _aspectratio 1.777778)))
      (else
        (Transformation|SetActorScale3D _charactercontroller _returnvalue_2)
        (Transformation|SetActorScale3D _optionscontroller _returnvalue_2)
        (Transformation|SetActorScale3D _maincontroller _returnvalue_2)
        (Transformation|SetActorScale3D _trackcontroller _returnvalue_2)
        (Transformation|SetActorScale3D _kartscontroller _returnvalue_2)))))

(fn Fadein
  (Variables|Default|SetFadingIn true))

(fn FadeOut
  (Variables|Default|SetFadingOut true))

(fn ShowBottomBar
  (if (not (Variables|Default|GetBottomBarVisible))
    (Variables|Default|SetBottomBarVisible true)
    (Variables|Default|SetBottomBarChanging true)))

(fn HideBottomBar
  (if (Variables|Default|GetBottomBarVisible)
    (Variables|Default|SetBottomBarVisible false)
    (Variables|Default|SetBottomBarChanging true)))

(fn SetBottomBarText
  (params (Text :type String))
  (Rendering|Components|TextRender|SetText (Variables|Default|GetBottomtext) Text))

(fn GetBottomBarZPos
  (bind _aspectratio (CallFunction|GetAspectRatio))
  (bind _returnvalue (Class|GameStateStatics|GetNearClipPlane))
  (bind _returnvalue_2 (Transformation|GetRelativeTransform (Variables|Default|GetBottomBar)))
  (return (- (* (/ (.X (Math|Vector|BreakVector (.Location (Math|Transform|BreakTransform _returnvalue_2)))) _returnvalue) (/ (* (Math|Trig|Tan(Degrees) (/ (Variables|/Script/Engine.CameraComponent|GetFieldOfView (Variables|Default|GetMenuCamera)) 2.0)) _returnvalue) _aspectratio) -1.0) 5.0)))