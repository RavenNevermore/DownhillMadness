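; Main menu intro camera pawn that takes over player control and handles screen fades.
; On BeginPlay it moves the current player pawn high above the origin and possesses itself.
; FadeIn and FadeOut set flags that Tick consumes to run timelines lerping Visibility in the Menu_Fade_PARAMS material parameter collection.
; When both flags are set, Tick stops the fade-in and starts the fade-out on the following tick.
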(event EventTick
  (params (DeltaSeconds :type Float%20%28single-precision%29))
  ;[1 1 1] Screen fadein / out
  (if (Variables|Default|GetFadingIn)
    (if (Variables|Default|GetFadingOut)
      (Variables|Default|SetFadingIn false)
      (bind _track (Timeline|ScreenFadeIN Stop)
        (:Update
          (Rendering|Material|SetScalarParameterValue "/Game/Materials/Menu_Main/Menu_Fade_PARAMS.Menu_Fade_PARAMS" "Visibility" (Math|Float|Lerp 1.0 0.0 _track) :!class /Script/Engine.KismetMaterialLibrary)))
      (else
        (Variables|Default|SetFadingIn false)
        (Timeline|ScreenFadeIN PlayFromStart)))
    (elif (Variables|Default|GetFadingOut)
      (Variables|Default|SetFadingOut false)
      (bind _newtrack_1 (Timeline|ScreenFadeOUT PlayFromStart)
        (:Update
          (Rendering|Material|SetScalarParameterValue "/Game/Materials/Menu_Main/Menu_Fade_PARAMS.Menu_Fade_PARAMS" "Visibility" (Math|Float|Lerp 0.0 1.0 _newtrack_1) :!class /Script/Engine.KismetMaterialLibrary))))))

(event EventBeginPlay
  (Transformation|SetActorLocation (Game|Player|GetPlayerPawn 0) "0.000000,0.000000,5000.000000" false)
  (Pawn|Possess (Game|GetPlayerController 0) self))

(fn ConstructionScript)

(fn Fadein
  (Variables|Default|SetFadingIn true))

(fn FadeOut
  (Variables|Default|SetFadingOut true))