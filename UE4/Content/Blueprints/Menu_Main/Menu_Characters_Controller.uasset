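; Main menu controller for the character screen, where up to four players join or leave and the confirmed player count is saved on Next.
; AddPlayer and RemovePlayer set flags that Tick turns into chained scale, move and fade timelines, re-laying out player panels while input is suppressed.
; Gates choose which slots animate when a player leaves or the menu fades.
; Each tick, scale-controller components drive cropping in per-player material parameter collections.
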(event EventBeginPlay
  ;[1 1 1] Initialize
  (Variables|Default|SetFadeOff_InProgress false)
  (Variables|Default|SetFadeIn_InProgress false)
  (Variables|Default|SetCurrentPlayerCount 1)
  (Rendering|Material|SetScalarParameterValue "/Game/Materials/Menu_Main/Menu_Characters_1_PARAMS.Menu_Characters_1_PARAMS" "Visibility" 0.0 :!class /Script/Engine.KismetMaterialLibrary)
  (Rendering|Material|SetScalarParameterValue "/Game/Materials/Menu_Main/Menu_Characters_2_PARAMS.Menu_Characters_2_PARAMS" "Visibility" 0.0 :!class /Script/Engine.KismetMaterialLibrary)
  (Rendering|Material|SetScalarParameterValue "/Game/Materials/Menu_Main/Menu_Characters_3_PARAMS.Menu_Characters_3_PARAMS" "Visibility" 0.0 :!class /Script/Engine.KismetMaterialLibrary)
  (Rendering|Material|SetScalarParameterValue "/Game/Materials/Menu_Main/Menu_Characters_4_PARAMS.Menu_Characters_4_PARAMS" "Visibility" 0.0 :!class /Script/Engine.KismetMaterialLibrary)
  ;[1 1 1] Load player count
  (bind _returnvalue (Class|GameStateStatics|GetNumberOfPlayers)))

(event EventTick
  (params (DeltaSeconds :type Float%20%28single-precision%29))
  (bind _handle_playerid (Variables|Default|GetHandle_PlayerID))
  (bind _handle_playerid_2 (Variables|Default|GetHandle_PlayerID))
  (bind _currentplayercount (Variables|Default|GetCurrentPlayerCount))
  (bind _handle_playerid_3 (Variables|Default|GetHandle_PlayerID))
  (bind _handle_playerid_4 (Variables|Default|GetHandle_PlayerID))
  (bind _handle_playerid_5 (Variables|Default|GetHandle_PlayerID))
  (Utilities|FlowControl|Sequence
    (:then_0
      ;[1 1 1] Input focus management
      (if (Variables|Default|GetInputFocus)
        (Utilities|FlowControl|Sequence
          (:then_0
            (Utilities|FlowControl|DoOnce false :!label _label
              (:Completed
                (Input|EnableInput (Game|GetPlayerController 0))
                (Variables|Default|SetSuppressInput false))))
          (:then_1
            (goto _label_2 Reset)))
        (else
          (Utilities|FlowControl|Sequence
            (:then_0
              (Utilities|FlowControl|DoOnce false :!label _label_2
                (:Completed
                  (Input|DisableInput (Game|GetPlayerController 0))
                  (Variables|Default|SetSuppressInput true))))
            (:then_1
              (goto _label Reset))))))
    (:then_1
      ;[1 1 1] Fade in / out
      (if (Variables|Default|GetFadeIn_InProgress)
        (Variables|Default|SetFadeIn_InProgress false)
        (Utilities|FlowControl|Sequence
          (:then_0
            (if (Variables|Default|GetPlayer2_Online)
              (goto _label_3 Open)
              (else
                (goto _label_3 Close))))
          (:then_1
            (if (Variables|Default|GetPlayer3_Online)
              (goto _label_4 Open)
              (else
                (goto _label_4 Close))))
          (:then_2
            (if (Variables|Default|GetPlayer4_Online)
              (goto _label_5 Open)
              (else
                (goto _label_5 Close))))
          (:then_3
            (bind _fadetrack (Timeline|FadeIn PlayFromStart)
              (:Update
                (Utilities|FlowControl|Sequence
                  (:then_0
                    (Rendering|Material|SetScalarParameterValue "/Game/Materials/Menu_Main/Menu_Characters_1_PARAMS.Menu_Characters_1_PARAMS" "Visibility" _fadetrack :!class /Script/Engine.KismetMaterialLibrary))
                  (:then_1
                    (Utilities|FlowControl|Gate true :!label _label_3
                      (:Exit
                        (Rendering|Material|SetScalarParameterValue "/Game/Materials/Menu_Main/Menu_Characters_2_PARAMS.Menu_Characters_2_PARAMS" "Visibility" _fadetrack :!class /Script/Engine.KismetMaterialLibrary))))
                  (:then_2
                    (Utilities|FlowControl|Gate true :!label _label_4
                      (:Exit
                        (Rendering|Material|SetScalarParameterValue "/Game/Materials/Menu_Main/Menu_Characters_3_PARAMS.Menu_Characters_3_PARAMS" "Visibility" _fadetrack :!class /Script/Engine.KismetMaterialLibrary))))
                  (:then_3
                    (Utilities|FlowControl|Gate true :!label _label_5
                      (:Exit
                        (Rendering|Material|SetScalarParameterValue "/Game/Materials/Menu_Main/Menu_Characters_4_PARAMS.Menu_Characters_4_PARAMS" "Visibility" _fadetrack :!class /Script/Engine.KismetMaterialLibrary)))))))))))
    (:then_2
      (if (Variables|Default|GetFadeOff_InProgress)
        (Variables|Default|SetFadeOff_InProgress false)
        (Utilities|FlowControl|Sequence
          (:then_0
            (if (Variables|Default|GetPlayer2_Online)
              (goto _label_6 Open)
              (else
                (goto _label_6 Close))))
          (:then_1
            (if (Variables|Default|GetPlayer3_Online)
              (goto _label_7 Open)
              (else
                (goto _label_7 Close))))
          (:then_2
            (if (Variables|Default|GetPlayer4_Online)
              (goto _label_8 Open)
              (else
                (goto _label_8 Close))))
          (:then_3
            (bind _fadetrack_2 (Timeline|FadeOut ReverseFromEnd)
              (:Update
                (Utilities|FlowControl|Sequence
                  (:then_0
                    (Rendering|Material|SetScalarParameterValue "/Game/Materials/Menu_Main/Menu_Characters_1_PARAMS.Menu_Characters_1_PARAMS" "Visibility" _fadetrack_2 :!class /Script/Engine.KismetMaterialLibrary))
                  (:then_1
                    (Utilities|FlowControl|Gate true :!label _label_6
                      (:Exit
                        (Rendering|Material|SetScalarParameterValue "/Game/Materials/Menu_Main/Menu_Characters_2_PARAMS.Menu_Characters_2_PARAMS" "Visibility" _fadetrack_2 :!class /Script/Engine.KismetMaterialLibrary))))
                  (:then_2
                    (Utilities|FlowControl|Gate true :!label _label_7
                      (:Exit
                        (Rendering|Material|SetScalarParameterValue "/Game/Materials/Menu_Main/Menu_Characters_3_PARAMS.Menu_Characters_3_PARAMS" "Visibility" _fadetrack_2 :!class /Script/Engine.KismetMaterialLibrary))))
                  (:then_3
                    (Utilities|FlowControl|Gate true :!label _label_8
                      (:Exit
                        (Rendering|Material|SetScalarParameterValue "/Game/Materials/Menu_Main/Menu_Characters_4_PARAMS.Menu_Characters_4_PARAMS" "Visibility" _fadetrack_2 :!class /Script/Engine.KismetMaterialLibrary)))))))))))
    (:then_3
      ;[1 1 1] Material cropping
      (bind _returnvalue (Transformation|GetRelativeTransform (Variables|Default|GetPlayer1_ScaleController)))
      (Rendering|Material|SetScalarParameterValue "/Game/Materials/Menu_Main/Menu_Characters_1_PARAMS.Menu_Characters_1_PARAMS" "UVScale" (.X (Math|Vector|BreakVector (.Scale (Math|Transform|BreakTransform _returnvalue)))) :!class /Script/Engine.KismetMaterialLibrary)
      (Rendering|Material|SetScalarParameterValue "/Game/Materials/Menu_Main/Menu_Characters_1_PARAMS.Menu_Characters_1_PARAMS" "UpperLeftCrop" (* (/ (- 1.0 (.X (Math|Vector|BreakVector (.Scale (Math|Transform|BreakTransform _returnvalue))))) 2.0) -1.0) :!class /Script/Engine.KismetMaterialLibrary)
      (Rendering|Material|SetScalarParameterValue "/Game/Materials/Menu_Main/Menu_Characters_1_PARAMS.Menu_Characters_1_PARAMS" "LowerRightCrop" (- 1.0 (/ (- 1.0 (.X (Math|Vector|BreakVector (.Scale (Math|Transform|BreakTransform _returnvalue))))) 2.0)) :!class /Script/Engine.KismetMaterialLibrary)
      (bind _returnvalue_2 (Transformation|GetRelativeTransform (Variables|Default|GetPlayer2_ScaleController)))
      (Rendering|Material|SetScalarParameterValue "/Game/Materials/Menu_Main/Menu_Characters_2_PARAMS.Menu_Characters_2_PARAMS" "UVScale" (.X (Math|Vector|BreakVector (.Scale (Math|Transform|BreakTransform _returnvalue_2)))) :!class /Script/Engine.KismetMaterialLibrary)
      (Rendering|Material|SetScalarParameterValue "/Game/Materials/Menu_Main/Menu_Characters_2_PARAMS.Menu_Characters_2_PARAMS" "UpperLeftCrop" (* (/ (- 1.0 (.X (Math|Vector|BreakVector (.Scale (Math|Transform|BreakTransform _returnvalue_2))))) 2.0) -1.0) :!class /Script/Engine.KismetMaterialLibrary)
      (Rendering|Material|SetScalarParameterValue "/Game/Materials/Menu_Main/Menu_Characters_2_PARAMS.Menu_Characters_2_PARAMS" "LowerRightCrop" (- 1.0 (/ (- 1.0 (.X (Math|Vector|BreakVector (.Scale (Math|Transform|BreakTransform _returnvalue_2))))) 2.0)) :!class /Script/Engine.KismetMaterialLibrary)
      (bind _returnvalue_3 (Transformation|GetRelativeTransform (Variables|Default|GetPlayer3_ScaleController)))
      (Rendering|Material|SetScalarParameterValue "/Game/Materials/Menu_Main/Menu_Characters_3_PARAMS.Menu_Characters_3_PARAMS" "UVScale" (.X (Math|Vector|BreakVector (.Scale (Math|Transform|BreakTransform _returnvalue_3)))) :!class /Script/Engine.KismetMaterialLibrary)
      (Rendering|Material|SetScalarParameterValue "/Game/Materials/Menu_Main/Menu_Characters_3_PARAMS.Menu_Characters_3_PARAMS" "UpperLeftCrop" (* (/ (- 1.0 (.X (Math|Vector|BreakVector (.Scale (Math|Transform|BreakTransform _returnvalue_3))))) 2.0) -1.0) :!class /Script/Engine.KismetMaterialLibrary)
      (Rendering|Material|SetScalarParameterValue "/Game/Materials/Menu_Main/Menu_Characters_3_PARAMS.Menu_Characters_3_PARAMS" "LowerRightCrop" (- 1.0 (/ (- 1.0 (.X (Math|Vector|BreakVector (.Scale (Math|Transform|BreakTransform _returnvalue_3))))) 2.0)) :!class /Script/Engine.KismetMaterialLibrary)
      (bind _returnvalue_4 (Transformation|GetRelativeTransform (Variables|Default|GetPlayer4_ScaleController)))
      (Rendering|Material|SetScalarParameterValue "/Game/Materials/Menu_Main/Menu_Characters_4_PARAMS.Menu_Characters_4_PARAMS" "UVScale" (.X (Math|Vector|BreakVector (.Scale (Math|Transform|BreakTransform _returnvalue_4)))) :!class /Script/Engine.KismetMaterialLibrary)
      (Rendering|Material|SetScalarParameterValue "/Game/Materials/Menu_Main/Menu_Characters_4_PARAMS.Menu_Characters_4_PARAMS" "UpperLeftCrop" (* (/ (- 1.0 (.X (Math|Vector|BreakVector (.Scale (Math|Transform|BreakTransform _returnvalue_4))))) 2.0) -1.0) :!class /Script/Engine.KismetMaterialLibrary)
      (Rendering|Material|SetScalarParameterValue "/Game/Materials/Menu_Main/Menu_Characters_4_PARAMS.Menu_Characters_4_PARAMS" "LowerRightCrop" (- 1.0 (/ (- 1.0 (.X (Math|Vector|BreakVector (.Scale (Math|Transform|BreakTransform _returnvalue_4))))) 2.0)) :!class /Script/Engine.KismetMaterialLibrary))
    (:then_4
      ;[1 1 1] Show player penel
      (if (Variables|Default|GetPlayerCountIncreased)
        (Utilities|FlowControl|Sequence
          (:then_0
            (Variables|Default|SetPlayerCountIncreased false))
          (:then_1
            ;;[1 1 1] Second player entered game
            (if (== _currentplayercount 2)
              (bind _scaletrack (Timeline|ScaleTimeline PlayFromStart)
                (:Update
                  (Utilities|FlowControl|Sequence
                    (:then_0
                      (CallFunction|ScalePlayerPanel _handle_playerid 1.0 0.5 _scaletrack))
                    (:then_1
                      (CallFunction|ScalePlayerPanel 1 1.0 0.5 _scaletrack))))
                (:Finished
                  (bind _scaletrack_2 (Timeline|MoveTimeline PlayFromStart)
                    (:Update
                      (Utilities|FlowControl|Sequence
                        (:then_0
                          (CallFunction|MovePlayerPanel 1 "0, 0, 0" "0,370.000000, 0" _scaletrack_2))
                        (:then_1
                          (CallFunction|MovePlayerPanel _handle_playerid "0, 0, 0" "0,-370.000000, 0" _scaletrack_2))))
                    (:Finished
                      (bind _scaletrack_3 (Timeline|FadeTimeline PlayFromStart)
                        (:Update
                          (CallFunction|BlendPlayerPanel _handle_playerid 0.0 1.0 _scaletrack_3))
                        (:Finished
                          (Variables|Default|SetSuppressInput false)
                          (Variables|Default|SetSlot1_PlayerID _handle_playerid)))))))))
          (:then_2
            ;;[1 1 1] Third player entered game
            (if (== _currentplayercount 3)
              (bind _scaletrack_4 (Timeline|ScaleTimeline_2 PlayFromStart)
                (:Update
                  (Utilities|FlowControl|Sequence
                    (:then_0
                      (CallFunction|ScalePlayerPanel 1 0.5 0.3 _scaletrack_4))
                    (:then_1
                      (CallFunction|ScalePlayerPanel (Variables|Default|GetSlot1_PlayerID) 0.5 0.3 _scaletrack_4))
                    (:then_2
                      (CallFunction|ScalePlayerPanel _handle_playerid_2 0.5 0.3 _scaletrack_4))))
                (:Finished
                  (bind _scaletrack_5 (Timeline|MoveTimeline_2 PlayFromStart)
                    (:Update
                      (Utilities|FlowControl|Sequence
                        (:then_0
                          (CallFunction|MovePlayerPanel 1 "0,370.000000, 0" "0,470.000000, 0" _scaletrack_5))
                        (:then_1
                          (CallFunction|MovePlayerPanel (Variables|Default|GetSlot1_PlayerID) "0,-370.000000, 0" "0,0.000000, 0" _scaletrack_5))
                        (:then_2
                          (CallFunction|MovePlayerPanel _handle_playerid_2 "0,0.000000, 0" "0,-470.000000, 0" _scaletrack_5))))
                    (:Finished
                      (bind _scaletrack_6 (Timeline|FadeTimeline_2 PlayFromStart)
                        (:Update
                          (CallFunction|BlendPlayerPanel _handle_playerid_2 0.0 1.0 _scaletrack_6))
                        (:Finished
                          (Variables|Default|SetSuppressInput false)
                          (Variables|Default|SetSlot2_PlayerID _handle_playerid_2)))))))))
          (:then_3
            ;;[1 1 1] Fourth player entered game
            (if (== _currentplayercount 4)
              (bind _scaletrack_7 (Timeline|ScaleTimeline_3 PlayFromStart)
                (:Update
                  (Utilities|FlowControl|Sequence
                    (:then_0
                      (CallFunction|ScalePlayerPanel 1 0.3 0.25 _scaletrack_7))
                    (:then_1
                      (CallFunction|ScalePlayerPanel (Variables|Default|GetSlot1_PlayerID) 0.3 0.25 _scaletrack_7))
                    (:then_2
                      (CallFunction|ScalePlayerPanel (Variables|Default|GetSlot2_PlayerID) 0.3 0.25 _scaletrack_7))
                    (:then_3
                      (CallFunction|ScalePlayerPanel _handle_playerid_5 0.3 0.25 _scaletrack_7))))
                (:Finished
                  (bind _scaletrack_8 (Timeline|MoveTimeline_3 PlayFromStart)
                    (:Update
                      (Utilities|FlowControl|Sequence
                        (:then_0
                          (CallFunction|MovePlayerPanel 1 "0,470.000000, 0" "0,540.000000, 0" _scaletrack_8))
                        (:then_1
                          (CallFunction|MovePlayerPanel (Variables|Default|GetSlot1_PlayerID) "0,0.000000, 0" "0,180.000000, 0" _scaletrack_8))
                        (:then_2
                          (CallFunction|MovePlayerPanel (Variables|Default|GetSlot2_PlayerID) "0,-470.000000, 0" "0,-180.000000, 0" _scaletrack_8))
                        (:then_3
                          (CallFunction|MovePlayerPanel _handle_playerid_5 "0,0.000000, 0" "0,-540.000000, 0" _scaletrack_8))))
                    (:Finished
                      (bind _scaletrack_9 (Timeline|FadeTimeline_3 PlayFromStart)
                        (:Update
                          (CallFunction|BlendPlayerPanel _handle_playerid_5 0.0 1.0 _scaletrack_9))
                        (:Finished
                          (Variables|Default|SetSuppressInput false)
                          (Variables|Default|SetSlot3_PlayerID _handle_playerid_5))))))))))))
    (:then_5
      ;[1 1 1] Hide player panel
      (if (Variables|Default|GetPlayerCountDecreased)
        (Utilities|FlowControl|Sequence
          (:then_0
            (Variables|Default|SetPlayerCountDecreased false))
          (:then_1
            ;;[1 1 1] Fade out panel
            (bind _scaletrack_10 (Timeline|FadeTimelineR PlayFromStart)
              (:Update
                (CallFunction|BlendPlayerPanel (Variables|Default|GetHandle_PlayerID) 1.0 0.0 _scaletrack_10))
              (:Finished
                (Utilities|FlowControl|Sequence
                  (:then_0
                    ;;[1 1 1] Second player left game
                    (if (== 1 (Variables|Default|GetCurrentPlayerCount))
                      (bind _scaletrack_11 (Timeline|MoveTimelineR PlayFromStart)
                        (:Update
                          (CallFunction|MovePlayerPanel 1 "0.000000,370.000000, 0" "0,0.000000, 0" _scaletrack_11))
                        (:Finished
                          (bind _scaletrack_12 (Timeline|ScaleTimelineR PlayFromStart)
                            (:Update
                              (CallFunction|ScalePlayerPanel 1 0.5 1.0 _scaletrack_12))
                            (:Finished
                              (Variables|Default|SetSuppressInput false)))))))
                  (:then_1
                    ;;[1 1 1] Third player left game
                    (if (== 2 (Variables|Default|GetCurrentPlayerCount))
                      (Utilities|FlowControl|Sequence
                        (:then_0
                          (if (== (Variables|Default|GetSlot1_PlayerID) _handle_playerid_4)
                            (Utilities|FlowControl|Sequence
                              (:then_0
                                (goto _label_9 Open))
                              (:then_1
                                (goto _label_12 Open))
                              (:then_2
                                (goto _label_14 Open)))
                            (else
                              (Utilities|FlowControl|Sequence
                                (:then_0
                                  (goto _label_9 Close))
                                (:then_1
                                  (goto _label_12 Close))
                                (:then_2
                                  (goto _label_14 Close))))))
                        (:then_1
                          (if (== (Variables|Default|GetSlot2_PlayerID) _handle_playerid_4)
                            (Utilities|FlowControl|Sequence
                              (:then_0
                                (goto _label_10 Open))
                              (:then_1
                                (goto _label_11 Open))
                              (:then_2
                                (goto _label_13 Open)))
                            (else
                              (Utilities|FlowControl|Sequence
                                (:then_0
                                  (goto _label_10 Close))
                                (:then_1
                                  (goto _label_11 Close))
                                (:then_2
                                  (goto _label_13 Close))))))
                        (:then_2
                          (bind _scaletrack_13 (Timeline|MoveTimelineR_2 PlayFromStart)
                            (:Update
                              (Utilities|FlowControl|Sequence
                                (:then_0
                                  (CallFunction|MovePlayerPanel 1 "0,470.000000, 0" "0,370.000000, 0" _scaletrack_13))
                                (:then_1
                                  (Utilities|FlowControl|Gate true :!label _label_9
                                    (:Exit
                                      (CallFunction|MovePlayerPanel (Variables|Default|GetSlot2_PlayerID) "0,-470.000000, 0" "0,-370.000000, 0" _scaletrack_13))))
                                (:then_2
                                  (Utilities|FlowControl|Gate true :!label _label_10
                                    (:Exit
                                      (CallFunction|MovePlayerPanel (Variables|Default|GetSlot1_PlayerID) "0,0.000000, 0" "0,-370.000000, 0" _scaletrack_13))))))
                            (:Finished
                              (bind _scaletrack_14 (Timeline|ScaleTimelineR_2 PlayFromStart)
                                (:Update
                                  (Utilities|FlowControl|Sequence
                                    (:then_0
                                      (CallFunction|ScalePlayerPanel 1 0.3 0.5 _scaletrack_14))
                                    (:then_1
                                      (Utilities|FlowControl|Gate true :!label _label_11
                                        (:Exit
                                          (CallFunction|ScalePlayerPanel (Variables|Default|GetSlot1_PlayerID) 0.3 0.5 _scaletrack_14))))
                                    (:then_2
                                      (Utilities|FlowControl|Gate true :!label _label_12
                                        (:Exit
                                          (CallFunction|ScalePlayerPanel (Variables|Default|GetSlot2_PlayerID) 0.3 0.5 _scaletrack_14))))))
                                (:Finished
                                  (Utilities|FlowControl|Sequence
                                    (:then_0
                                      (Utilities|FlowControl|Gate true :!label _label_13
                                        (:Exit
                                          (Variables|Default|SetSlot2_PlayerID 0))))
                                    (:then_1
                                      (Utilities|FlowControl|Gate true :!label _label_14
                                        (:Exit
                                          (Variables|Default|SetSlot1_PlayerID (Variables|Default|GetSlot2_PlayerID))
                                          (Variables|Default|SetSlot2_PlayerID 0)))))
                                  (Variables|Default|SetSuppressInput false)))))))))
                  (:then_2
                    ;;[1 1 1] Fourth player left game
                    (if (== 3 (Variables|Default|GetCurrentPlayerCount))
                      (Utilities|FlowControl|Sequence
                        (:then_0
                          (if (== (Variables|Default|GetSlot1_PlayerID) _handle_playerid_3)
                            (Utilities|FlowControl|Sequence
                              (:then_0
                                (goto _label_15 Open))
                              (:then_1
                                (goto _label_16 Open))
                              (:then_2
                                (goto _label_21 Open))
                              (:then_3
                                (goto _label_22 Open))
                              (:then_4
                                (goto _label_27 Open)))
                            (else
                              (Utilities|FlowControl|Sequence
                                (:then_0
                                  (goto _label_15 Close))
                                (:then_1
                                  (goto _label_16 Close))
                                (:then_2
                                  (goto _label_21 Close))
                                (:then_3
                                  (goto _label_22 Close))
                                (:then_4
                                  (goto _label_27 Close))))))
                        (:then_1
                          (if (== (Variables|Default|GetSlot2_PlayerID) _handle_playerid_3)
                            (Utilities|FlowControl|Sequence
                              (:then_0
                                (goto _label_17 Open))
                              (:then_1
                                (goto _label_18 Open))
                              (:then_2
                                (goto _label_23 Open))
                              (:then_3
                                (goto _label_24 Open))
                              (:then_4
                                (goto _label_28 Open)))
                            (else
                              (Utilities|FlowControl|Sequence
                                (:then_0
                                  (goto _label_17 Close))
                                (:then_1
                                  (goto _label_18 Close))
                                (:then_2
                                  (goto _label_23 Close))
                                (:then_3
                                  (goto _label_24 Close))
                                (:then_4
                                  (goto _label_28 Close))))))
                        (:then_2
                          (if (== (Variables|Default|GetSlot3_PlayerID) _handle_playerid_3)
                            (Utilities|FlowControl|Sequence
                              (:then_0
                                (goto _label_19 Open))
                              (:then_1
                                (goto _label_20 Open))
                              (:then_2
                                (goto _label_25 Open))
                              (:then_3
                                (goto _label_26 Open))
                              (:then_4
                                (goto _label_29 Open)))
                            (else
                              (Utilities|FlowControl|Sequence
                                (:then_0
                                  (goto _label_19 Close))
                                (:then_1
                                  (goto _label_20 Close))
                                (:then_2
                                  (goto _label_25 Close))
                                (:then_3
                                  (goto _label_26 Close))
                                (:then_4
                                  (goto _label_29 Close))))))
                        (:then_3
                          (bind _scaletrack_15 (Timeline|MoveTimelineR_3 PlayFromStart)
                            (:Update
                              (Utilities|FlowControl|Sequence
                                (:then_0
                                  (CallFunction|MovePlayerPanel 1 "0,540.000000, 0" "0,470.000000, 0" _scaletrack_15))
                                (:then_1
                                  (Utilities|FlowControl|Gate true :!label _label_15
                                    (:Exit
                                      (CallFunction|MovePlayerPanel (Variables|Default|GetSlot2_PlayerID) "0,-180.000000,0.000000" "0.000000,0.000000, 0" _scaletrack_15))))
                                (:then_2
                                  (Utilities|FlowControl|Gate true :!label _label_16
                                    (:Exit
                                      (CallFunction|MovePlayerPanel (Variables|Default|GetSlot3_PlayerID) "0,-540.000000,0.000000" "0.000000,-470.000000, 0" _scaletrack_15))))
                                (:then_3
                                  (Utilities|FlowControl|Gate true :!label _label_17
                                    (:Exit
                                      (CallFunction|MovePlayerPanel (Variables|Default|GetSlot1_PlayerID) "0,180.000000,0.000000" "0.000000,0.000000, 0" _scaletrack_15))))
                                (:then_4
                                  (Utilities|FlowControl|Gate true :!label _label_18
                                    (:Exit
                                      (CallFunction|MovePlayerPanel (Variables|Default|GetSlot3_PlayerID) "0,-540.000000,0.000000" "0.000000,-470.000000, 0" _scaletrack_15))))
                                (:then_5
                                  (Utilities|FlowControl|Gate true :!label _label_19
                                    (:Exit
                                      (CallFunction|MovePlayerPanel (Variables|Default|GetSlot1_PlayerID) "0,180.000000,0.000000" "0.000000,0.000000, 0" _scaletrack_15))))
                                (:then_6
                                  (Utilities|FlowControl|Gate true :!label _label_20
                                    (:Exit
                                      (CallFunction|MovePlayerPanel (Variables|Default|GetSlot2_PlayerID) "0,-180.000000,0.000000" "0.000000,-470.000000, 0" _scaletrack_15))))))
                            (:Finished
                              (bind _scaletrack_16 (Timeline|ScaleTimelineR_3 PlayFromStart)
                                (:Update
                                  (Utilities|FlowControl|Sequence
                                    (:then_0
                                      (CallFunction|ScalePlayerPanel 1 0.25 0.3 _scaletrack_16))
                                    (:then_1
                                      (Utilities|FlowControl|Gate true :!label _label_21
                                        (:Exit
                                          (CallFunction|ScalePlayerPanel (Variables|Default|GetSlot2_PlayerID) 0.25 0.3 _scaletrack_16))))
                                    (:then_2
                                      (Utilities|FlowControl|Gate true :!label _label_22
                                        (:Exit
                                          (CallFunction|ScalePlayerPanel (Variables|Default|GetSlot3_PlayerID) 0.25 0.3 _scaletrack_16))))
                                    (:then_3
                                      (Utilities|FlowControl|Gate true :!label _label_23
                                        (:Exit
                                          (CallFunction|ScalePlayerPanel (Variables|Default|GetSlot1_PlayerID) 0.25 0.3 _scaletrack_16))))
                                    (:then_4
                                      (Utilities|FlowControl|Gate true :!label _label_24
                                        (:Exit
                                          (CallFunction|ScalePlayerPanel (Variables|Default|GetSlot3_PlayerID) 0.25 0.3 _scaletrack_16))))
                                    (:then_5
                                      (Utilities|FlowControl|Gate true :!label _label_25
                                        (:Exit
                                          (CallFunction|ScalePlayerPanel (Variables|Default|GetSlot1_PlayerID) 0.25 0.3 _scaletrack_16))))
                                    (:then_6
                                      (Utilities|FlowControl|Gate true :!label _label_26
                                        (:Exit
                                          (CallFunction|ScalePlayerPanel (Variables|Default|GetSlot2_PlayerID) 0.25 0.3 _scaletrack_16))))))
                                (:Finished
                                  (Utilities|FlowControl|Sequence
                                    (:then_0
                                      (Utilities|FlowControl|Gate true :!label _label_27
                                        (:Exit
                                          (Variables|Default|SetSlot1_PlayerID (Variables|Default|GetSlot2_PlayerID))
                                          (Variables|Default|SetSlot2_PlayerID (Variables|Default|GetSlot3_PlayerID))
                                          (Variables|Default|SetSlot3_PlayerID 0))))
                                    (:then_1
                                      (Utilities|FlowControl|Gate true :!label _label_28
                                        (:Exit
                                          (Variables|Default|SetSlot2_PlayerID (Variables|Default|GetSlot3_PlayerID))
                                          (Variables|Default|SetSlot3_PlayerID 0))))
                                    (:then_2
                                      (Utilities|FlowControl|Gate true :!label _label_29
                                        (:Exit
                                          (Variables|Default|SetSlot3_PlayerID 0)))))
                                  (Variables|Default|SetSuppressInput false))))))))))))))))))

(event Input|GamepadEvents|GamepadFaceButtonBottom
  ;[1 1 1] Button input events
  (:Pressed
    (if (not (Variables|Default|GetSuppressInput))
      ;[1 1 1] Save player count to globals
      (Class|GameStateStatics|SetNumberOfPlayers (Math|Conversions|ToByte(Integer) (Variables|Default|GetCurrentPlayerCount)))
      ;[1 1 1] Button event fire
      (Default|CallPressButtonNext))))

(event Input|KeyboardEvents|Enter
  ;[1 1 1] Button input events
  (:Pressed
    (if (not (Variables|Default|GetSuppressInput))
      ;[1 1 1] Save player count to globals
      (Class|GameStateStatics|SetNumberOfPlayers (Math|Conversions|ToByte(Integer) (Variables|Default|GetCurrentPlayerCount)))
      ;[1 1 1] Button event fire
      (Default|CallPressButtonNext))))

(event Input|GamepadEvents|GamepadFaceButtonRight
  ;[1 1 1] Button input events
  (:Pressed
    (if (not (Variables|Default|GetSuppressInput))
      ;[1 1 1] Button event fire
      (Default|CallPressButtonBack))))

(event Input|KeyboardEvents|Backspace
  ;[1 1 1] Button input events
  (:Pressed
    (if (not (Variables|Default|GetSuppressInput))
      ;[1 1 1] Button event fire
      (Default|CallPressButtonBack))))

(fn ConstructionScript)

(fn GetFocus
  (Variables|Default|SetInputFocus true)
  (Default|GetFocus (Variables|Default|GetCharacterSet1))
  (Default|GetFocus (Variables|Default|GetCharacterSet2))
  (Default|GetFocus (Variables|Default|GetCharacterSet3))
  (Default|GetFocus (Variables|Default|GetCharacterSet4)))

(fn SetCharacterRenderInstances
  (params (CharacterSet1 :type Character%20Camera%20Object%20Reference) (CharacterSet2 :type Character%20Camera%20Object%20Reference) (CharacterSet3 :type Character%20Camera%20Object%20Reference) (CharacterSet4 :type Character%20Camera%20Object%20Reference))
  (Utilities|FlowControl|Sequence
    (:then_0
      (Variables|Default|SetCharacterSet1 CharacterSet1))
    (:then_1
      (Variables|Default|SetCharacterSet2 CharacterSet2))
    (:then_2
      (Variables|Default|SetCharacterSet3 CharacterSet3))
    (:then_3
      (Variables|Default|SetCharacterSet4 CharacterSet4))))

(fn LeaveFocus
  (Variables|Default|SetInputFocus false)
  (Default|LeaveFocus (Variables|Default|GetCharacterSet1))
  (Default|LeaveFocus (Variables|Default|GetCharacterSet1MSK))
  (Default|LeaveFocus (Variables|Default|GetCharacterSet2))
  (Default|LeaveFocus (Variables|Default|GetCharacterSet2MSK))
  (Default|LeaveFocus (Variables|Default|GetCharacterSet3))
  (Default|LeaveFocus (Variables|Default|GetCharacterSet3MSK))
  (Default|LeaveFocus (Variables|Default|GetCharacterSet4))
  (Default|LeaveFocus (Variables|Default|GetCharacterSet4MSK)))

(fn ShowCharacterMenu
  (Variables|Default|SetFadeIn_InProgress true))

(fn HideCharacterMenu
  (Variables|Default|SetFadeOff_InProgress true))

(fn AddPlayer
  (params (PlayerID :type Integer))
  (if (not (Variables|Default|GetSuppressInput))
    (Utilities|FlowControl|Sequence
      (:then_0
        (if (== PlayerID 1)
          (if (not (Variables|Default|GetPlayer1_Online))
            (Variables|Default|SetPlayer1_Online true)
            (Variables|Default|SetPlayerCountIncreased true :!label _label)
            (Variables|Default|SetSuppressInput true)
            (Variables|Default|SetCurrentPlayerCount (+ (Variables|Default|GetCurrentPlayerCount) 1))
            (Variables|Default|SetHandle_PlayerID PlayerID))))
      (:then_1
        (if (== PlayerID 2)
          (if (not (Variables|Default|GetPlayer2_Online))
            (Variables|Default|SetPlayer2_Online true)
            (goto _label))))
      (:then_2
        (if (== PlayerID 3)
          (if (not (Variables|Default|GetPlayer3_Online))
            (Variables|Default|SetPlayer3_Online true)
            (goto _label))))
      (:then_3
        (if (== PlayerID 4)
          (if (not (Variables|Default|GetPlayer4_Online))
            (Variables|Default|SetPlayer4_Online true)
            (goto _label)))))))

(fn RemovePlayer
  (params (PlayerID :type Integer))
  (if (not (Variables|Default|GetSuppressInput))
    (Utilities|FlowControl|Sequence
      (:then_0
        (if (== PlayerID 1)
          (if (Variables|Default|GetPlayer1_Online)
            (Variables|Default|SetPlayer1_Online false)
            (Variables|Default|SetPlayerCountDecreased true :!label _label)
            (Variables|Default|SetSuppressInput true)
            (Variables|Default|SetCurrentPlayerCount (- (Variables|Default|GetCurrentPlayerCount) 1))
            (Variables|Default|SetHandle_PlayerID PlayerID))))
      (:then_1
        (if (== PlayerID 2)
          (if (Variables|Default|GetPlayer2_Online)
            (Variables|Default|SetPlayer2_Online false)
            (goto _label))))
      (:then_2
        (if (== PlayerID 3)
          (if (Variables|Default|GetPlayer3_Online)
            (Variables|Default|SetPlayer3_Online false)
            (goto _label))))
      (:then_3
        (if (== PlayerID 4)
          (if (Variables|Default|GetPlayer4_Online)
            (Variables|Default|SetPlayer4_Online false)
            (goto _label)))))))

(fn ScalePlayerPanel
  (params (PlayerID :type Integer) (StartWidth :type Float%20%28single-precision%29) (TargetWidth :type Float%20%28single-precision%29) (Alpha :type Float%20%28single-precision%29))
  (bind _returnvalue (Math|Float|Lerp StartWidth TargetWidth Alpha))
  (bind _returnvalue_2 (Math|Vector|MakeVector _returnvalue 1.0 1.0))
  (Utilities|FlowControl|Sequence
    (:then_0
      (if (== PlayerID 1)
        (Transformation|SetRelativeScale3D (Variables|Default|GetPlayer1_ScaleController) _returnvalue_2)))
    (:then_1
      (if (== PlayerID 2)
        (Transformation|SetRelativeScale3D (Variables|Default|GetPlayer2_ScaleController) _returnvalue_2)))
    (:then_2
      (if (== PlayerID 3)
        (Transformation|SetRelativeScale3D (Variables|Default|GetPlayer3_ScaleController) _returnvalue_2)))
    (:then_3
      (if (== PlayerID 4)
        (Transformation|SetRelativeScale3D (Variables|Default|GetPlayer4_ScaleController) _returnvalue_2)))))

(fn MovePlayerPanel
  (params (PlayerID :type Integer) (StartPos :type Vector) (TargetPos :type Vector) (Alpha :type Float%20%28single-precision%29))
  (bind (_x _y _z) (Math|Vector|BreakVector TargetPos))
  (bind (_x_2 _y_2 _z_2) (Math|Vector|BreakVector StartPos))
  (bind _returnvalue (Math|Float|Lerp _z_2 _z Alpha))
  (bind _returnvalue_2 (Math|Float|Lerp _x_2 _x Alpha))
  (bind _returnvalue_3 (Math|Float|Lerp _y_2 _y Alpha))
  (bind _returnvalue_4 (Math|Vector|MakeVector _returnvalue_2 _returnvalue_3 _returnvalue))
  (Utilities|FlowControl|Sequence
    (:then_0
      (if (== PlayerID 1)
        (Transformation|SetRelativeLocation (Variables|Default|GetPlayer1_LocationController) _returnvalue_4 false)))
    (:then_1
      (if (== PlayerID 2)
        (Transformation|SetRelativeLocation (Variables|Default|GetPlayer2_LocationController) _returnvalue_4 false)))
    (:then_2
      (if (== PlayerID 3)
        (Transformation|SetRelativeLocation (Variables|Default|GetPlayer3_LocationController) _returnvalue_4 false)))
    (:then_3
      (if (== PlayerID 4)
        (Transformation|SetRelativeLocation (Variables|Default|GetPlayer4_LocationController) _returnvalue_4 false)))))

(fn BlendPlayerPanel
  (params (PlayerID :type Integer) (StartTransparency :type Float%20%28single-precision%29) (TargetTransparency :type Float%20%28single-precision%29) (Alpha :type Float%20%28single-precision%29))
  (bind _returnvalue (Math|Float|Lerp StartTransparency TargetTransparency Alpha))
  (Utilities|FlowControl|Sequence
    (:then_0
      (if (== PlayerID 1)
        (Rendering|Material|SetScalarParameterValue "/Game/Materials/Menu_Main/Menu_Characters_1_PARAMS.Menu_Characters_1_PARAMS" "Visibility" _returnvalue :!class /Script/Engine.KismetMaterialLibrary)))
    (:then_1
      (if (== PlayerID 2)
        (Rendering|Material|SetScalarParameterValue "/Game/Materials/Menu_Main/Menu_Characters_2_PARAMS.Menu_Characters_2_PARAMS" "Visibility" _returnvalue :!class /Script/Engine.KismetMaterialLibrary)))
    (:then_2
      (if (== PlayerID 3)
        (Rendering|Material|SetScalarParameterValue "/Game/Materials/Menu_Main/Menu_Characters_3_PARAMS.Menu_Characters_3_PARAMS" "Visibility" _returnvalue :!class /Script/Engine.KismetMaterialLibrary)))
    (:then_3
      (if (== PlayerID 4)
        (Rendering|Material|SetScalarParameterValue "/Game/Materials/Menu_Main/Menu_Characters_4_PARAMS.Menu_Characters_4_PARAMS" "Visibility" _returnvalue :!class /Script/Engine.KismetMaterialLibrary)))))