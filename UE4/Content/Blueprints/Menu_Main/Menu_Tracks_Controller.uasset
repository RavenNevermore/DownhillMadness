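; Main menu track selection controller that lets the player pick the Workshop or one of two race tracks.
; Keyboard and gamepad input cycles the selection, though Left from Workshop lands on Track 1, and confirm or back calls event dispatchers.
; Tick polls flags to toggle input focus, update text, materials and icon glow, and start timelines fading visibility through a Material Parameter Collection.
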(event EventBeginPlay
  ;[1 1 1] Initialize
  (Variables|Default|SetFadeOff_InProgress false)
  (Variables|Default|SetFadeIn_InProgress false)
  (Rendering|Material|SetScalarParameterValue "/Game/Materials/Menu_Main/Menu_Tracks_PARAMS.Menu_Tracks_PARAMS" "Visibility" 0.0 :!class /Script/Engine.KismetMaterialLibrary)
  (Variables|Default|SetSelectedTrackINDX 0)
  (Rendering|Components|TextRender|SetText (Variables|Default|GetSelectionText) "")
  (Rendering|Material|SetMaterial (Variables|Default|GetTrack1) 1 "/Game/Materials/Menu_Main/Menu_Tracks_Unselected_MAT.Menu_Tracks_Unselected_MAT")
  (Rendering|Material|SetMaterial (Variables|Default|GetTrack2) 1 "/Game/Materials/Menu_Main/Menu_Tracks_Unselected_MAT.Menu_Tracks_Unselected_MAT"))

(event EventTick
  (params (DeltaSeconds :type Float%20%28single-precision%29))
  (bind _selectedtrackindx (Variables|Default|GetSelectedTrackINDX))
  (Utilities|FlowControl|Sequence
    (:then_0
      ;[1 1 1] Input focus management
      (if (Variables|Default|GetInputFocus)
        (Utilities|FlowControl|Sequence
          (:then_0
            (Utilities|FlowControl|DoOnce false :!label _label
              (:Completed
                (Input|EnableInput (Game|GetPlayerController 0))
                (Variables|Default|SetSuppressInput false))))
          (:then_1
            (goto _label_2 Reset)))
        (else
          (Utilities|FlowControl|Sequence
            (:then_0
              (Utilities|FlowControl|DoOnce false :!label _label_2
                (:Completed
                  (Input|DisableInput (Game|GetPlayerController 0))
                  (Variables|Default|SetSuppressInput true))))
            (:then_1
              (goto _label Reset))))))
    (:then_1
      ;[1 1 1] Fade in / out
      (if (Variables|Default|GetFadeIn_InProgress)
        (Variables|Default|SetFadeIn_InProgress false)
        (bind _fadetrack (Timeline|FadeIn PlayFromStart)
          (:Update
            (Rendering|Material|SetScalarParameterValue "/Game/Materials/Menu_Main/Menu_Tracks_PARAMS.Menu_Tracks_PARAMS" "Visibility" _fadetrack :!class /Script/Engine.KismetMaterialLibrary)))))
    (:then_2
      (if (Variables|Default|GetFadeOff_InProgress)
        (Variables|Default|SetFadeOff_InProgress false)
        (bind _fadetrack_2 (Timeline|FadeOut ReverseFromEnd)
          (:Update
            (Rendering|Material|SetScalarParameterValue "/Game/Materials/Menu_Main/Menu_Tracks_PARAMS.Menu_Tracks_PARAMS" "Visibility" _fadetrack_2 :!class /Script/Engine.KismetMaterialLibrary)))))
    (:then_3
      ;[1 1 1] Material effects
      (if (Variables|Default|GetSelectedChanged)
        (Utilities|FlowControl|Sequence
          (:then_0
            (goto _label_3 Reset))
          (:then_1
            _)))
      (Utilities|FlowControl|DoOnce false :!label _label_3
        (:Completed
          (Utilities|FlowControl|Sequence
            (:then_0
              (if (== _selectedtrackindx 0)
                (Rendering|Components|TextRender|SetText (Variables|Default|GetSelectionText) "< Workshop >")
                (Rendering|SetVisibility (Variables|Default|GetWorkshop_Icon_Glow) true false)
                (CallFunction|SetAllTracksMaterial)
                (Variables|Default|SetSelectedChanged false :!label _label_4)))
            (:then_1
              (if (== _selectedtrackindx 1)
                (Rendering|Components|TextRender|SetText (Variables|Default|GetSelectionText) "< Track 1 >")
                (Rendering|Material|SetMaterial (Variables|Default|GetTrack1) 1 "/Game/Materials/Menu_Main/Menu_Tracks_Selected_MAT.Menu_Tracks_selected_MAT")
                (CallFunction|SetAllTracksMaterial 1)
                (Utilities|FlowControl|Sequence
                  (:then_0
                    (goto _label_4))
                  (:then_1
                    (Rendering|SetVisibility (Variables|Default|GetWorkshop_Icon_Glow) false false :!label _label_5)))))
            (:then_2
              (if (== _selectedtrackindx 2)
                (Rendering|Components|TextRender|SetText (Variables|Default|GetSelectionText) "< Track 2 >")
                (Rendering|Material|SetMaterial (Variables|Default|GetTrack2) 1 "/Game/Materials/Menu_Main/Menu_Tracks_Selected_MAT.Menu_Tracks_selected_MAT")
                (CallFunction|SetAllTracksMaterial 2)
                (Utilities|FlowControl|Sequence
                  (:then_0
                    (goto _label_4))
                  (:then_1
                    (goto _label_5)))))))))))

(event Input|GamepadEvents|GamepadFaceButtonBottom
  (bind _selectedtrackindx (Variables|Default|GetSelectedTrackINDX))
  ;[1 1 1] Button input events
  (:Pressed
    (if (not (Variables|Default|GetSuppressInput))
      (Utilities|FlowControl|Sequence
        (:then_0
          (if (== _selectedtrackindx 0)
            (Default|CallPressButtonStartWorkshop)))
        (:then_1
          (if (== _selectedtrackindx 1)
            (Variables|Default|SetSelectedTrack "Map_1")
            (Default|CallPressButtonStartRace (Variables|Default|GetSelectedTrack) :!label _label)))
        (:then_2
          (if (== _selectedtrackindx 2)
            (Variables|Default|SetSelectedTrack "Map_2")
            (goto _label)))))))

(event Input|KeyboardEvents|Enter
  (bind _selectedtrackindx (Variables|Default|GetSelectedTrackINDX))
  ;[1 1 1] Button input events
  (:Pressed
    (if (not (Variables|Default|GetSuppressInput))
      (Utilities|FlowControl|Sequence
        (:then_0
          (if (== _selectedtrackindx 0)
            (Default|CallPressButtonStartWorkshop)))
        (:then_1
          (if (== _selectedtrackindx 1)
            (Variables|Default|SetSelectedTrack "Map_1")
            (Default|CallPressButtonStartRace (Variables|Default|GetSelectedTrack) :!label _label)))
        (:then_2
          (if (== _selectedtrackindx 2)
            (Variables|Default|SetSelectedTrack "Map_2")
            (goto _label)))))))

(event Input|KeyboardEvents|Left
  ;[1 1 1] Button input events
  (:Pressed
    (if (not (Variables|Default|GetSuppressInput))
      (if (> (Variables|Default|GetSelectedTrackINDX) 0)
        (Variables|Default|SetSelectedTrackINDX (- (Variables|Default|GetSelectedTrackINDX) 1))
        (else
          (Variables|Default|SetSelectedTrackINDX 1)))
      (Variables|Default|SetSelectedChanged true))))

(event Input|GamepadEvents|GamepadLeftStickLeft
  ;[1 1 1] Button input events
  (:Pressed
    (if (not (Variables|Default|GetSuppressInput))
      (if (> (Variables|Default|GetSelectedTrackINDX) 0)
        (Variables|Default|SetSelectedTrackINDX (- (Variables|Default|GetSelectedTrackINDX) 1))
        (else
          (Variables|Default|SetSelectedTrackINDX 1)))
      (Variables|Default|SetSelectedChanged true))))

(event Input|KeyboardEvents|Right
  ;[1 1 1] Button input events
  (:Pressed
    (if (not (Variables|Default|GetSuppressInput))
      (if (< (Variables|Default|GetSelectedTrackINDX) 2)
        (Variables|Default|SetSelectedTrackINDX (+ (Variables|Default|GetSelectedTrackINDX) 1))
        (else
          (Variables|Default|SetSelectedTrackINDX 0)))
      (Variables|Default|SetSelectedChanged true))))

(event Input|GamepadEvents|GamepadDPadRight
  ;[1 1 1] Button input events
  (:Pressed
    (if (not (Variables|Default|GetSuppressInput))
      (if (< (Variables|Default|GetSelectedTrackINDX) 2)
        (Variables|Default|SetSelectedTrackINDX (+ (Variables|Default|GetSelectedTrackINDX) 1))
        (else
          (Variables|Default|SetSelectedTrackINDX 0)))
      (Variables|Default|SetSelectedChanged true))))

(event Input|GamepadEvents|GamepadLeftStickRight
  ;[1 1 1] Button input events
  (:Pressed
    (if (not (Variables|Default|GetSuppressInput))
      (if (< (Variables|Default|GetSelectedTrackINDX) 2)
        (Variables|Default|SetSelectedTrackINDX (+ (Variables|Default|GetSelectedTrackINDX) 1))
        (else
          (Variables|Default|SetSelectedTrackINDX 0)))
      (Variables|Default|SetSelectedChanged true))))

(event Input|GamepadEvents|GamepadFaceButtonRight
  ;[1 1 1] Button input events
  (:Pressed
    (if (not (Variables|Default|GetSuppressInput))
      (Default|CallPressButtonBack))))

(event Input|KeyboardEvents|Backspace
  ;[1 1 1] Button input events
  (:Pressed
    (if (not (Variables|Default|GetSuppressInput))
      (Default|CallPressButtonBack))))

(event Input|GamepadEvents|GamepadDPadLeft
  ;[1 1 1] Button input events
  (:Pressed
    (if (not (Variables|Default|GetSuppressInput))
      (if (> (Variables|Default|GetSelectedTrackINDX) 0)
        (Variables|Default|SetSelectedTrackINDX (- (Variables|Default|GetSelectedTrackINDX) 1))
        (else
          (Variables|Default|SetSelectedTrackINDX 1)))
      (Variables|Default|SetSelectedChanged true))))

(fn ConstructionScript)

(fn GetFocus
  (Variables|Default|SetInputFocus true))

(fn LeaveFocus
  (Variables|Default|SetInputFocus false))

(fn ShowTracksMenu
  (Variables|Default|SetFadeIn_InProgress true))

(fn HideTracksMenu
  (Variables|Default|SetFadeOff_InProgress true)
  (Rendering|Components|TextRender|SetText (Variables|Default|GetSelectionText) ""))

(fn SetAllTracksMaterial
  (params (ExceptionINDX :type Integer))
  (Utilities|FlowControl|Sequence
    (:then_0
      (if (== ExceptionINDX 0)
        (Rendering|Material|SetMaterial (Variables|Default|GetTrack1) 1 "/Game/Materials/Menu_Main/Menu_Tracks_Unselected_MAT.Menu_Tracks_Unselected_MAT")
        (Rendering|Material|SetMaterial (Variables|Default|GetTrack2) 1 "/Game/Materials/Menu_Main/Menu_Tracks_Unselected_MAT.Menu_Tracks_Unselected_MAT")))
    (:then_1
      (if (== ExceptionINDX 1)
        (Rendering|Material|SetMaterial (Variables|Default|GetTrack2) 1 "/Game/Materials/Menu_Main/Menu_Tracks_Unselected_MAT.Menu_Tracks_Unselected_MAT")))
    (:then_2
      (if (== ExceptionINDX 2)
        (Rendering|Material|SetMaterial (Variables|Default|GetTrack1) 1 "/Game/Materials/Menu_Main/Menu_Tracks_Unselected_MAT.Menu_Tracks_Unselected_MAT")))))