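; Controller options menu Blueprint for the main menu, tracking focus and visibility and handling the back action.
; Tick watches InputFocus and uses two cross-resetting DoOnce gates to enable or disable player input and update SuppressInput once per focus change.
; Gamepad right face button or Backspace calls PressButtonBack unless input is suppressed.
; GetFocus/LeaveFocus and ShowOptionsMenu/HideOptionsMenu only set the focus and visibility flags.
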(event EventTick
  (params (DeltaSeconds :type Float%20%28single-precision%29))
  ;[1 1 1] Input focus management
  (if (Variables|Default|GetInputFocus)
    (Utilities|FlowControl|Sequence
      (:then_0
        (Utilities|FlowControl|DoOnce false :!label _label
          (:Completed
            (Input|EnableInput (Game|GetPlayerController 0))
            (Variables|Default|SetSuppressInput false))))
      (:then_1
        (goto _label_2 Reset)))
    (else
      (Utilities|FlowControl|Sequence
        (:then_0
          (Utilities|FlowControl|DoOnce false :!label _label_2
            (:Completed
              (Input|DisableInput (Game|GetPlayerController 0))
              (Variables|Default|SetSuppressInput true))))
        (:then_1
          (goto _label Reset))))))

(event Input|GamepadEvents|GamepadFaceButtonRight
  (:Pressed
    (if (not (Variables|Default|GetSuppressInput))
      (Default|CallPressButtonBack))))

(event Input|KeyboardEvents|Backspace
  (:Pressed
    (if (not (Variables|Default|GetSuppressInput))
      (Default|CallPressButtonBack))))

(fn ConstructionScript)

(fn GetFocus
  (Variables|Default|SetInputFocus true))

(fn LeaveFocus
  (Variables|Default|SetInputFocus false))

(fn ShowOptionsMenu
  (Variables|Default|SetIsVisible true))

(fn HideOptionsMenu
  (Variables|Default|SetIsVisible false))