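; Main menu music player that plays an intro track, then alternates between two loop variations.
; Tick accumulates playback position and starts the next track just before the current one ends, using gates to switch variations on the first loop's length.
; Timelines fade the intro in and, once FadeOut is called, all tracks out, scaled by the music volume option.
; Tick also applies volume setting changes, with the second variation quieter.
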(event EventBeginPlay
  (bind _music_intro (Variables|Default|GetMusic_Intro))
  (Utilities|FlowControl|Sequence
    (:then_0
      (Variables|Default|SetIntroLength (Variables|/Script/Engine.SoundBase|GetDuration (Variables|/Script/Engine.AudioComponent|GetSound (Variables|Default|GetMusic_Intro)))))
    (:then_1
      (Variables|Default|SetLoopLength (Variables|/Script/Engine.SoundBase|GetDuration (Variables|/Script/Engine.AudioComponent|GetSound (Variables|Default|GetMusic_Loop_Var1)))))
    (:then_2
      (bind _musicvolume (Class|GameStateStatics|GetGameOptions))
      (bind _fadein (Timeline|FadeInTL PlayFromStart)
        (:Update
          (Audio|Components|Audio|SetVolumeMultiplier _music_intro (* _fadein _musicvolume) :!class /Script/Engine.AudioComponent))))
    (:then_3
      (Components|Activation|Activate _music_intro false))))

(event EventTick
  (params (DeltaSeconds :type Float%20%28single-precision%29))
  (bind _music_loop_var1 (Variables|Default|GetMusic_Loop_Var1))
  (bind _music_loop_var2 (Variables|Default|GetMusic_Loop_Var2))
  (Utilities|FlowControl|Sequence
    (:then_0
      (Variables|Default|SetTrackPosition (+ DeltaSeconds (Variables|Default|GetTrackPosition))))
    (:then_1
      (if (< (- (Variables|Default|GetIntroLength) (Variables|Default|GetTrackPosition)) 0.166)
        (Utilities|FlowControl|DoOnce false
          (:Completed
            (Variables|Default|SetTrackPosition 0.0)
            (Components|Activation|Activate (Variables|Default|GetMusic_Loop_Var1) false)
            (goto _label Open)))))
    (:then_2
      (Utilities|FlowControl|Gate true :!label _label
        (:Exit
          (if (< (- (Variables|Default|GetLoopLength) (Variables|Default|GetTrackPosition)) 0.166)
            (Utilities|FlowControl|Sequence
              (:then_0
                (Utilities|FlowControl|Gate true :!label _label_2
                  (:Exit
                    (if (not (Components|Activation|IsActive _music_loop_var1))
                      (Components|Activation|Activate _music_loop_var1 false)
                      (Utilities|FlowControl|Sequence
                        (:then_0
                          (goto _label_2 Close))
                        (:then_1
                          (goto _label_4 Open))
                        (:then_2
                          (Variables|Default|SetTrackPosition 0.0 :!label _label_3)))))))
              (:then_1
                (Utilities|FlowControl|Gate false :!label _label_4
                  (:Exit
                    (if (not (Components|Activation|IsActive _music_loop_var2))
                      (Components|Activation|Activate _music_loop_var2 false)
                      (Utilities|FlowControl|Sequence
                        (:then_0
                          (goto _label_2 Open))
                        (:then_1
                          (goto _label_4 Close))
                        (:then_2
                          (goto _label_3))))))))))))
    (:then_3
      (if (Variables|Default|GetFadingOut)
        (Variables|Default|SetFadingOut false)
        (bind _musicvolume (Class|GameStateStatics|GetGameOptions))
        (bind _fadeout (Timeline|FadeOutTL PlayFromStart)
          (:Update
            (Utilities|FlowControl|Sequence
              (:then_0
                (Audio|Components|Audio|SetVolumeMultiplier (Variables|Default|GetMusic_Intro) (* _fadeout _musicvolume) :!class /Script/Engine.AudioComponent))
              (:then_1
                (Audio|Components|Audio|SetVolumeMultiplier (Variables|Default|GetMusic_Loop_Var1) (* _fadeout _musicvolume) :!class /Script/Engine.AudioComponent))
              (:then_2
                (Audio|Components|Audio|SetVolumeMultiplier (Variables|Default|GetMusic_Loop_Var2) (* _fadeout _musicvolume) :!class /Script/Engine.AudioComponent))))
          (:Finished
            (Variables|Default|SetFadedout true)))))
    (:then_4
      ;[1 1 1] Use music volume setting
      (if (not (Variables|Default|GetFadingOut))
        (if (not (Variables|Default|GetFadedout))
          (bind _musicvolume_2 (Class|GameStateStatics|GetGameOptions))
          (if (!= _musicvolume_2 (Variables|Default|GetLastVolume))
            (Utilities|FlowControl|Sequence
              (:then_0
                (Variables|Default|SetLastVolume _musicvolume_2))
              (:then_1
                (Audio|Components|Audio|SetVolumeMultiplier (Variables|Default|GetMusic_Intro) _musicvolume_2 :!class /Script/Engine.AudioComponent))
              (:then_2
                (Audio|Components|Audio|SetVolumeMultiplier (Variables|Default|GetMusic_Loop_Var1) _musicvolume_2 :!class /Script/Engine.AudioComponent))
              (:then_3
                (Audio|Components|Audio|SetVolumeMultiplier (Variables|Default|GetMusic_Loop_Var2) (* _musicvolume_2 0.75) :!class /Script/Engine.AudioComponent)))))))))

(fn ConstructionScript)

(fn FadeOut
  (Variables|Default|SetFadingOut true))