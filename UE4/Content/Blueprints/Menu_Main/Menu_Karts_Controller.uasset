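; Main-menu controller for the kart selection screen, supporting one to four local players.
; SetPlayerStates, also fed by RestoreState from saved controller indexes, scales and positions panels by player count and slot.
; Tick maps players to kart render instances and writes panel crop and timeline fades into per-panel Material Parameter Collections.
; While focused, it handles Back input and fires Next automatically once all online players have selected.
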(event EventBeginPlay
  ;[1 1 1] Initialize
  (Variables|Default|SetFadeOff_InProgress false)
  (Variables|Default|SetFadeIn_InProgress false)
  (Variables|Default|SetCurrentPlayerCount 1)
  (Rendering|Material|SetScalarParameterValue "/Game/Materials/Menu_Main/Menu_Karts_1_PARAMS.Menu_Karts_1_PARAMS" "Visibility" 0.0 :!class /Script/Engine.KismetMaterialLibrary)
  (Rendering|Material|SetScalarParameterValue "/Game/Materials/Menu_Main/Menu_Karts_2_PARAMS.Menu_Karts_2_PARAMS" "Visibility" 0.0 :!class /Script/Engine.KismetMaterialLibrary)
  (Rendering|Material|SetScalarParameterValue "/Game/Materials/Menu_Main/Menu_Karts_3_PARAMS.Menu_Karts_3_PARAMS" "Visibility" 0.0 :!class /Script/Engine.KismetMaterialLibrary)
  (Rendering|Material|SetScalarParameterValue "/Game/Materials/Menu_Main/Menu_Karts_4_PARAMS.Menu_Karts_4_PARAMS" "Visibility" 0.0 :!class /Script/Engine.KismetMaterialLibrary)
  ;[1 1 1] Load player count
  (bind _returnvalue (Class|GameStateStatics|GetNumberOfPlayers))
  (Variables|Default|SetCurrentPlayerCount (Math|Conversions|ToInteger(Byte) _returnvalue)))

(event EventTick
  (params (DeltaSeconds :type Float%20%28single-precision%29))
  (bind _player4_slot (Variables|Default|GetPlayer4_Slot))
  (bind _palyer2_slot (Variables|Default|GetPalyer2_Slot))
  (bind _player3_slot (Variables|Default|GetPlayer3_Slot))
  (Utilities|FlowControl|Sequence
    (:then_0
      ;[1 1 1] Input focus management
      (if (Variables|Default|GetInputFocus)
        (Utilities|FlowControl|Sequence
          (:then_0
            (Utilities|FlowControl|DoOnce false :!label _label
              (:Completed
                (Input|EnableInput (Game|GetPlayerController 0))
                (Variables|Default|SetSuppressInput false))))
          (:then_1
            (goto _label_2 Reset)))
        (else
          (Utilities|FlowControl|Sequence
            (:then_0
              (Utilities|FlowControl|DoOnce false :!label _label_2
                (:Completed
                  (Input|DisableInput (Game|GetPlayerController 0))
                  (Variables|Default|SetSuppressInput true))))
            (:then_1
              (goto _label Reset))))))
    (:then_1
      ;[1 1 1] Fade in / out
      (if (Variables|Default|GetFadeIn_InProgress)
        (Variables|Default|SetFadeIn_InProgress false)
        (Utilities|FlowControl|Sequence
          (:then_0
            (if (Variables|Default|GetPlayer2_Online)
              (goto _label_3 Open)
              (else
                (goto _label_3 Close))))
          (:then_1
            (if (Variables|Default|GetPlayer3_Online)
              (goto _label_4 Open)
              (else
                (goto _label_4 Close))))
          (:then_2
            (if (Variables|Default|GetPlayer4_Online)
              (goto _label_5 Open)
              (else
                (goto _label_5 Close))))
          (:then_3
            (bind _fadetrack (Timeline|FadeInTL PlayFromStart)
              (:Update
                (Utilities|FlowControl|Sequence
                  (:then_0
                    (Rendering|Material|SetScalarParameterValue "/Game/Materials/Menu_Main/Menu_Karts_1_PARAMS.Menu_Karts_1_PARAMS" "Visibility" _fadetrack :!class /Script/Engine.KismetMaterialLibrary))
                  (:then_1
                    (Utilities|FlowControl|Gate true :!label _label_3
                      (:Exit
                        (Rendering|Material|SetScalarParameterValue "/Game/Materials/Menu_Main/Menu_Karts_2_PARAMS.Menu_Karts_2_PARAMS" "Visibility" _fadetrack :!class /Script/Engine.KismetMaterialLibrary))))
                  (:then_2
                    (Utilities|FlowControl|Gate true :!label _label_4
                      (:Exit
                        (Rendering|Material|SetScalarParameterValue "/Game/Materials/Menu_Main/Menu_Karts_3_PARAMS.Menu_Karts_3_PARAMS" "Visibility" _fadetrack :!class /Script/Engine.KismetMaterialLibrary))))
                  (:then_3
                    (Utilities|FlowControl|Gate true :!label _label_5
                      (:Exit
                        (Rendering|Material|SetScalarParameterValue "/Game/Materials/Menu_Main/Menu_Karts_4_PARAMS.Menu_Karts_4_PARAMS" "Visibility" _fadetrack :!class /Script/Engine.KismetMaterialLibrary)))))))))))
    (:then_2
      (if (Variables|Default|GetFadeOff_InProgress)
        (Variables|Default|SetFadeOff_InProgress false)
        (Utilities|FlowControl|Sequence
          (:then_0
            (if (Variables|Default|GetPlayer2_Online)
              (goto _label_6 Open)
              (else
                (goto _label_6 Close))))
          (:then_1
            (if (Variables|Default|GetPlayer3_Online)
              (goto _label_7 Open)
              (else
                (goto _label_7 Close))))
          (:then_2
            (if (Variables|Default|GetPlayer4_Online)
              (goto _label_8 Open)
              (else
                (goto _label_8 Close))))
          (:then_3
            (bind _fadetrack_2 (Timeline|FadeOutTL ReverseFromEnd)
              (:Update
                (Utilities|FlowControl|Sequence
                  (:then_0
                    (Rendering|Material|SetScalarParameterValue "/Game/Materials/Menu_Main/Menu_Karts_1_PARAMS.Menu_Karts_1_PARAMS" "Visibility" _fadetrack_2 :!class /Script/Engine.KismetMaterialLibrary))
                  (:then_1
                    (Utilities|FlowControl|Gate true :!label _label_6
                      (:Exit
                        (Rendering|Material|SetScalarParameterValue "/Game/Materials/Menu_Main/Menu_Karts_2_PARAMS.Menu_Karts_2_PARAMS" "Visibility" _fadetrack_2 :!class /Script/Engine.KismetMaterialLibrary))))
                  (:then_2
                    (Utilities|FlowControl|Gate true :!label _label_7
                      (:Exit
                        (Rendering|Material|SetScalarParameterValue "/Game/Materials/Menu_Main/Menu_Karts_3_PARAMS.Menu_Karts_3_PARAMS" "Visibility" _fadetrack_2 :!class /Script/Engine.KismetMaterialLibrary))))
                  (:then_3
                    (Utilities|FlowControl|Gate true :!label _label_8
                      (:Exit
                        (Rendering|Material|SetScalarParameterValue "/Game/Materials/Menu_Main/Menu_Karts_4_PARAMS.Menu_Karts_4_PARAMS" "Visibility" _fadetrack_2 :!class /Script/Engine.KismetMaterialLibrary)))))))))))
    (:then_3
      ;[1 1 1] Material cropping
      (bind _returnvalue (Transformation|GetRelativeTransform (Variables|Default|GetPlayer1_ScaleController)))
      (Rendering|Material|SetScalarParameterValue "/Game/Materials/Menu_Main/Menu_Karts_1_PARAMS.Menu_Karts_1_PARAMS" "UVScale" (.X (Math|Vector|BreakVector (.Scale (Math|Transform|BreakTransform _returnvalue)))) :!class /Script/Engine.KismetMaterialLibrary)
      (Rendering|Material|SetScalarParameterValue "/Game/Materials/Menu_Main/Menu_Karts_1_PARAMS.Menu_Karts_1_PARAMS" "UpperLeftCrop" (* (/ (- 1.0 (.X (Math|Vector|BreakVector (.Scale (Math|Transform|BreakTransform _returnvalue))))) 2.0) -1.0) :!class /Script/Engine.KismetMaterialLibrary)
      (Rendering|Material|SetScalarParameterValue "/Game/Materials/Menu_Main/Menu_Karts_1_PARAMS.Menu_Karts_1_PARAMS" "LowerRightCrop" (- 1.0 (/ (- 1.0 (.X (Math|Vector|BreakVector (.Scale (Math|Transform|BreakTransform _returnvalue))))) 2.0)) :!class /Script/Engine.KismetMaterialLibrary)
      (bind _returnvalue_2 (Transformation|GetRelativeTransform (Variables|Default|GetPlayer2_ScaleController)))
      (Rendering|Material|SetScalarParameterValue "/Game/Materials/Menu_Main/Menu_Karts_2_PARAMS.Menu_Karts_2_PARAMS" "UVScale" (.X (Math|Vector|BreakVector (.Scale (Math|Transform|BreakTransform _returnvalue_2)))) :!class /Script/Engine.KismetMaterialLibrary)
      (Rendering|Material|SetScalarParameterValue "/Game/Materials/Menu_Main/Menu_Karts_2_PARAMS.Menu_Karts_2_PARAMS" "UpperLeftCrop" (* (/ (- 1.0 (.X (Math|Vector|BreakVector (.Scale (Math|Transform|BreakTransform _returnvalue_2))))) 2.0) -1.0) :!class /Script/Engine.KismetMaterialLibrary)
      (Rendering|Material|SetScalarParameterValue "/Game/Materials/Menu_Main/Menu_Karts_2_PARAMS.Menu_Karts_2_PARAMS" "LowerRightCrop" (- 1.0 (/ (- 1.0 (.X (Math|Vector|BreakVector (.Scale (Math|Transform|BreakTransform _returnvalue_2))))) 2.0)) :!class /Script/Engine.KismetMaterialLibrary)
      (bind _returnvalue_3 (Transformation|GetRelativeTransform (Variables|Default|GetPlayer3_ScaleController)))
      (Rendering|Material|SetScalarParameterValue "/Game/Materials/Menu_Main/Menu_Karts_3_PARAMS.Menu_Karts_3_PARAMS" "UVScale" (.X (Math|Vector|BreakVector (.Scale (Math|Transform|BreakTransform _returnvalue_3)))) :!class /Script/Engine.KismetMaterialLibrary)
      (Rendering|Material|SetScalarParameterValue "/Game/Materials/Menu_Main/Menu_Karts_3_PARAMS.Menu_Karts_3_PARAMS" "UpperLeftCrop" (* (/ (- 1.0 (.X (Math|Vector|BreakVector (.Scale (Math|Transform|BreakTransform _returnvalue_3))))) 2.0) -1.0) :!class /Script/Engine.KismetMaterialLibrary)
      (Rendering|Material|SetScalarParameterValue "/Game/Materials/Menu_Main/Menu_Karts_3_PARAMS.Menu_Karts_3_PARAMS" "LowerRightCrop" (- 1.0 (/ (- 1.0 (.X (Math|Vector|BreakVector (.Scale (Math|Transform|BreakTransform _returnvalue_3))))) 2.0)) :!class /Script/Engine.KismetMaterialLibrary)
      (bind _returnvalue_4 (Transformation|GetRelativeTransform (Variables|Default|GetPlayer4_ScaleController)))
      (Rendering|Material|SetScalarParameterValue "/Game/Materials/Menu_Main/Menu_Karts_4_PARAMS.Menu_Karts_4_PARAMS" "UVScale" (.X (Math|Vector|BreakVector (.Scale (Math|Transform|BreakTransform _returnvalue_4)))) :!class /Script/Engine.KismetMaterialLibrary)
      (Rendering|Material|SetScalarParameterValue "/Game/Materials/Menu_Main/Menu_Karts_4_PARAMS.Menu_Karts_4_PARAMS" "UpperLeftCrop" (* (/ (- 1.0 (.X (Math|Vector|BreakVector (.Scale (Math|Transform|BreakTransform _returnvalue_4))))) 2.0) -1.0) :!class /Script/Engine.KismetMaterialLibrary)
      (Rendering|Material|SetScalarParameterValue "/Game/Materials/Menu_Main/Menu_Karts_4_PARAMS.Menu_Karts_4_PARAMS" "LowerRightCrop" (- 1.0 (/ (- 1.0 (.X (Math|Vector|BreakVector (.Scale (Math|Transform|BreakTransform _returnvalue_4))))) 2.0)) :!class /Script/Engine.KismetMaterialLibrary))
    (:then_4
      ;[1 1 1] Auto proceed to next menu
      (if (Variables|Default|GetInputFocus)
        (if (Variables|Default|GetAllPlayersSelected)
          (Default|CallPressButtonNext))))
    (:then_5
      ;[1 1 1] Screen ref transfer
      (Utilities|FlowControl|Sequence
        (:then_0
          (Default|SetScreenReference (Variables|Default|GetKartsInstance1)))
        (:then_1
          (Utilities|FlowControl|Sequence
            (:then_0
              (if (== _palyer2_slot 2)
                (Default|SetScreenReference (Variables|Default|GetKartsInstance2) 1)))
            (:then_1
              (if (== _palyer2_slot 3)
                (Default|SetScreenReference (Variables|Default|GetKartsInstance3) 1)))
            (:then_2
              (if (== _palyer2_slot 4)
                (Default|SetScreenReference (Variables|Default|GetKartsInstance4) 1)))))
        (:then_2
          (Utilities|FlowControl|Sequence
            (:then_0
              (if (== _player3_slot 2)
                (Default|SetScreenReference (Variables|Default|GetKartsInstance2) 2)))
            (:then_1
              (if (== _player3_slot 3)
                (Default|SetScreenReference (Variables|Default|GetKartsInstance3) 2)))
            (:then_2
              (if (== _player3_slot 4)
                (Default|SetScreenReference (Variables|Default|GetKartsInstance4) 2)))))
        (:then_3
          (Utilities|FlowControl|Sequence
            (:then_0
              (if (== _player4_slot 2)
                (Default|SetScreenReference (Variables|Default|GetKartsInstance2) 3)))
            (:then_1
              (if (== _player4_slot 3)
                (Default|SetScreenReference (Variables|Default|GetKartsInstance3) 3)))
            (:then_2
              (if (== _player4_slot 4)
                (Default|SetScreenReference (Variables|Default|GetKartsInstance4) 3)))))))))

(event Input|GamepadEvents|GamepadFaceButtonRight
  ;[1 1 1] Button input events
  (:Pressed
    (if (not (Variables|Default|GetSuppressInput))
      ;[1 1 1] Button event fire
      (Default|CallPressButtonBack))))

(event Input|KeyboardEvents|Backspace
  ;[1 1 1] Button input events
  (:Pressed
    (if (not (Variables|Default|GetSuppressInput))
      ;[1 1 1] Button event fire
      (Default|CallPressButtonBack))))

(fn ConstructionScript)

(fn SetPlayerStates
  (params (Player2_Online :type Boolean) (Player3_Online :type Boolean) (Player4_Online :type Boolean) (Player2_SlotID :type Integer) (Player3_SlotID :type Integer) (Player4_SlotID :type Integer) (PlayerCount :type Integer))
  (bind _returnvalue (Math|Vector|MakeVector 0.0 -5.4e+02 0.0))
  (bind _returnvalue_2 (Math|Vector|MakeVector 0.0 -3.7e+02 0.0))
  (bind _returnvalue_3 (Math|Vector|MakeVector 0.0 0.0 0.0))
  (bind _returnvalue_4 (Math|Vector|MakeVector 0.0 -4.7e+02 0.0))
  (bind _returnvalue_5 (Math|Vector|MakeVector 0.0 1.8e+02 0.0))
  (bind _returnvalue_6 (Math|Vector|MakeVector 0.0 -1.8e+02 0.0))
  (Utilities|FlowControl|Sequence
    (:then_0
      (Variables|Default|SetPlayer2_Online Player2_Online))
    (:then_1
      (Variables|Default|SetPlayer3_Online Player3_Online))
    (:then_2
      (Variables|Default|SetPlayer4_Online Player4_Online))
    (:then_3
      (Variables|Default|SetPalyer2_Slot Player2_SlotID))
    (:then_4
      (Variables|Default|SetPlayer3_Slot Player3_SlotID))
    (:then_5
      (Variables|Default|SetPlayer4_Slot Player4_SlotID))
    (:then_6
      (Variables|Default|SetCurrentPlayerCount PlayerCount))
    (:then_7
      (Utilities|FlowControl|Sequence
        (:then_0
          (if (== (Variables|Default|GetCurrentPlayerCount) 1)
            ;[1 1 1] Setup one player screen
            (Utilities|FlowControl|Sequence
              (:then_0
                (Transformation|SetRelativeScale3D (Variables|Default|GetPlayer1_ScaleController) "1.000000,1.000000,1.000000"))
              (:then_1
                (Transformation|SetRelativeLocation (Variables|Default|GetPlayer1_LocationController) (Math|Vector|MakeVector 0.0 0.0 0.0) false)))))
        (:then_1
          (if (== (Variables|Default|GetCurrentPlayerCount) 2)
            ;[1 1 1] Setup two player screen
            (Utilities|FlowControl|Sequence
              (:then_0
                (Transformation|SetRelativeScale3D (Variables|Default|GetPlayer1_ScaleController) "0.500000,1.000000,1.000000")
                (Transformation|SetRelativeScale3D (Variables|Default|GetPlayer2_ScaleController) "0.500000,1.000000,1.000000")
                (Transformation|SetRelativeScale3D (Variables|Default|GetPlayer3_ScaleController) "0.500000,1.000000,1.000000")
                (Transformation|SetRelativeScale3D (Variables|Default|GetPlayer4_ScaleController) "0.500000,1.000000,1.000000"))
              (:then_1
                (Utilities|FlowControl|Sequence
                  (:then_0
                    (Transformation|SetRelativeLocation (Variables|Default|GetPlayer1_LocationController) (Math|Vector|MakeVector 0.0 3.7e+02 0.0) false))
                  (:then_1
                    (if (== (Variables|Default|GetPalyer2_Slot) 2)
                      (Transformation|SetRelativeLocation (Variables|Default|GetPlayer2_LocationController) _returnvalue_2 false)))
                  (:then_2
                    (if (== (Variables|Default|GetPalyer2_Slot) 3)
                      (Transformation|SetRelativeLocation (Variables|Default|GetPlayer3_LocationController) _returnvalue_2 false)))
                  (:then_3
                    (if (== (Variables|Default|GetPalyer2_Slot) 4)
                      (Transformation|SetRelativeLocation (Variables|Default|GetPlayer4_LocationController) _returnvalue_2 false))))))))
        (:then_2
          (if (== (Variables|Default|GetCurrentPlayerCount) 3)
            ;[1 1 1] Setup three player screen
            (Utilities|FlowControl|Sequence
              (:then_0
                (Transformation|SetRelativeScale3D (Variables|Default|GetPlayer1_ScaleController) "0.300000,1.000000,1.000000")
                (Transformation|SetRelativeScale3D (Variables|Default|GetPlayer2_ScaleController) "0.300000,1.000000,1.000000")
                (Transformation|SetRelativeScale3D (Variables|Default|GetPlayer3_ScaleController) "0.300000,1.000000,1.000000")
                (Transformation|SetRelativeScale3D (Variables|Default|GetPlayer4_ScaleController) "0.300000,1.000000,1.000000"))
              (:then_1
                (Utilities|FlowControl|Sequence
                  (:then_0
                    (Transformation|SetRelativeLocation (Variables|Default|GetPlayer1_LocationController) (Math|Vector|MakeVector 0.0 4.7e+02 0.0) false))
                  (:then_1
                    (if (== (Variables|Default|GetPalyer2_Slot) 2)
                      (Transformation|SetRelativeLocation (Variables|Default|GetPlayer2_LocationController) _returnvalue_3 false)))
                  (:then_2
                    (if (== (Variables|Default|GetPalyer2_Slot) 3)
                      (Transformation|SetRelativeLocation (Variables|Default|GetPlayer3_LocationController) _returnvalue_3 false)))
                  (:then_3
                    (if (== (Variables|Default|GetPalyer2_Slot) 4)
                      (Transformation|SetRelativeLocation (Variables|Default|GetPlayer4_LocationController) _returnvalue_3 false)))
                  (:then_4
                    (Utilities|FlowControl|Sequence
                      (:then_0
                        (if (== (Variables|Default|GetPlayer3_Slot) 2)
                          (Transformation|SetRelativeLocation (Variables|Default|GetPlayer2_LocationController) _returnvalue_4 false)))
                      (:then_1
                        (if (== (Variables|Default|GetPlayer3_Slot) 3)
                          (Transformation|SetRelativeLocation (Variables|Default|GetPlayer3_LocationController) _returnvalue_4 false)))
                      (:then_2
                        (if (== (Variables|Default|GetPlayer3_Slot) 4)
                          (Transformation|SetRelativeLocation (Variables|Default|GetPlayer4_LocationController) _returnvalue_4 false))))))))))
        (:then_3
          (if (== (Variables|Default|GetCurrentPlayerCount) 4)
            ;[1 1 1] Setup four player screen
            (Utilities|FlowControl|Sequence
              (:then_0
                (Transformation|SetRelativeScale3D (Variables|Default|GetPlayer1_ScaleController) "0.250000,1.000000,1.000000")
                (Transformation|SetRelativeScale3D (Variables|Default|GetPlayer2_ScaleController) "0.250000,1.000000,1.000000")
                (Transformation|SetRelativeScale3D (Variables|Default|GetPlayer3_ScaleController) "0.250000,1.000000,1.000000")
                (Transformation|SetRelativeScale3D (Variables|Default|GetPlayer4_ScaleController) "0.250000,1.000000,1.000000"))
              (:then_1
                (Utilities|FlowControl|Sequence
                  (:then_0
                    (Transformation|SetRelativeLocation (Variables|Default|GetPlayer1_LocationController) (Math|Vector|MakeVector 0.0 5.4e+02 0.0) false))
                  (:then_1
                    (if (== (Variables|Default|GetPalyer2_Slot) 2)
                      (Transformation|SetRelativeLocation (Variables|Default|GetPlayer2_LocationController) _returnvalue_5 false)))
                  (:then_2
                    (if (== (Variables|Default|GetPalyer2_Slot) 3)
                      (Transformation|SetRelativeLocation (Variables|Default|GetPlayer3_LocationController) _returnvalue_5 false)))
                  (:then_3
                    (if (== (Variables|Default|GetPalyer2_Slot) 4)
                      (Transformation|SetRelativeLocation (Variables|Default|GetPlayer4_LocationController) _returnvalue_5 false)))
                  (:then_4
                    (Utilities|FlowControl|Sequence
                      (:then_0
                        (if (== (Variables|Default|GetPlayer3_Slot) 2)
                          (Transformation|SetRelativeLocation (Variables|Default|GetPlayer2_LocationController) _returnvalue_6 false)))
                      (:then_1
                        (if (== (Variables|Default|GetPlayer3_Slot) 3)
                          (Transformation|SetRelativeLocation (Variables|Default|GetPlayer3_LocationController) _returnvalue_6 false)))
                      (:then_2
                        (if (== (Variables|Default|GetPlayer3_Slot) 4)
                          (Transformation|SetRelativeLocation (Variables|Default|GetPlayer4_LocationController) _returnvalue_6 false)))
                      (:then_3
                        (Utilities|FlowControl|Sequence
                          (:then_0
                            (if (== (Variables|Default|GetPlayer4_Slot) 2)
                              (Transformation|SetRelativeLocation (Variables|Default|GetPlayer2_LocationController) _returnvalue false)))
                          (:then_1
                            (if (== (Variables|Default|GetPlayer4_Slot) 3)
                              (Transformation|SetRelativeLocation (Variables|Default|GetPlayer3_LocationController) _returnvalue false)))
                          (:then_2
                            (if (== (Variables|Default|GetPlayer4_Slot) 4)
                              (Transformation|SetRelativeLocation (Variables|Default|GetPlayer4_LocationController) _returnvalue false))))))))))))))))

(fn GetFocus
  (Variables|Default|SetInputFocus true)
  (Variables|Default|SetSuppressInput false)
  (Variables|Default|SetPlayer1_Selected false)
  (Variables|Default|SetPlayer2_Selected false)
  (Variables|Default|SetPlayer3_Selected false)
  (Variables|Default|SetPlayer4_Selected false)
  (Variables|Default|SetAllPlayersSelected false)
  (Default|SetFocus (Variables|Default|GetKartsInstance1))
  (Default|SetFocus (Variables|Default|GetKartsInstance2))
  (Default|SetFocus (Variables|Default|GetKartsInstance3))
  (Default|SetFocus (Variables|Default|GetKartsInstance4)))

(fn LeaveFocus
  (Variables|Default|SetInputFocus false)
  (Variables|Default|SetSuppressInput true)
  (Default|LeaveFocus (Variables|Default|GetKartsInstance1))
  (Default|LeaveFocus (Variables|Default|GetKartsInstance2))
  (Default|LeaveFocus (Variables|Default|GetKartsInstance3))
  (Default|LeaveFocus (Variables|Default|GetKartsInstance4)))

(fn SetKartsRenderInstances
  (params (KartsRenderSet1 :type Vehicle%20Camera%20Object%20Reference) (KartsRenderSet2 :type Vehicle%20Camera%20Object%20Reference) (KartsRenderSet3 :type Vehicle%20Camera%20Object%20Reference) (KartsRenderSet4 :type Vehicle%20Camera%20Object%20Reference))
  (Variables|Default|SetKartsInstance1 KartsRenderSet1)
  (Variables|Default|SetKartsInstance2 KartsRenderSet2)
  (Variables|Default|SetKartsInstance3 KartsRenderSet3)
  (Variables|Default|SetKartsInstance4 KartsRenderSet4))

(fn ShowKartsMenu
  (Variables|Default|SetFadeIn_InProgress true))

(fn HideKartsMenu
  (Variables|Default|SetFadeOff_InProgress true))

(fn PlayerKartSelected
  (params (PlayerID :type Integer))
  (Utilities|FlowControl|Sequence
    (:then_0
      (Variables|Default|SetAllPlayersSelected true))
    (:then_1
      (if (== PlayerID 1)
        (Variables|Default|SetPlayer1_Selected true)))
    (:then_2
      (if (== PlayerID 2)
        (Variables|Default|SetPlayer2_Selected true)))
    (:then_3
      (if (== PlayerID 3)
        (Variables|Default|SetPlayer3_Selected true)))
    (:then_4
      (if (== PlayerID 4)
        (Variables|Default|SetPlayer4_Selected true)))
    (:then_5
      (Utilities|FlowControl|Sequence
        (:then_0
          (if (not (Variables|Default|GetPlayer1_Selected))
            (Variables|Default|SetAllPlayersSelected false :!label _label)))
        (:then_1
          (if (Variables|Default|GetPlayer2_Online)
            (if (not (Variables|Default|GetPlayer2_Selected))
              (goto _label))))
        (:then_2
          (if (Variables|Default|GetPlayer3_Online)
            (if (not (Variables|Default|GetPlayer3_Selected))
              (goto _label))))
        (:then_3
          (if (Variables|Default|GetPlayer4_Online)
            (if (not (Variables|Default|GetPlayer4_Selected))
              (goto _label))))))))

(fn PlayerKartUnselected
  (params (PlayerID :type Integer))
  (Utilities|FlowControl|Sequence
    (:then_0
      (if (== PlayerID 1)
        (Variables|Default|SetPlayer1_Selected false)
        (Variables|Default|SetAllPlayersSelected false :!label _label)))
    (:then_1
      (if (== PlayerID 2)
        (Variables|Default|SetPlayer2_Selected false)
        (goto _label)))
    (:then_2
      (if (== PlayerID 3)
        (Variables|Default|SetPlayer3_Selected false)
        (goto _label)))
    (:then_3
      (if (== PlayerID 4)
        (Variables|Default|SetPlayer4_Selected false)
        (goto _label)))))

(fn RestoreState
  (bind _returnvalue (Class|GameStateStatics|GetControllerIndexes))
  (for (_array_element _array_index) _returnvalue
    (Utilities|FlowControl|Sequence
      (:then_0
        (if (== _array_index 1)
          (if (!= _array_element 0)
            (Variables|Default|SetPalyer2_Slot (Math|Conversions|ToInteger(Byte) (+ _array_element 1)))
            (Utilities|FlowControl|Sequence :!label _label
              (:then_0
                (if (== (Math|Conversions|ToInteger(Byte) (+ _array_element 1)) 2)
                  (Variables|Default|SetPlayer2_Online true)))
              (:then_1
                (if (== (Math|Conversions|ToInteger(Byte) (+ _array_element 1)) 3)
                  (Variables|Default|SetPlayer3_Online true)))
              (:then_2
                (if (== (Math|Conversions|ToInteger(Byte) (+ _array_element 1)) 4)
                  (Variables|Default|SetPlayer4_Online true)))))))
      (:then_1
        (if (== _array_index 2)
          (if (!= _array_element 0)
            (Variables|Default|SetPlayer3_Slot (Math|Conversions|ToInteger(Byte) (+ _array_element 1)))
            (goto _label))))
      (:then_2
        (if (== _array_index 3)
          (if (!= _array_element 0)
            (Variables|Default|SetPlayer4_Slot (Math|Conversions|ToInteger(Byte) (+ _array_element 1)))
            (goto _label))))))
  (bind _returnvalue_2 (Class|GameStateStatics|GetNumberOfPlayers))
  (CallFunction|SetPlayerStates (Variables|Default|GetPlayer2_Online) (Variables|Default|GetPlayer3_Online) (Variables|Default|GetPlayer4_Online) (Variables|Default|GetPalyer2_Slot) (Variables|Default|GetPlayer3_Slot) (Variables|Default|GetPlayer4_Slot) (Math|Conversions|ToInteger(Byte) _returnvalue_2)))