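; Per-player kart selection turntable for the main menu, with a scene capture that renders to a render target.
; Eight sockets hold spawned vehicles; left/right input starts a 45-degree lerped turn while FrontArrows keep constant world rotation.
; Each step rotates the vehicle and socket arrays, respawning only one end vehicle to cycle any list length, with index 3 as selection.
; Focus toggles input, capture and visibility; events report selection changes.
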(event EventBeginPlay
  ;[1 1 1] Initialize
  (Variables|Default|SetVehicleRotation (Transformation|GetWorldRotation (Variables|Default|GetTurntableSocket0)))
  (bind _returnvalue (Class|GameStateStatics|GetAvailableVehicles))
  (Variables|Default|SetAvailableVehicles _returnvalue)
  (for _index (range 0 2)
    (Utilities|Array|Insert (Variables|Default|GetAvailableVehicles) (Utilities|Array|Get(acopy) (Variables|Default|GetAvailableVehicles) (Utilities|Array|LastIndex (Variables|Default|GetAvailableVehicles))))
    (Utilities|Array|RemoveIndex (Variables|Default|GetAvailableVehicles) (Utilities|Array|LastIndex (Variables|Default|GetAvailableVehicles))))
  (Variables|Default|SetTurntableSockets (Utilities|Array|MakeArray (Variables|Default|GetTurntableSocket5) (Variables|Default|GetTurntableSocket6) (Variables|Default|GetTurntableSocket7) (Variables|Default|GetTurntableSocket0) (Variables|Default|GetTurntableSocket1) (Variables|Default|GetTurntableSocket2) (Variables|Default|GetTurntableSocket3) (Variables|Default|GetTurntableSocket4)))
  (for _index_2 (range 0 7)
    (bind _returnvalue_2 (Class|VehicleSpawnerLibrary|SpawnVehicle (Utilities|Array|Get(acopy) (Variables|Default|GetAvailableVehicles) (Math|Integer|%(Integer) _index_2 (Utilities|Array|Length (Variables|Default|GetAvailableVehicles)))) (Transformation|GetWorldLocation (Utilities|Array|Get(acopy) (Variables|Default|GetTurntableSockets) _index_2)) (Variables|Default|GetVehicleRotation)))
    (Class|VehiclePartBase|HidePart _returnvalue_2)
    (Class|Actor|AttachRootComponentto _returnvalue_2 (Utilities|Array|Get(acopy) (Variables|Default|GetTurntableSockets) _index_2) "None" "SnapToTarget")
    (Utilities|Array|Add (Variables|Default|GetSpawnedVehicles) _returnvalue_2)))

(event EventTick
  (params (DeltaSeconds :type Float%20%28single-precision%29))
  (bind _spawnedvehicles (Variables|Default|GetSpawnedVehicles))
  ;[1 1 1] Update logic
  (if (Variables|Default|GetHasFocus)
    (Variables|Default|SetRotationAlpha (+ (* DeltaSeconds (Variables|Default|GetRotationSpeed)) (Variables|Default|GetRotationAlpha)))
    (if (> (Variables|Default|GetRotationAlpha) 1.0)
      (Variables|Default|SetControlsActive true)
      (Variables|Default|SetRotationAlpha 1.0))
    (Transformation|SetWorldRotation (Variables|Default|GetTurntableRoot) (Math|Rotator|Lerp(Rotator) (Variables|Default|GetTurntableStartRotation) (Variables|Default|GetTurntableTargetRotation) (Variables|Default|GetRotationAlpha) true) false)
    (for _index (range 0 (Utilities|Array|LastIndex _spawnedvehicles))
      (Transformation|SetWorldRotation (Variables|/Script/DownhillMadness.VehicleBodyBase|GetFrontArrow (Utilities|Array|Get(acopy) _spawnedvehicles _index)) (Variables|Default|GetVehicleRotation) false))))

(event Input|KeyboardEvents|Enter
  (bind _availablevehicles (Variables|Default|GetAvailableVehicles))
  ;[1 1 1] Input event handling
  (:Pressed
    (if (Variables|Default|GetHasFocus)
      (if (Variables|Default|GetControlsActive)
        (if (not (Variables|Default|GetSuppressed))
          (Default|CallKartSelected (Math|Conversions|ToInteger(Byte) (Variables|Default|GetPlayerIndex)) (Variables|Default|GetScreenRef) (Utilities|Array|Get(acopy) _availablevehicles (Math|Integer|%(Integer) 3 (Utilities|Array|Length _availablevehicles)))))))))

(event Input|KeyboardEvents|Right
  (bind _turntableroot (Variables|Default|GetTurntableRoot))
  (bind _returnvalue (Transformation|GetWorldRotation _turntableroot))
  (bind (_pitch _yaw _roll) (Class|KismetMathLibrary|BreakRot _returnvalue))
  ;[1 1 1] Input event handling
  (:Pressed
    (if (Variables|Default|GetHasFocus)
      (if (Variables|Default|GetControlsActive)
        (if (not (Variables|Default|GetSuppressed))
          (CallFunction|SelectNextVehicle)
          (Variables|Default|SetControlsActive false)
          (Variables|Default|SetTurntableTargetRotation (Class|KismetMathLibrary|MakeRot _pitch (+ _yaw 45.0) _roll))
          (Variables|Default|SetTurntableStartRotation _returnvalue)
          (Variables|Default|SetRotationAlpha 0.0)
          (Default|CallKartUnselected (Math|Conversions|ToInteger(Byte) (Variables|Default|GetPlayerIndex))))))))

(event Input|KeyboardEvents|Left
  (bind _turntableroot (Variables|Default|GetTurntableRoot))
  (bind _returnvalue (Transformation|GetWorldRotation _turntableroot))
  (bind (_pitch _yaw _roll) (Class|KismetMathLibrary|BreakRot _returnvalue))
  ;[1 1 1] Input event handling
  (:Pressed
    (if (Variables|Default|GetHasFocus)
      (if (Variables|Default|GetControlsActive)
        (if (not (Variables|Default|GetSuppressed))
          (CallFunction|SelectPreviousVehicle)
          (Variables|Default|SetControlsActive false)
          (Variables|Default|SetTurntableTargetRotation (Class|KismetMathLibrary|MakeRot _pitch (+ _yaw -45.0) _roll))
          (Variables|Default|SetTurntableStartRotation _returnvalue)
          (Variables|Default|SetRotationAlpha 0.0)
          (Default|CallKartUnselected (Math|Conversions|ToInteger(Byte) (Variables|Default|GetPlayerIndex))))))))

(event Input|GamepadEvents|GamepadLeftStickLeft
  (bind _turntableroot (Variables|Default|GetTurntableRoot))
  (bind _returnvalue (Transformation|GetWorldRotation _turntableroot))
  (bind (_pitch _yaw _roll) (Class|KismetMathLibrary|BreakRot _returnvalue))
  ;[1 1 1] Input event handling
  (:Pressed
    (if (Variables|Default|GetHasFocus)
      (if (Variables|Default|GetControlsActive)
        (if (not (Variables|Default|GetSuppressed))
          (CallFunction|SelectPreviousVehicle)
          (Variables|Default|SetControlsActive false)
          (Variables|Default|SetTurntableTargetRotation (Class|KismetMathLibrary|MakeRot _pitch (+ _yaw -45.0) _roll))
          (Variables|Default|SetTurntableStartRotation _returnvalue)
          (Variables|Default|SetRotationAlpha 0.0)
          (Default|CallKartUnselected (Math|Conversions|ToInteger(Byte) (Variables|Default|GetPlayerIndex))))))))

(event Input|GamepadEvents|GamepadDPadLeft
  (bind _turntableroot (Variables|Default|GetTurntableRoot))
  (bind _returnvalue (Transformation|GetWorldRotation _turntableroot))
  (bind (_pitch _yaw _roll) (Class|KismetMathLibrary|BreakRot _returnvalue))
  ;[1 1 1] Input event handling
  (:Pressed
    (if (Variables|Default|GetHasFocus)
      (if (Variables|Default|GetControlsActive)
        (if (not (Variables|Default|GetSuppressed))
          (CallFunction|SelectPreviousVehicle)
          (Variables|Default|SetControlsActive false)
          (Variables|Default|SetTurntableTargetRotation (Class|KismetMathLibrary|MakeRot _pitch (+ _yaw -45.0) _roll))
          (Variables|Default|SetTurntableStartRotation _returnvalue)
          (Variables|Default|SetRotationAlpha 0.0)
          (Default|CallKartUnselected (Math|Conversions|ToInteger(Byte) (Variables|Default|GetPlayerIndex))))))))

(event Input|GamepadEvents|GamepadDPadRight
  (bind _turntableroot (Variables|Default|GetTurntableRoot))
  (bind _returnvalue (Transformation|GetWorldRotation _turntableroot))
  (bind (_pitch _yaw _roll) (Class|KismetMathLibrary|BreakRot _returnvalue))
  ;[1 1 1] Input event handling
  (:Pressed
    (if (Variables|Default|GetHasFocus)
      (if (Variables|Default|GetControlsActive)
        (if (not (Variables|Default|GetSuppressed))
          (CallFunction|SelectNextVehicle)
          (Variables|Default|SetControlsActive false)
          (Variables|Default|SetTurntableTargetRotation (Class|KismetMathLibrary|MakeRot _pitch (+ _yaw 45.0) _roll))
          (Variables|Default|SetTurntableStartRotation _returnvalue)
          (Variables|Default|SetRotationAlpha 0.0)
          (Default|CallKartUnselected (Math|Conversions|ToInteger(Byte) (Variables|Default|GetPlayerIndex))))))))

(event Input|GamepadEvents|GamepadLeftStickRight
  (bind _turntableroot (Variables|Default|GetTurntableRoot))
  (bind _returnvalue (Transformation|GetWorldRotation _turntableroot))
  (bind (_pitch _yaw _roll) (Class|KismetMathLibrary|BreakRot _returnvalue))
  ;[1 1 1] Input event handling
  (:Pressed
    (if (Variables|Default|GetHasFocus)
      (if (Variables|Default|GetControlsActive)
        (if (not (Variables|Default|GetSuppressed))
          (CallFunction|SelectNextVehicle)
          (Variables|Default|SetControlsActive false)
          (Variables|Default|SetTurntableTargetRotation (Class|KismetMathLibrary|MakeRot _pitch (+ _yaw 45.0) _roll))
          (Variables|Default|SetTurntableStartRotation _returnvalue)
          (Variables|Default|SetRotationAlpha 0.0)
          (Default|CallKartUnselected (Math|Conversions|ToInteger(Byte) (Variables|Default|GetPlayerIndex))))))))

(event Input|GamepadEvents|GamepadFaceButtonBottom
  (bind _availablevehicles (Variables|Default|GetAvailableVehicles))
  ;[1 1 1] Input event handling
  (:Pressed
    (if (Variables|Default|GetHasFocus)
      (if (Variables|Default|GetControlsActive)
        (if (not (Variables|Default|GetSuppressed))
          (Default|CallKartSelected (Math|Conversions|ToInteger(Byte) (Variables|Default|GetPlayerIndex)) (Variables|Default|GetScreenRef) (Utilities|Array|Get(acopy) _availablevehicles (Math|Integer|%(Integer) 3 (Utilities|Array|Length _availablevehicles)))))))))

(fn ConstructionScript
  (bind _capturescene (Variables|Default|GetCaptureScene))
  (Variables|/Script/Engine.SceneCaptureComponent2D|SetTextureTarget _capturescene (Variables|Default|GetRenderTarget))
  (Variables|/Script/Engine.SceneCaptureComponent|SetMaxViewDistanceOverride _capturescene (Variables|Default|GetMaxViewDistance)))

(fn SelectPreviousVehicle
  (bind _spawnedvehicles (Variables|Default|GetSpawnedVehicles))
  (bind _availablevehicles (Variables|Default|GetAvailableVehicles))
  (bind _turntablesockets (Variables|Default|GetTurntableSockets))
  (bind _availablevehicles_2 (Variables|Default|GetAvailableVehicles))
  (bind _turntablesockets_2 (Variables|Default|GetTurntableSockets))
  (bind _returnvalue (Utilities|Array|LastIndex _spawnedvehicles))
  (bind _returnvalue_2 (Utilities|Array|LastIndex _availablevehicles))
  (bind _returnvalue_3 (Utilities|Array|LastIndex _turntablesockets))
  (bind _item (Utilities|Array|Get(acopy) _spawnedvehicles _returnvalue))
  (bind _item_2 (Utilities|Array|Get(acopy) _availablevehicles _returnvalue_2))
  (bind _item_3 (Utilities|Array|Get(acopy) _turntablesockets _returnvalue_3))
  (Class|Actor|DetachRootComponentfromParent _item true)
  (Class|VehicleBodyBase|DestroyVehicle _item)
  (Utilities|Array|RemoveIndex _spawnedvehicles _returnvalue)
  (bind _returnvalue_4 (Class|VehicleSpawnerLibrary|SpawnVehicle _item_2 (Transformation|GetWorldLocation _item_3) (Variables|Default|GetVehicleRotation)))
  (Class|Actor|AttachRootComponentto _returnvalue_4 _item_3 "None" "SnapToTarget")
  (Utilities|Array|Insert (Variables|Default|GetSpawnedVehicles) _returnvalue_4)
  (Utilities|Array|Insert _availablevehicles_2 _item_2)
  (Utilities|Array|Insert _turntablesockets_2 _item_3)
  (Utilities|Array|RemoveIndex _availablevehicles_2 _returnvalue_2)
  (Utilities|Array|RemoveIndex _turntablesockets_2 _returnvalue_3))

(fn SelectNextVehicle
  (bind _spawnedvehicles (Variables|Default|GetSpawnedVehicles))
  (bind _availablevehicles (Variables|Default|GetAvailableVehicles))
  (bind _turntablesockets (Variables|Default|GetTurntableSockets))
  (bind _availablevehicles_2 (Variables|Default|GetAvailableVehicles))
  (bind _turntablesockets_2 (Variables|Default|GetTurntableSockets))
  (bind _item (Utilities|Array|Get(acopy) _turntablesockets))
  (bind _item_2 (Utilities|Array|Get(acopy) _spawnedvehicles))
  (Class|Actor|DetachRootComponentfromParent _item_2 true)
  (Class|VehicleBodyBase|DestroyVehicle _item_2)
  (Utilities|Array|RemoveIndex _spawnedvehicles)
  (bind _returnvalue (Class|VehicleSpawnerLibrary|SpawnVehicle (Utilities|Array|Get(acopy) _availablevehicles (Math|Integer|%(Integer) 8 (Utilities|Array|Length _availablevehicles))) (Transformation|GetWorldLocation _item) (Variables|Default|GetVehicleRotation)))
  (Class|Actor|AttachRootComponentto _returnvalue _item "None" "SnapToTarget")
  (Utilities|Array|Add (Variables|Default|GetSpawnedVehicles) _returnvalue)
  (Utilities|Array|Add _availablevehicles_2 (Utilities|Array|Get(acopy) _availablevehicles_2))
  (Utilities|Array|Add _turntablesockets_2 (Utilities|Array|Get(acopy) _turntablesockets_2))
  (Utilities|Array|RemoveIndex _availablevehicles_2)
  (Utilities|Array|RemoveIndex _turntablesockets_2))

(fn SetFocus
  (Input|EnableInput (Class|GameStateStatics|GetPlayerControllerfromID (- (Math|Conversions|ToInteger(Byte) (Variables|Default|GetPlayerIndex)) 1)))
  (Variables|Default|SetHasFocus true)
  (Components|Activation|Activate (Variables|Default|GetCaptureScene) false)
  (for _array_element (Variables|Default|GetSpawnedVehicles)
    (Class|VehiclePartBase|ShowPart _array_element)))

(fn LeaveFocus
  (Input|DisableInput (Class|GameStateStatics|GetPlayerControllerfromID (- (Math|Conversions|ToInteger(Byte) (Variables|Default|GetPlayerIndex)) 1)))
  (Variables|Default|SetHasFocus false)
  (Components|Activation|Deactivate (Variables|Default|GetCaptureScene))
  (for _array_element (Variables|Default|GetSpawnedVehicles)
    (Class|VehiclePartBase|HidePart _array_element)))

(fn Activate
  (Variables|Default|SetControlsActive true))

(fn Deactivate
  (Variables|Default|SetControlsActive false))

(fn SetScreenReference
  (params (ScreenRef :type Integer))
  (Variables|Default|SetScreenRef ScreenRef))

(fn GetKartName
  (bind _availablevehicles (Variables|Default|GetAvailableVehicles))
  (return (Class|GameStateStatics|ReplaceUmlaut (.vehicleName (Utilities|Struct|BreakSerializedVehicle (Utilities|Array|Get(acopy) _availablevehicles (Math|Integer|%(Integer) 3 (Utilities|Array|Length _availablevehicles))))))))

(fn Suppress
  (Variables|Default|SetSuppressed true))

(fn Unsuppress
  (Variables|Default|SetSuppressed false))