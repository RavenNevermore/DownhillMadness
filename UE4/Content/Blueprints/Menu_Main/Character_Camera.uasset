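; Main menu per-player character selection turntable, filmed by a scene capture into a render target.
; Left/right input steps through five characters, saves the choice globally and rotates the turntable by timeline while characters keep facing the camera.
; Start and Back are forwarded for players other than player one; focus functions toggle input and capture.
; On BeginPlay the locked fifth character is swapped for the real one if Ratatosk is unlocked.
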(event EventBeginPlay
  (bind _returnvalue (Class|GameStateStatics|GetRatatoskUnlocked))
  (if _returnvalue
    (Development|SetHiddeninGame (Variables|Default|GetAnimatedCharacter5Locked) true false)
    (Development|SetHiddeninGame (Variables|Default|GetAnimatedCharacter5) false false)))

(event EventTick
  (params (DeltaSeconds :type Float%20%28single-precision%29))
  (bind _char2 (Variables|Default|GetChar2))
  (bind _char3 (Variables|Default|GetChar3))
  (bind _char1 (Variables|Default|GetChar1))
  (bind _char0 (Variables|Default|GetChar0))
  (bind _char4 (Variables|Default|GetChar4))
  (bind _returnvalue (Transformation|GetWorldRotation _char4))
  (bind _returnvalue_2 (Transformation|GetWorldRotation _char2))
  (bind _returnvalue_3 (Transformation|GetWorldRotation _char3))
  (bind _returnvalue_4 (Transformation|GetWorldRotation _char1))
  (bind _returnvalue_5 (Transformation|GetWorldRotation _char0))
  (bind (_pitch _yaw _roll) (Class|KismetMathLibrary|BreakRot _returnvalue))
  (bind (_pitch_2 _yaw_2 _roll_2) (Class|KismetMathLibrary|BreakRot _returnvalue_2))
  (bind (_pitch_3 _yaw_3 _roll_3) (Class|KismetMathLibrary|BreakRot _returnvalue_3))
  (bind (_pitch_4 _yaw_4 _roll_4) (Class|KismetMathLibrary|BreakRot _returnvalue_4))
  (bind (_pitch_5 _yaw_5 _roll_5) (Class|KismetMathLibrary|BreakRot _returnvalue_5))
  (Utilities|FlowControl|Sequence
    (:then_0
      ;[1 1 1] Align players to camera
      (Utilities|FlowControl|Sequence :!label _label
        (:then_0
          (Transformation|SetWorldRotation _char2 (Class|KismetMathLibrary|MakeRot _pitch_2 9e+01 _roll_2) false))
        (:then_1
          (Transformation|SetWorldRotation _char3 (Class|KismetMathLibrary|MakeRot _pitch_3 9e+01 _roll_3) false))
        (:then_2
          (Transformation|SetWorldRotation _char1 (Class|KismetMathLibrary|MakeRot _pitch_4 9e+01 _roll_4) false))
        (:then_3
          (Transformation|SetWorldRotation _char0 (Class|KismetMathLibrary|MakeRot _pitch_5 9e+01 _roll_5) false))
        (:then_4
          (Transformation|SetWorldRotation _char4 (Class|KismetMathLibrary|MakeRot _pitch 9e+01 _roll) false))))
    (:then_1
      ;[1 1 1] Turntable controller
      (if (not (Variables|Default|GetSuppressInput))
        (if (Variables|Default|GetTurnTable)
          (Variables|Default|SetSuppressInput true)
          (bind _turn (Timeline|Timeline_0 PlayFromStart)
            (:Update
              (Utilities|FlowControl|Sequence
                (:then_0
                  (Transformation|SetRelativeRotation (Variables|Default|GetTurntable_HLP) (Class|KismetMathLibrary|MakeRot 0.0 (Math|Float|Lerp (Variables|Default|GetCurrentRotation) (Variables|Default|GetNewRotation) _turn) 0.0) false))
                (:then_1
                  (goto _label))))
            (:Finished
              (Variables|Default|SetCurrentRotation (Variables|Default|GetNewRotation))
              (Variables|Default|SetSuppressInput false)
              (Variables|Default|SetTurnTable false))))))))

(event Input|GamepadEvents|GamepadLeftStickRight
  ;[1 1 1] Button inputs
  (:Pressed
    (if (not (Variables|Default|GetSuppressInput))
      (if (not (Variables|Default|GetSuppressCharacterChange))
        (if (< (Variables|Default|GetSelectedCharacterID) 4)
          (Utilities|FlowControl|Sequence
            (:then_0
              (Variables|Default|SetNewRotation (+ (Variables|Default|GetCurrentRotation) 45.0)))
            (:then_1
              (Variables|Default|SetTurnTable true))
            (:then_2
              (Variables|Default|SetSelectedCharacterID (+ (Variables|Default|GetSelectedCharacterID) 1)))
            (:then_3
              ;[1 1 1] Save to globals
              (Class|GameStateStatics|SetSelectedCharacter (Math|Conversions|ToByte(Integer) (- (Variables|Default|GetLocalPlayerID) 1)) (Math|Conversions|ToByte(Integer) (Variables|Default|GetSelectedCharacterID))))))))))

(event Input|KeyboardEvents|Right
  ;[1 1 1] Button inputs
  (:Pressed
    (if (not (Variables|Default|GetSuppressInput))
      (if (not (Variables|Default|GetSuppressCharacterChange))
        (if (< (Variables|Default|GetSelectedCharacterID) 4)
          (Utilities|FlowControl|Sequence
            (:then_0
              (Variables|Default|SetNewRotation (+ (Variables|Default|GetCurrentRotation) 45.0)))
            (:then_1
              (Variables|Default|SetTurnTable true))
            (:then_2
              (Variables|Default|SetSelectedCharacterID (+ (Variables|Default|GetSelectedCharacterID) 1)))
            (:then_3
              ;[1 1 1] Save to globals
              (Class|GameStateStatics|SetSelectedCharacter (Math|Conversions|ToByte(Integer) (- (Variables|Default|GetLocalPlayerID) 1)) (Math|Conversions|ToByte(Integer) (Variables|Default|GetSelectedCharacterID))))))))))

(event Input|GamepadEvents|GamepadLeftStickLeft
  ;[1 1 1] Button inputs
  (:Pressed
    (if (not (Variables|Default|GetSuppressInput))
      (if (not (Variables|Default|GetSuppressCharacterChange))
        (if (> (Variables|Default|GetSelectedCharacterID) 0)
          (Utilities|FlowControl|Sequence
            (:then_0
              (Variables|Default|SetNewRotation (- (Variables|Default|GetCurrentRotation) 45.0)))
            (:then_1
              (Variables|Default|SetTurnTable true))
            (:then_2
              (Variables|Default|SetSelectedCharacterID (- (Variables|Default|GetSelectedCharacterID) 1)))
            (:then_3
              ;[1 1 1] Save to globals
              (Class|GameStateStatics|SetSelectedCharacter (Math|Conversions|ToByte(Integer) (- (Variables|Default|GetLocalPlayerID) 1)) (Math|Conversions|ToByte(Integer) (Variables|Default|GetSelectedCharacterID))))))))))

(event Input|KeyboardEvents|Left
  ;[1 1 1] Button inputs
  (:Pressed
    (if (not (Variables|Default|GetSuppressInput))
      (if (not (Variables|Default|GetSuppressCharacterChange))
        (if (> (Variables|Default|GetSelectedCharacterID) 0)
          (Utilities|FlowControl|Sequence
            (:then_0
              (Variables|Default|SetNewRotation (- (Variables|Default|GetCurrentRotation) 45.0)))
            (:then_1
              (Variables|Default|SetTurnTable true))
            (:then_2
              (Variables|Default|SetSelectedCharacterID (- (Variables|Default|GetSelectedCharacterID) 1)))
            (:then_3
              ;[1 1 1] Save to globals
              (Class|GameStateStatics|SetSelectedCharacter (Math|Conversions|ToByte(Integer) (- (Variables|Default|GetLocalPlayerID) 1)) (Math|Conversions|ToByte(Integer) (Variables|Default|GetSelectedCharacterID))))))))))

(event Input|GamepadEvents|GamepadSpecialRight
  (bind _localplayerid (Variables|Default|GetLocalPlayerID))
  ;[1 1 1] Button inputs
  (:Pressed
    (if (not (Variables|Default|GetSuppressInput))
      (if (!= _localplayerid 1)
        (Default|CallPressButtonStart _localplayerid)))))

(event Input|GamepadEvents|GamepadDPadRight
  ;[1 1 1] Button inputs
  (:Pressed
    (if (not (Variables|Default|GetSuppressInput))
      (if (not (Variables|Default|GetSuppressCharacterChange))
        (if (< (Variables|Default|GetSelectedCharacterID) 4)
          (Utilities|FlowControl|Sequence
            (:then_0
              (Variables|Default|SetNewRotation (+ (Variables|Default|GetCurrentRotation) 45.0)))
            (:then_1
              (Variables|Default|SetTurnTable true))
            (:then_2
              (Variables|Default|SetSelectedCharacterID (+ (Variables|Default|GetSelectedCharacterID) 1)))
            (:then_3
              ;[1 1 1] Save to globals
              (Class|GameStateStatics|SetSelectedCharacter (Math|Conversions|ToByte(Integer) (- (Variables|Default|GetLocalPlayerID) 1)) (Math|Conversions|ToByte(Integer) (Variables|Default|GetSelectedCharacterID))))))))))

(event Input|GamepadEvents|GamepadDPadLeft
  ;[1 1 1] Button inputs
  (:Pressed
    (if (not (Variables|Default|GetSuppressInput))
      (if (not (Variables|Default|GetSuppressCharacterChange))
        (if (> (Variables|Default|GetSelectedCharacterID) 0)
          (Utilities|FlowControl|Sequence
            (:then_0
              (Variables|Default|SetNewRotation (- (Variables|Default|GetCurrentRotation) 45.0)))
            (:then_1
              (Variables|Default|SetTurnTable true))
            (:then_2
              (Variables|Default|SetSelectedCharacterID (- (Variables|Default|GetSelectedCharacterID) 1)))
            (:then_3
              ;[1 1 1] Save to globals
              (Class|GameStateStatics|SetSelectedCharacter (Math|Conversions|ToByte(Integer) (- (Variables|Default|GetLocalPlayerID) 1)) (Math|Conversions|ToByte(Integer) (Variables|Default|GetSelectedCharacterID))))))))))

(event Input|GamepadEvents|GamepadSpecialLeft
  (bind _localplayerid (Variables|Default|GetLocalPlayerID))
  ;[1 1 1] Button inputs
  (:Pressed
    (if (not (Variables|Default|GetSuppressInput))
      (if (!= _localplayerid 1)
        (Default|CallPressButtonBack _localplayerid)))))

(fn ConstructionScript
  (bind _capturescene (Variables|Default|GetCaptureScene))
  (Variables|/Script/Engine.SceneCaptureComponent2D|SetTextureTarget _capturescene (Variables|Default|GetCaptureTextureRT))
  (Variables|/Script/Engine.SceneCaptureComponent|SetMaxViewDistanceOverride _capturescene (Variables|Default|GetCaptureDistance)))

(fn SetCharacterMaterial
  (params (Material :type Material%20Object%20Reference) (CharacterINDX :type Integer) (MaterialINDX :type Integer))
  (Utilities|FlowControl|Sequence
    (:then_0
      (if (== CharacterINDX 1)
        (Rendering|Material|SetMaterial (Variables|Default|GetChar2) (stale _index) Material :!label _label)))
    (:then_1
      (if (== CharacterINDX 2)
        (Rendering|Material|SetMaterial (Variables|Default|GetChar3) (stale _index_2) Material :!label _label_2)))
    (:then_2
      (if (== CharacterINDX 3)
        (Rendering|Material|SetMaterial (Variables|Default|GetChar1) (stale _index_3) Material :!label _label_3)))
    (:then_3
      (if (== CharacterINDX 4)
        (Rendering|Material|SetMaterial (Variables|Default|GetChar0) (stale _index_4) Material :!label _label_4)))
    (:then_4
      (if (== CharacterINDX 5)
        (Rendering|Material|SetMaterial (Variables|Default|GetChar4) (stale _index_5) Material :!label _label_5)))
    (:then_5
      (if (== CharacterINDX -1)
        (Utilities|FlowControl|Sequence
          (:then_0
            (goto _label))
          (:then_1
            (goto _label_2))
          (:then_2
            (goto _label_3))
          (:then_3
            (goto _label_4))
          (:then_4
            (goto _label_5)))))
    (:then_6
      (if (== MaterialINDX -1)
        (Utilities|FlowControl|Sequence
          (:then_0
            (for _index (range 0 (- (Rendering|Material|GetNumMaterials (Variables|Default|GetChar2)) 1))
              (goto _label)))
          (:then_1
            (for _index_2 (range 0 (- (Rendering|Material|GetNumMaterials (Variables|Default|GetChar3)) 1))
              (goto _label_2)))
          (:then_2
            (for _index_3 (range 0 (- (Rendering|Material|GetNumMaterials (Variables|Default|GetChar1)) 1))
              (goto _label_3)))
          (:then_3
            (for _index_4 (range 0 (- (Rendering|Material|GetNumMaterials (Variables|Default|GetChar0)) 1))
              (goto _label_4)))
          (:then_4
            (for _index_5 (range 0 (- (Rendering|Material|GetNumMaterials (Variables|Default|GetChar4)) 1))
              (goto _label_5))))))))

(fn TurnTableRight
  (if (not (Variables|Default|GetSuppressInput))
    (Variables|Default|SetTurnTable true)))

(fn TurnTableLeft
  (if (not (Variables|Default|GetSuppressInput))
    (Variables|Default|SetTurnLeft true)))

(fn GetFocus
  (bind _localplayerid (Variables|Default|GetLocalPlayerID))
  (bind _returnvalue (- _localplayerid 1))
  (bind _returnvalue_2 (Game|GetPlayerController _returnvalue))
  (Pawn|Possess _returnvalue_2 (Game|Player|GetPlayerPawn _returnvalue))
  (Input|EnableInput _returnvalue_2)
  (Components|Activation|Activate (Variables|Default|GetCaptureScene) false)
  (Variables|Default|SetSuppressInput false))

(fn LeaveFocus
  (Input|DisableInput (Game|GetPlayerController (- (Variables|Default|GetLocalPlayerID) 1)))
  (Components|Activation|Deactivate (Variables|Default|GetCaptureScene))
  (Variables|Default|SetSuppressInput true))

(fn Deactivate
  (Variables|Default|SetSuppressCharacterChange true))

(fn Activate
  (Variables|Default|SetSuppressCharacterChange false))