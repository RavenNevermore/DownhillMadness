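; Menu helper Blueprint that exposes the saved player count and character picks for up to four players, and can open the main menu level.
; Initialize loads the GlobalData save slot as Global_DataTransfer, or creates an unsaved default object if none exists, then caches its values.
; GetPlayerCount and GetPlayerCharacter read those cached values, with character lookup by player IDs one to four.
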(fn ConstructionScript)

(fn GetPlayerCount
  (return (Variables|Default|GetPlayerCount)))

(fn GetPlayerCharacter
  (params (PlayerID :type Integer))
  (Utilities|FlowControl|Sequence
    (:then_0
      (if (== PlayerID 1)
        (Variables|Default|SetPlayerCharacterRET (Variables|Default|GetPlayer1Character))
        (return (Variables|Default|GetPlayerCharacterRET))))
    (:then_1
      (if (== PlayerID 2)
        (Variables|Default|SetPlayerCharacterRET (Variables|Default|GetPlayer2Character))
        (return (Variables|Default|GetPlayerCharacterRET))))
    (:then_2
      (if (== PlayerID 3)
        (Variables|Default|SetPlayerCharacterRET (Variables|Default|GetPlayer3Character))
        (return (Variables|Default|GetPlayerCharacterRET))))
    (:then_3
      (if (== PlayerID 4)
        (Variables|Default|SetPlayerCharacterRET (Variables|Default|GetPlayer4Character))
        (return (Variables|Default|GetPlayerCharacterRET))))))

(fn Initialize
  (bind _returnvalue (SaveGame|DoesSaveGameExist "GlobalData"))
  (if _returnvalue
    (bind _returnvalue_2 (SaveGame|LoadGamefromSlot "GlobalData"))
    (bind _asglobal_datatransfer_c (Utilities|Casting|CastToGlobal_DataTransfer _returnvalue_2))
    (Variables|Default|SetGlobalData _asglobal_datatransfer_c)
    (else
      (bind _returnvalue_3 (SaveGame|CreateSaveGameObject "/Game/Blueprints/Global_DataTransfer.Global_DataTransfer_C"))
      (bind _asglobal_datatransfer_c_2 (Utilities|Casting|CastToGlobal_DataTransfer _returnvalue_3))
      (Variables|Default|SetGlobalData _asglobal_datatransfer_c_2)))
  (Variables|Default|SetPlayer1Character (Variables|/Game/Blueprints/Global_DataTransfer.Global_DataTransfer_C|GetPlayer_1_CharacterID (Variables|Default|GetGlobalData)))
  (Variables|Default|SetPlayer2Character (Variables|/Game/Blueprints/Global_DataTransfer.Global_DataTransfer_C|GetPlayer_2_CharacterID (Variables|Default|GetGlobalData)))
  (Variables|Default|SetPlayer3Character (Variables|/Game/Blueprints/Global_DataTransfer.Global_DataTransfer_C|GetPlayer_3_CharacterID (Variables|Default|GetGlobalData)))
  (Variables|Default|SetPlayer4Character (Variables|/Game/Blueprints/Global_DataTransfer.Global_DataTransfer_C|GetPlayer_4_CharacterID (Variables|Default|GetGlobalData)))
  (Variables|Default|SetPlayerCount (Variables|/Game/Blueprints/Global_DataTransfer.Global_DataTransfer_C|GetPlayerCount (Variables|Default|GetGlobalData))))

(fn GotoMainMenu
  (Game|OpenLevel(byName) "Menu_Main"))